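; Base swinging door Blueprint for the procedural city, opened by interaction and closed automatically.
; Front and back trigger volumes track which side the Player entered first, which sets the swing direction.
; FnInteract calls the open event, where a timeline lerps the door's yaw a quarter turn.
; Leaving a trigger waits OpenDuration, then plays the closing timeline if both sides are clear, with state flags gating each movement.
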(event OnComponentBeginOverlap(TriggerFront)
  (params (OverlappedComponent :type Primitive%20Component%20Object%20Reference) (OtherActor :type Actor%20Object%20Reference) (OtherComp :type Primitive%20Component%20Object%20Reference) (OtherBodyIndex :type Integer) (bFromSweep :type Boolean) (SweepResult :type Hit%20Result%20Structure%20%28by%20ref%29))
  ;[1 1 1] Check that we overlapped the Player
  (if (Actor|ActorHasTag OtherActor "Player")
    ;[1 1 1] If no one is already here, set parameters
    (if (not (Variables|Default|GetSomeoneHere))
      (Variables|Default|SetFrontTrigger true)
      (Variables|Default|SetBackTrigger false)
      (Variables|Default|SetSomeoneHere true))))

(event OnComponentEndOverlap(TriggerFront)
  (params (OverlappedComponent :type Primitive%20Component%20Object%20Reference) (OtherActor :type Actor%20Object%20Reference) (OtherComp :type Primitive%20Component%20Object%20Reference) (OtherBodyIndex :type Integer))
  ;[1 1 1] Check that we overlapped the Player
  (if (Actor|ActorHasTag OtherActor "Player")
    ;[1 1 1] Wait OpenDuration and then close the door
    (Variables|Default|SetFrontTrigger false)
    (Utilities|FlowControl|Delay (Variables|Setup|GetOpenDuration))
    (CallFunction|EventCloseDoor)
    (Variables|Default|SetSomeoneHere false)))

(event OnComponentBeginOverlap(TriggerBack)
  (params (OverlappedComponent :type Primitive%20Component%20Object%20Reference) (OtherActor :type Actor%20Object%20Reference) (OtherComp :type Primitive%20Component%20Object%20Reference) (OtherBodyIndex :type Integer) (bFromSweep :type Boolean) (SweepResult :type Hit%20Result%20Structure%20%28by%20ref%29))
  ;[1 1 1] Check that we overlapped the Player
  (if (Actor|ActorHasTag OtherActor "Player")
    ;[1 1 1] If no one is already here, set parameters
    (if (not (Variables|Default|GetSomeoneHere))
      (Variables|Default|SetBackTrigger true)
      (Variables|Default|SetFrontTrigger false)
      (Variables|Default|SetSomeoneHere true))))

(event OnComponentEndOverlap(TriggerBack)
  (params (OverlappedComponent :type Primitive%20Component%20Object%20Reference) (OtherActor :type Actor%20Object%20Reference) (OtherComp :type Primitive%20Component%20Object%20Reference) (OtherBodyIndex :type Integer))
  ;[1 1 1] Check that we overlapped the Player
  (if (Actor|ActorHasTag OtherActor "Player")
    ;[1 1 1] Wait OverlapDuration and then close the door
    (Variables|Default|SetBackTrigger false)
    (Utilities|FlowControl|Delay (Variables|Setup|GetOpenDuration))
    (CallFunction|EventCloseDoor)
    (Variables|Default|SetSomeoneHere false)))

(fn ConstructionScript)

(event Custom|EventOpenDoor
  ;[1 1 1] Check that we can open the door and are not already openning it
  (if (and (Variables|Default|GetCanOpen) (not (Variables|Default|GetOpening)))
    (if (Variables|Default|GetFrontTrigger)
      (Variables|Default|SetGoalRotation -9e+01)
      (bind _alpha (Timeline|TM_Open PlayFromStart)
        (:Update
          (Transformation|SetRelativeRotation (Variables|Default|GetDoor) (Math|Rotator|MakeRotator 0.0 0.0 (Math|Float|Lerp 0.0 (Variables|Default|GetGoalRotation) _alpha)) false false))
        (:Finished
          (Variables|Default|SetCanClose true)
          (Variables|Default|SetCanOpen false)
          (Variables|Default|SetOpening false)))
      (elif (Variables|Default|GetBackTrigger)
        (Variables|Default|SetGoalRotation 9e+01)
        (Timeline|TM_Open PlayFromStart)))))

(event Custom|EventCloseDoor
  ;[1 1 1] Check that we can close the door and are not already closing it
  (if (and (Variables|Default|GetCanClose) (not (Variables|Default|GetClosing)))
    (if (and (not (Variables|Default|GetFrontTrigger)) (not (Variables|Default|GetBackTrigger)))
      (bind _alpha (Timeline|TM_Close PlayFromStart)
        (:Update
          (Transformation|SetRelativeRotation (Variables|Default|GetDoor) (Math|Rotator|MakeRotator 0.0 0.0 (Math|Float|Lerp (Variables|Default|GetGoalRotation) 0.0 _alpha)) false false)
          (Variables|Default|SetClosing true))
        (:Finished
          (Variables|Default|SetCanOpen true)
          (Variables|Default|SetCanClose false)
          (Variables|Default|SetClosing false))))))

(event EventFnInteract
  (params (Reference%20Actor :type Actor%20Object%20Reference))
  (Variables|Default|SetOwnerActor Reference%20Actor)
  ;[1 1 1] Check that we can interact
  (if (Variables|Setup|GetCanInteract)
    (CallFunction|EventOpenDoor)))