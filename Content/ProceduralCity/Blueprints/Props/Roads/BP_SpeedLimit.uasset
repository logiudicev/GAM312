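; Speed limit sign prop for procedural city roads that shows its limit as text and can be knocked over by vehicles.
; The construction script displays the SpeedLimit value and applies a max draw distance cull to the body and head.
; FnSetRoadType overrides the text with a fixed speed for the given road type.
; A hit from an actor tagged pcgVehicle turns on physics simulation for the body.
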(event Collision|EventHit
  (params (MyComp :type Primitive%20Component%20Object%20Reference) (Other :type Actor%20Object%20Reference) (OtherComp :type Primitive%20Component%20Object%20Reference) (bSelfMoved :type Boolean) (HitLocation :type Vector :default "0, 0, 0") (HitNormal :type Vector :default "0, 0, 0") (NormalImpulse :type Vector :default "0, 0, 0") (Hit :type Hit%20Result%20Structure%20%28by%20ref%29))
  ;[1 1 1] If hit by a vehicle, simulate physics
  (if (Actor|ActorHasTag Other "pcgVehicle")
    (Physics|SetSimulatePhysics (Variables|Default|GetBody) true)))

(event EventFnSetRoadType
  (params (Road%20Type :type Enum_RoadType%20Enum :default "NewEnumerator0"))
  (Variables|Setup|SetRoadType Road%20Type)
  (Utilities|FlowControl|Sequence
    (:then_0
      ;[1 1 1] Set the Speed limit based on the Road Type
      (switch Utilities|FlowControl|Switch|SwitchonEnum_RoadType (Variables|Setup|GetRoadType)
        (:NewEnumerator0
          (Variables|Default|SetRoadSpeed "70"))
        (:NewEnumerator1
          (Variables|Default|SetRoadSpeed "55"))
        (:NewEnumerator2
          (Variables|Default|SetRoadSpeed "35"))
        (:NewEnumerator3
          (Variables|Default|SetRoadSpeed "25"))))
    (:then_1
      ;[1 1 1] Set the text to the road speed
      (Rendering|Components|TextRender|SetText (Variables|Default|GetText_Limit) (Variables|Default|GetRoadSpeed)))))

(fn ConstructionScript
  ;[1 1 1] Set Speed
  (Rendering|Components|TextRender|SetText (Variables|Default|GetText_Limit) (Utilities|Text|ToText(Integer) (Variables|Setup|GetSpeedLimit)))
  ;[1 1 1] Set Max Draw Distance
  (Class|PrimitiveComponent|SetCullDistance (Variables|Default|GetBody) (Variables|Setup|GetMaxDrawDistance)))