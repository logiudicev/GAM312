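; Elevator landing frame for the procedural city that calls a linked cage and provides sliding doors and direction lights.
; Interacting while the player is inside the door trigger sets this frame as the cage's current target and starts it moving.
; The up and down lights compare cage height to the frame's target height to show travel direction.
; Doors open and close by timeline-driven Y scaling, auto-closing after a delay.
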(event OnComponentBeginOverlap(Door_Trigger)
  (params (OverlappedComponent :type Primitive%20Component%20Object%20Reference) (OtherActor :type Actor%20Object%20Reference) (OtherComp :type Primitive%20Component%20Object%20Reference) (OtherBodyIndex :type Integer) (bFromSweep :type Boolean) (SweepResult :type Hit%20Result%20Structure%20%28by%20ref%29))
  ;[1 1 1] Detect if we overlapped the Player and set CanInteract to True
  (if (Actor|ActorHasTag OtherActor "Player")
    (Variables|Setup|SetCanInteract true)))

(event OnComponentEndOverlap(Door_Trigger)
  (params (OverlappedComponent :type Primitive%20Component%20Object%20Reference) (OtherActor :type Actor%20Object%20Reference) (OtherComp :type Primitive%20Component%20Object%20Reference) (OtherBodyIndex :type Integer))
  ;[1 1 1] Detect that we overlapped the Player and set CanInteract to False
  (if (Actor|ActorHasTag OtherActor "Player")
    (Variables|Setup|SetCanInteract false)))

(event EventFnInteract
  (params (Reference%20Actor :type Actor%20Object%20Reference))
  (Variables|Default|SetOwnerActor Reference%20Actor)
  ;[1 1 1] Check that we can interact
  (if (Variables|Setup|GetCanInteract)
    ;[1 1 1] Set Self to CurrentFrame
    (Variables|/Game/ProceduralCity/Blueprints/Props/Elevators/BP_Elevator_Base.BP_Elevator_Base_C|SetCurrentFrame (Variables|Setup|GetCageRef) self)
    ;[1 1 1] Start moving elevator
    (Variables|/Game/ProceduralCity/Blueprints/Props/Elevators/BP_Elevator_Base.BP_Elevator_Base_C|SetMoveElevator (Variables|Setup|GetCageRef) true)
    (CallFunction|FnSetLights false)))

(fn ConstructionScript)

(fn FnSetLights
  (params (Turn%20Off :type Boolean))
  (LocalVariables|SetOff Turn%20Off)
  (Utilities|IsValid (Variables|Setup|GetCageRef)
    (:Is%20Valid
      (if (LocalVariables|GetOff)
        (Rendering|Material|SetMaterial (Variables|Default|GetDown) 0 "/Game/ProceduralCity/Materials/Elevator/MI_Elevator_Light_Off.MI_Elevator_Light_Off")
        (Rendering|Material|SetMaterial (Variables|Default|GetUp) 0 "/Game/ProceduralCity/Materials/Elevator/MI_Elevator_Light_Off.MI_Elevator_Light_Off")
        (else
          ;[1 1 1] Is Cage higher than this frame?
          (if (> (.z (Transformation|GetActorLocation (Variables|Setup|GetCageRef))) (Variables|Setup|GetTargetHeight))
            (Rendering|Material|SetMaterial (Variables|Default|GetDown) 0 "/Game/ProceduralCity/Materials/Elevator/MI_Elevator_Light_Red.MI_Elevator_Light_Red")
            (Rendering|Material|SetMaterial (Variables|Default|GetUp) 0 "/Game/ProceduralCity/Materials/Elevator/MI_Elevator_Light_Off.MI_Elevator_Light_Off")
            (else
              (Rendering|Material|SetMaterial (Variables|Default|GetDown) 0 "/Game/ProceduralCity/Materials/Elevator/MI_Elevator_Light_Off.MI_Elevator_Light_Off")
              (Rendering|Material|SetMaterial (Variables|Default|GetUp) 0 "/Game/ProceduralCity/Materials/Elevator/MI_Elevator_Light_Green.MI_Elevator_Light_Green"))))))))

(event Custom|EventOpenDoors
  (bind _alpha (Timeline|TM_Open PlayFromStart)
    (:Update
      (Transformation|SetRelativeScale3D (Variables|Default|GetDoorRight) (Math|Vector|MakeVector 1.0 (Math|Float|Lerp 1.0 0.1 _alpha) 1.0))
      (Variables|Default|SetDoorOpen true))
    (:Finished
      ;[1 1 1] Wait OpenDoorDelay and if doors are still open, close them
      (Utilities|FlowControl|Delay (Variables|Setup|GetOpenDoorDelay))
      (if (Variables|Default|GetDoorOpen)
        (CallFunction|EventCloseDoors)
        (Variables|Default|SetDoorOpen false)))))

(event Custom|EventCloseDoors
  (bind _alpha (Timeline|TM_Close PlayFromStart)
    (:Update
      (Transformation|SetRelativeScale3D (Variables|Default|GetDoorRight) (Math|Vector|MakeVector 1.0 (Math|Float|Lerp 0.1 1.0 _alpha) 1.0)))))