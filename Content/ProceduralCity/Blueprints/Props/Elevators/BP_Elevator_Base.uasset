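; Base elevator cage for procedural city props, which carries the player between floors picked from a HUD menu.
; BeginPlay spawns a BP_ElevatorFrame per floor, at listed or evenly spaced heights.
; Interacting inside the panel trigger opens the menu; FnSetFloor picks a target frame, closing any open doors before travel.
; Tick teleports or moves the cage at constant speed, then timelines scale doors open alongside the frame's, auto-closing after a delay.
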(event OnComponentBeginOverlap(Panel_Trigger)
  (params (OverlappedComponent :type Primitive%20Component%20Object%20Reference) (OtherActor :type Actor%20Object%20Reference) (OtherComp :type Primitive%20Component%20Object%20Reference) (OtherBodyIndex :type Integer) (bFromSweep :type Boolean) (SweepResult :type Hit%20Result%20Structure%20%28by%20ref%29))
  ;[1 1 1] TRIGGERS
  (if (Actor|ActorHasTag OtherActor "Player")
    (Variables|Default|SetOnPanel true)))

(event OnComponentEndOverlap(Panel_Trigger)
  (params (OverlappedComponent :type Primitive%20Component%20Object%20Reference) (OtherActor :type Actor%20Object%20Reference) (OtherComp :type Primitive%20Component%20Object%20Reference) (OtherBodyIndex :type Integer))
  ;[1 1 1] TRIGGERS
  (if (Actor|ActorHasTag OtherActor "Player")
    (Variables|Default|SetOnPanel false)))

(event OnComponentBeginOverlap(Door_Trigger)
  (params (OverlappedComponent :type Primitive%20Component%20Object%20Reference) (OtherActor :type Actor%20Object%20Reference) (OtherComp :type Primitive%20Component%20Object%20Reference) (OtherBodyIndex :type Integer) (bFromSweep :type Boolean) (SweepResult :type Hit%20Result%20Structure%20%28by%20ref%29))
  ;[1 1 1] TRIGGERS
  (if (Actor|ActorHasTag OtherActor "Player")
    (Variables|Default|SetOnDoors true)))

(event OnComponentEndOverlap(Door_Trigger)
  (params (OverlappedComponent :type Primitive%20Component%20Object%20Reference) (OtherActor :type Actor%20Object%20Reference) (OtherComp :type Primitive%20Component%20Object%20Reference) (OtherBodyIndex :type Integer))
  ;[1 1 1] TRIGGERS
  (if (Actor|ActorHasTag OtherActor "Player")
    (Variables|Default|SetOnDoors false)))

(event EventFnInteract
  (params (Reference%20Actor :type Actor%20Object%20Reference))
  (Variables|Interaction|SetOwnerActor Reference%20Actor)
  ;[1 1 1] Check that we can interact
  (if (Variables|Interaction|GetCanInteract)
    ;[1 1 1] Check if the Player is infront of the panel, if so show the menu
    (if (Variables|Default|GetOnPanel)
      (CallFunction|EventShowMenu))))

(event EventBeginPlay
  (CallFunction|FnSpawnFrames))

(event EventTick
  (params (DeltaSeconds :type Float%20%28single-precision%29))
  (Variables|Default|SetDeltaSecs DeltaSeconds)
  (|MOVEELEVATOR))

(fn ConstructionScript)

(fn FnSetFloor
  (params (Target%20Floor :type Integer))
  ;[1 1 1] Set TargetFloor and get a reference to the Current Frame for that floor
  (bind _output_get (Variables|Setup|SetTargetFloor (Math|Integer|Clamp(Integer) Target%20Floor 1 (Variables|Setup|GetTotalFloors))))
  (Variables|Default|SetCurrentFrame (Utilities|Array|Get(acopy) (Variables|Default|GetFrameList) (- _output_get 1)))
  ;[1 1 1] Check if the door is open, if so, close it
  (if (Variables|Default|GetDoorOpen)
    (CallFunction|EventCloseDoors true)
    (else
      (Variables|Default|SetMoveElevator true))))

(fn FnSpawnFrames
  (bind _returnvalue (Transformation|GetActorLocation))
  ;[1 1 1] Loop through all the floors
  (for _index (range 1 (Variables|Setup|GetTotalFloors))
    (Variables|Setup|SetTargetFloor _index)
    (if (Variables|Setup|GetUseFloorHeights)
      ;[1 1 1] Set TargetHeight from list
      (Variables|Default|SetTargetHeight (Utilities|Array|Get(acopy) (Variables|Setup|GetFloorHeights) (- (Variables|Setup|GetTargetFloor) 1)))
      (else
        ;[1 1 1] Calculate TargetHeight
        (Variables|Default|SetTargetHeight (* (Math|Conversions|ToFloat(Integer) (Variables|Setup|GetTargetFloor)) (Variables|Setup|GetFloorHeight)))))
    ;[1 1 1] Spawn frame at this floor
    (bind _returnvalue_2 (Game|SpawnActorfromClass "/Game/ProceduralCity/Blueprints/Props/Elevators/BP_ElevatorFrame.BP_ElevatorFrame_C" (Math|Transform|MakeTransform (Math|Vector|MakeVector (.x _returnvalue) (.y _returnvalue) (Variables|Default|GetTargetHeight)) (Transformation|GetActorRotation)) "Undefined" 0 0))
    (LocalVariables|SetSpawnedFrame _returnvalue_2)
    ;[1 1 1] Set Parameters
    (Variables|/Game/ProceduralCity/Blueprints/Props/Elevators/BP_ElevatorFrame.BP_ElevatorFrame_C|SetCageRef (LocalVariables|GetSpawnedFrame) self)
    (Variables|/Game/ProceduralCity/Blueprints/Props/Elevators/BP_ElevatorFrame.BP_ElevatorFrame_C|SetOpenDoorDelay (LocalVariables|GetSpawnedFrame) (Variables|Setup|GetOpenDoorDelay))
    (Variables|/Game/ProceduralCity/Blueprints/Props/Elevators/BP_ElevatorFrame.BP_ElevatorFrame_C|SetTargetHeight (LocalVariables|GetSpawnedFrame) (Variables|Default|GetTargetHeight))
    ;[1 1 1] Add Frame to the list
    (Utilities|Array|Add (Variables|Default|GetFrameList) (LocalVariables|GetSpawnedFrame))))

(event Custom|EventOpenDoors
  (Utilities|FlowControl|Sequence
    (:then_0
      (bind _alpha (Timeline|TM_Open PlayFromStart)
        (:Update
          (Transformation|SetRelativeScale3D (Variables|Default|GetDoorRight) (Math|Vector|MakeVector 1.0 (Math|Float|Lerp 1.0 0.1 _alpha) 1.0))
          (Variables|Default|SetDoorOpen true))
        (:Finished
          ;[1 1 1] Wait OpenDoorDelay and if doors are still open, close them
          (Utilities|FlowControl|Delay (Variables|Setup|GetOpenDoorDelay))
          (if (Variables|Default|GetDoorOpen)
            (CallFunction|EventCloseDoors false)
            (Variables|Default|SetDoorOpen false)))))
    (:then_1
      ;[1 1 1] Open Frame Doors
      (Utilities|IsValid (Variables|Default|GetCurrentFrame)
        (:Is%20Valid
          (Default|EventOpenDoors (Variables|Default|GetCurrentFrame)))))))

(event Custom|EventCloseDoors
  (params (Move%20Elevator :type Boolean))
  (Variables|Default|SetCanMove Move%20Elevator)
  (Utilities|FlowControl|Sequence
    (:then_0
      (bind _alpha (Timeline|TM_Close PlayFromStart)
        (:Update
          (Transformation|SetRelativeScale3D (Variables|Default|GetDoorRight) (Math|Vector|MakeVector 1.0 (Math|Float|Lerp 0.1 1.0 _alpha) 1.0)))
        (:Finished
          (if (Variables|Default|GetCanMove)
            (Variables|Default|SetMoveElevator true)))))
    (:then_1
      ;[1 1 1] Close Frame Doors
      (Utilities|IsValid (Variables|Default|GetCurrentFrame)
        (:Is%20Valid
          (Default|EventCloseDoors (Variables|Default|GetCurrentFrame)))))))

(event Custom|EventShowMenu
  ;[1 1 1] Create HUD and set parameters
  (bind _returnvalue (UserInterface|CreateWidget "/Game/ProceduralCity/Blueprints/Widgets/WBP_ElevatorHUD.WBP_ElevatorHUD_C"))
  (bind _output_get (Variables|Default|SetHUD _returnvalue))
  (UserInterface|Viewport|AddtoPlayerScreen _output_get)
  (Default|FnSetOwner (Variables|Default|GetHUD) self)
  (Default|FnSetTotalFloors (Variables|Default|GetHUD) (Variables|Setup|GetTotalFloors))
  (Default|FnShowMenu (Variables|Default|GetHUD)))