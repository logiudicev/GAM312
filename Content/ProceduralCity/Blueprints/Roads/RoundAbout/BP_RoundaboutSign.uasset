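; BP_RoundaboutSign is a roundabout sign for the procedural city that displays a town name as in-world text between lamp components.
; Its construction script applies the name and text size, sets a configurable cull distance on the sign and a fixed one on the two lamps.
; FnSetNameSize repeats the text and size update so other code can change the displayed name.
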(fn ConstructionScript
  (Rendering|Components|TextRender|SetText (Variables|Default|GetName) (Variables|Setup|GetTownName))
  (Rendering|Components|TextRender|SetWorldSize (Variables|Default|GetName) (Variables|Setup|GetTextSize))
  ;[1 1 1] Set Max Draw Distance
  (Class|PrimitiveComponent|SetCullDistance (Variables|Default|GetSign) (Variables|Setup|GetMaxDrawDistance))
  (Class|PrimitiveComponent|SetCullDistance (Variables|Default|GetLampL) 5e+03))

(fn FnSetNameSize
  (params (Town%20Name :type Text) (Text%20Size :type Float%20%28single-precision%29))
  (Rendering|Components|TextRender|SetText (Variables|Default|GetName) Town%20Name)
  (Rendering|Components|TextRender|SetWorldSize (Variables|Default|GetName) Text%20Size))