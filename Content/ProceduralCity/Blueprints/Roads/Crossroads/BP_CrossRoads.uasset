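; BP_CrossRoads is a procedural-city crossroads piece: a scaled road plane with markings, stop signs and traffic lights.
; Its Construction Script sizes and dresses it from road type, line count and prop settings.
; SetDefaults applies per-type prop and line-style presets, then rebuilds through a near-copy of that logic.
; Optional traces beyond two-line ends strip markings and props on hitting non-road actors or crossroads, also calling SetDefaults on hit crossroads.
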(event Custom|Set%20Defaults
  (CallFunction|FnSetDefaults)
  (CallFunction|FnGenerateCrossroads)
  (CallFunction|FnCheckforRoads))

(event EventBeginPlay
  (CallFunction|FnSetDrawDistance))

(fn ConstructionScript
  (bind _stopsign_back (Variables|Default|GetStopSign_Back))
  (bind _trafficlight_front (Variables|Default|GetTrafficLight_Front))
  (bind _stopsign_front (Variables|Default|GetStopSign_Front))
  (bind _stopsign_front_2 (Variables|Default|GetStopSign_Front))
  (bind _relativelocation (Variables|/Script/Engine.SceneComponent|GetRelativeLocation _trafficlight_front))
  (bind _relativelocation_2 (Variables|/Script/Engine.SceneComponent|GetRelativeLocation _stopsign_front))
  (bind _relativelocation_3 (Variables|/Script/Engine.SceneComponent|GetRelativeLocation _stopsign_back))
  (bind _relativelocation_4 (Variables|/Script/Engine.SceneComponent|GetRelativeLocation _stopsign_front_2))
  (CallFunction|FnSetDrawDistance)
  (Utilities|FlowControl|Sequence
    (:then_0
      ;[1 1 1] Set Plane material
      (Rendering|Material|SetMaterial (Variables|Default|GetPlane) 0 (Variables|Setup|GetBaseMaterial))
      (Utilities|FlowControl|Sequence
        (:then_0
          (switch Utilities|FlowControl|Switch|SwitchonEnum_RoadType (Variables|Setup|GetRoadType)
            (:NewEnumerator0
              (Variables|Default|SetRoadIndex 0)
              (if (Variables|Setup|GetShowMarkings)
                (if (not (Variables|Setup|GetCurvedMesh?))
                  ;[1 1 1] Set correct static mesh for the markings
                  (Components|StaticMesh|SetStaticMesh (Variables|Default|GetRoadMarks_Front) "/Game/ProceduralCity/Meshes/Roads/ModularRoads/SM_CrossRoads_Highway.SM_CrossRoads_Highway")
                  (Components|StaticMesh|SetStaticMesh (Variables|Default|GetRoadMarks_Back) "/Game/ProceduralCity/Meshes/Roads/ModularRoads/SM_CrossRoads_Highway.SM_CrossRoads_Highway")
                  (else
                    ;[1 1 1] Set correct static mesh for the markings
                    (Components|StaticMesh|SetStaticMesh (Variables|Default|GetRoadMarks_Front) "/Game/ProceduralCity/Meshes/Roads/RoundAbout/SM_CrossRoads_Bent_Big_Highway.SM_CrossRoads_Bent_Big_Highway")
                    (Components|StaticMesh|SetStaticMesh (Variables|Default|GetRoadMarks_Back) "/Game/ProceduralCity/Meshes/Roads/RoundAbout/SM_CrossRoads_Bent_Big_Highway.SM_CrossRoads_Bent_Big_Highway")))
                ;[1 1 1] Set correct location for road markings
                (Transformation|SetRelativeLocation (Variables|Default|GetRoadMarks_Front) (Math|Vector|MakeVector (.x (Variables|/Script/Engine.SceneComponent|GetRelativeLocation (Variables|Default|GetAnchor_Front))) 0.0 0.0) false true)
                (Transformation|SetRelativeLocation (Variables|Default|GetRoadMarks_Back) (Math|Vector|MakeVector (.x (Variables|/Script/Engine.SceneComponent|GetRelativeLocation (Variables|Default|GetAnchor_Back))) 0.0 0.0) false true)))
            (:NewEnumerator1
              (Variables|Default|SetRoadIndex 1)
              (if (Variables|Setup|GetShowMarkings)
                (if (not (Variables|Setup|GetCurvedMesh?))
                  ;[1 1 1] Set correct static mesh for the markings
                  (Components|StaticMesh|SetStaticMesh (Variables|Default|GetRoadMarks_Front) "/Game/ProceduralCity/Meshes/Roads/ModularRoads/SM_CrossRoads_Main.SM_CrossRoads_Main")
                  (Components|StaticMesh|SetStaticMesh (Variables|Default|GetRoadMarks_Back) "/Game/ProceduralCity/Meshes/Roads/ModularRoads/SM_CrossRoads_Main.SM_CrossRoads_Main")
                  (else
                    ;[1 1 1] Set correct static mesh for the markings
                    (Components|StaticMesh|SetStaticMesh (Variables|Default|GetRoadMarks_Front) "/Game/ProceduralCity/Meshes/Roads/RoundAbout/SM_CrossRoads_Bent_Big_Main.SM_CrossRoads_Bent_Big_Main")
                    (Components|StaticMesh|SetStaticMesh (Variables|Default|GetRoadMarks_Back) "/Game/ProceduralCity/Meshes/Roads/RoundAbout/SM_CrossRoads_Bent_Big_Main.SM_CrossRoads_Bent_Big_Main")))
                ;[1 1 1] Set correct location for road markings
                (Transformation|SetRelativeLocation (Variables|Default|GetRoadMarks_Front) (Math|Vector|MakeVector (.x (Variables|/Script/Engine.SceneComponent|GetRelativeLocation (Variables|Default|GetAnchor_Front))) 0.0 0.0) false true)
                (Transformation|SetRelativeLocation (Variables|Default|GetRoadMarks_Back) (Math|Vector|MakeVector (.x (Variables|/Script/Engine.SceneComponent|GetRelativeLocation (Variables|Default|GetAnchor_Back))) 0.0 0.0) false true)))
            (:NewEnumerator2
              (Variables|Default|SetRoadIndex 2)
              (if (Variables|Setup|GetShowMarkings)
                ;[1 1 1] Set correct static mesh for the markings
                (Components|StaticMesh|SetStaticMesh (Variables|Default|GetRoadMarks_Front) "/Game/ProceduralCity/Meshes/Roads/ModularRoads/SM_CrossRoads_Minor.SM_CrossRoads_Minor")
                (Components|StaticMesh|SetStaticMesh (Variables|Default|GetRoadMarks_Back) "/Game/ProceduralCity/Meshes/Roads/ModularRoads/SM_CrossRoads_Minor.SM_CrossRoads_Minor")
                ;[1 1 1] Set correct location for road markings
                (Transformation|SetRelativeLocation (Variables|Default|GetRoadMarks_Front) (Math|Vector|MakeVector (.x (Variables|/Script/Engine.SceneComponent|GetRelativeLocation (Variables|Default|GetAnchor_Front))) 0.0 0.0) false true)
                (Transformation|SetRelativeLocation (Variables|Default|GetRoadMarks_Back) (Math|Vector|MakeVector (.x (Variables|/Script/Engine.SceneComponent|GetRelativeLocation (Variables|Default|GetAnchor_Back))) 0.0 0.0) false true)))
            (:NewEnumerator3
              (Variables|Default|SetRoadIndex 3)
              (if (Variables|Setup|GetShowMarkings)
                ;[1 1 1] Set correct static mesh for the markings
                (Components|StaticMesh|SetStaticMesh (Variables|Default|GetRoadMarks_Front) "/Game/ProceduralCity/Meshes/Roads/ModularRoads/SM_CrossRoads_Side.SM_CrossRoads_Side")
                (Components|StaticMesh|SetStaticMesh (Variables|Default|GetRoadMarks_Back) "/Game/ProceduralCity/Meshes/Roads/ModularRoads/SM_CrossRoads_Side.SM_CrossRoads_Side")
                ;[1 1 1] Set correct location for road markings
                (Transformation|SetRelativeLocation (Variables|Default|GetRoadMarks_Front) (Math|Vector|MakeVector (.x (Variables|/Script/Engine.SceneComponent|GetRelativeLocation (Variables|Default|GetAnchor_Front))) 0.0 0.0) false true)
                (Transformation|SetRelativeLocation (Variables|Default|GetRoadMarks_Back) (Math|Vector|MakeVector (.x (Variables|/Script/Engine.SceneComponent|GetRelativeLocation (Variables|Default|GetAnchor_Back))) 0.0 0.0) false true)))))
        (:then_1
          (|SETSCALES))
        (:then_2
          (Rendering|SetVisibility (Variables|Default|GetPlane) (Variables|Setup|GetShowMiddle) false))))
    (:then_1
      (switch Utilities|FlowControl|Switch|SwitchonEnum_CrossRoads_Lines (Variables|Setup|GetLines)
        (:NewEnumerator0
          ;[1 1 1] Hide the back line and center the front line
          (Rendering|SetVisibility (Variables|Default|GetRoadMarks_Back) false false)
          (Transformation|SetRelativeLocation (Variables|Default|GetRoadMarks_Front) "-20.000000, 0,1.000000" false true)
          (Utilities|FlowControl|Sequence
            (:then_0
              ;[1 1 1] Do we add Stop Signs?
              (if (Variables|Setup|GetAddStopSign)
                ;[1 1 1] Set the actor class and the scale
                (ChildActorComponent|SetChildActorClass (Variables|Default|GetStopSign_Front) "/Game/ProceduralCity/Blueprints/Props/Roads/BP_StopSign.BP_StopSign_C")
                (Transformation|SetWorldScale3D (Variables|Default|GetStopSign_Front) "1.000000,1.000000,1.000000")
                ;[1 1 1] Set location
                (Transformation|SetRelativeLocation _stopsign_front (Math|Vector|MakeVector 0.0 (.y _relativelocation_2) (.z _relativelocation_2)) false true)
                (else
                  (ChildActorComponent|SetChildActorClass (Variables|Default|GetStopSign_Front) 0))))
            (:then_1
              ;[1 1 1] Do we add traffic lights?
              (if (Variables|Setup|GetAddTrafficLight)
                ;[1 1 1] Set location and scale
                (Transformation|SetWorldScale3D (Variables|Default|GetTrafficLight_Front) "1.000000,1.000000,1.000000")
                (Transformation|SetRelativeLocation _trafficlight_front (Math|Vector|MakeVector 0.0 (.y _relativelocation) (.z _relativelocation)) false true)
                (switch Utilities|FlowControl|Switch|SwitchonEnum_TrafficLightType (Variables|Setup|GetLightType)
                  (:NewEnumerator0
                    (ChildActorComponent|SetChildActorClass (Variables|Default|GetTrafficLight_Front) "/Game/ProceduralCity/Blueprints/Props/Roads/BP_StopLightSmall.BP_StopLightSmall_C"))
                  (:NewEnumerator1
                    (ChildActorComponent|SetChildActorClass (Variables|Default|GetTrafficLight_Front) "/Game/ProceduralCity/Blueprints/Props/Roads/BP_StopLightBig.BP_StopLightBig_C")))
                (else
                  (ChildActorComponent|SetChildActorClass (Variables|Default|GetTrafficLight_Front) 0)
                  (ChildActorComponent|SetChildActorClass (Variables|Default|GetTrafficLight_Front) 0))))))
        (:NewEnumerator1
          (Utilities|FlowControl|Sequence
            (:then_0
              ;[1 1 1] Do we add Stop Signs?
              (if (Variables|Setup|GetAddStopSign)
                ;[1 1 1] Set the actor class and the scale
                (ChildActorComponent|SetChildActorClass (Variables|Default|GetStopSign_Front) "/Game/ProceduralCity/Blueprints/Props/Roads/BP_StopSign.BP_StopSign_C")
                (Transformation|SetWorldScale3D (Variables|Default|GetStopSign_Front) "1.000000,1.000000,1.000000")
                ;[1 1 1] Set the correct location
                (Transformation|SetRelativeLocation _stopsign_front_2 (Math|Vector|MakeVector (.x (Variables|/Script/Engine.SceneComponent|GetRelativeLocation (Variables|Default|GetAnchor_Front))) (.y _relativelocation_4) (.z _relativelocation_4)) false true)
                (Transformation|SetRelativeLocation _stopsign_back (Math|Vector|MakeVector (.x (Variables|/Script/Engine.SceneComponent|GetRelativeLocation (Variables|Default|GetAnchor_Back))) (.y _relativelocation_3) (.z _relativelocation_3)) false true)
                (else
                  (ChildActorComponent|SetChildActorClass (Variables|Default|GetStopSign_Front) 0))))
            (:then_1
              ;[1 1 1] Do we add traffic lights?
              (if (Variables|Setup|GetAddTrafficLight)
                (Transformation|SetWorldScale3D (Variables|Default|GetTrafficLight_Front) "1.000000,1.000000,1.000000")
                (switch Utilities|FlowControl|Switch|SwitchonEnum_TrafficLightType (Variables|Setup|GetLightType)
                  (:NewEnumerator0
                    (ChildActorComponent|SetChildActorClass (Variables|Default|GetTrafficLight_Front) "/Game/ProceduralCity/Blueprints/Props/Roads/BP_StopLightSmall.BP_StopLightSmall_C"))
                  (:NewEnumerator1
                    (ChildActorComponent|SetChildActorClass (Variables|Default|GetTrafficLight_Front) "/Game/ProceduralCity/Blueprints/Props/Roads/BP_StopLightBig.BP_StopLightBig_C")))
                (else
                  (ChildActorComponent|SetChildActorClass (Variables|Default|GetTrafficLight_Front) 0)
                  (ChildActorComponent|SetChildActorClass (Variables|Default|GetTrafficLight_Front) 0))))))))
    (:then_2
      (CallFunction|FnSetLineStyle))
    (:then_3
      (CallFunction|FnCheckforRoads))))

(fn FnSetDefaults
  ;[1 1 1] Switch on Road Type
  (switch Utilities|FlowControl|Switch|SwitchonEnum_RoadType (Variables|Setup|GetRoadType)
    (:NewEnumerator0
      (Variables|Setup|SetAddStopSign false)
      (Variables|Setup|SetAddTrafficLight true)
      (Variables|Setup|SetLightType "NewEnumerator1")
      (Variables|Setup|SetLineStyle "NewEnumerator1"))
    (:NewEnumerator1
      (Variables|Setup|SetAddStopSign false)
      (Variables|Setup|SetAddTrafficLight true)
      (Variables|Setup|SetLightType "NewEnumerator1")
      (Variables|Setup|SetLineStyle "NewEnumerator1"))
    (:NewEnumerator2
      (Variables|Setup|SetAddStopSign false)
      (Variables|Setup|SetAddTrafficLight true)
      (Variables|Setup|SetLightType "NewEnumerator0")
      (Variables|Setup|SetLineStyle "NewEnumerator0"))
    (:NewEnumerator3
      (Variables|Setup|SetAddStopSign true)
      (Variables|Setup|SetAddTrafficLight false)
      (Variables|Setup|SetLightType "NewEnumerator0")
      (Variables|Setup|SetLineStyle "NewEnumerator0"))))

(fn FnGenerateCrossroads
  (bind _stopsign_back (Variables|Default|GetStopSign_Back))
  (bind _trafficlight_front (Variables|Default|GetTrafficLight_Front))
  (bind _stopsign_front (Variables|Default|GetStopSign_Front))
  (bind _stopsign_front_2 (Variables|Default|GetStopSign_Front))
  (bind _relativelocation (Variables|/Script/Engine.SceneComponent|GetRelativeLocation _trafficlight_front))
  (bind _relativelocation_2 (Variables|/Script/Engine.SceneComponent|GetRelativeLocation _stopsign_front))
  (bind _relativelocation_3 (Variables|/Script/Engine.SceneComponent|GetRelativeLocation _stopsign_back))
  (bind _relativelocation_4 (Variables|/Script/Engine.SceneComponent|GetRelativeLocation _stopsign_front_2))
  (CallFunction|FnSetDrawDistance)
  (Utilities|FlowControl|Sequence
    (:then_0
      ;[1 1 1] Set Plane material
      (Rendering|Material|SetMaterial (Variables|Default|GetPlane) 0 (Variables|Setup|GetBaseMaterial))
      (Utilities|FlowControl|Sequence
        (:then_0
          (switch Utilities|FlowControl|Switch|SwitchonEnum_RoadType (Variables|Setup|GetRoadType)
            (:NewEnumerator0
              (Variables|Default|SetRoadIndex 0)
              (if (Variables|Setup|GetShowMarkings)
                (if (not (Variables|Setup|GetCurvedMesh?))
                  ;[1 1 1] Set correct static mesh for the markings
                  (Components|StaticMesh|SetStaticMesh (Variables|Default|GetRoadMarks_Front) "/Game/ProceduralCity/Meshes/Roads/ModularRoads/SM_CrossRoads_Highway.SM_CrossRoads_Highway")
                  (Components|StaticMesh|SetStaticMesh (Variables|Default|GetRoadMarks_Back) "/Game/ProceduralCity/Meshes/Roads/ModularRoads/SM_CrossRoads_Highway.SM_CrossRoads_Highway")
                  (else
                    ;[1 1 1] Set correct static mesh for the markings
                    (Components|StaticMesh|SetStaticMesh (Variables|Default|GetRoadMarks_Front) "/Game/ProceduralCity/Meshes/Roads/RoundAbout/SM_CrossRoadsBent_Small_Highway.SM_CrossRoadsBent_Small_Highway")
                    (Components|StaticMesh|SetStaticMesh (Variables|Default|GetRoadMarks_Back) "/Game/ProceduralCity/Meshes/Roads/RoundAbout/SM_CrossRoadsBent_Small_Highway.SM_CrossRoadsBent_Small_Highway")))
                ;[1 1 1] Set correct location for road markings
                (Transformation|SetRelativeLocation (Variables|Default|GetRoadMarks_Front) (Math|Vector|MakeVector (.x (Variables|/Script/Engine.SceneComponent|GetRelativeLocation (Variables|Default|GetAnchor_Front))) 0.0 0.0) false true)
                (Transformation|SetRelativeLocation (Variables|Default|GetRoadMarks_Back) (Math|Vector|MakeVector (.x (Variables|/Script/Engine.SceneComponent|GetRelativeLocation (Variables|Default|GetAnchor_Back))) 0.0 0.0) false true)))
            (:NewEnumerator1
              (Variables|Default|SetRoadIndex 1)
              (if (Variables|Setup|GetShowMarkings)
                (if (not (Variables|Setup|GetCurvedMesh?))
                  ;[1 1 1] Set correct static mesh for the markings
                  (Components|StaticMesh|SetStaticMesh (Variables|Default|GetRoadMarks_Front) "/Game/ProceduralCity/Meshes/Roads/ModularRoads/SM_CrossRoads_Main.SM_CrossRoads_Main")
                  (Components|StaticMesh|SetStaticMesh (Variables|Default|GetRoadMarks_Back) "/Game/ProceduralCity/Meshes/Roads/ModularRoads/SM_CrossRoads_Main.SM_CrossRoads_Main")
                  (else
                    ;[1 1 1] Set correct static mesh for the markings
                    (Components|StaticMesh|SetStaticMesh (Variables|Default|GetRoadMarks_Front) "/Game/ProceduralCity/Meshes/Roads/RoundAbout/SM_CrossRoads_Bent_Big_Main.SM_CrossRoads_Bent_Big_Main")
                    (Components|StaticMesh|SetStaticMesh (Variables|Default|GetRoadMarks_Back) "/Game/ProceduralCity/Meshes/Roads/RoundAbout/SM_CrossRoads_Bent_Big_Main.SM_CrossRoads_Bent_Big_Main")))
                ;[1 1 1] Set correct location for road markings
                (Transformation|SetRelativeLocation (Variables|Default|GetRoadMarks_Front) (Math|Vector|MakeVector (.x (Variables|/Script/Engine.SceneComponent|GetRelativeLocation (Variables|Default|GetAnchor_Front))) 0.0 0.0) false true)
                (Transformation|SetRelativeLocation (Variables|Default|GetRoadMarks_Back) (Math|Vector|MakeVector (.x (Variables|/Script/Engine.SceneComponent|GetRelativeLocation (Variables|Default|GetAnchor_Back))) 0.0 0.0) false true)))
            (:NewEnumerator2
              (Variables|Default|SetRoadIndex 2)
              (if (Variables|Setup|GetShowMarkings)
                ;[1 1 1] Set correct static mesh for the markings
                (Components|StaticMesh|SetStaticMesh (Variables|Default|GetRoadMarks_Front) "/Game/ProceduralCity/Meshes/Roads/ModularRoads/SM_CrossRoads_Minor.SM_CrossRoads_Minor")
                (Components|StaticMesh|SetStaticMesh (Variables|Default|GetRoadMarks_Back) "/Game/ProceduralCity/Meshes/Roads/ModularRoads/SM_CrossRoads_Minor.SM_CrossRoads_Minor")
                ;[1 1 1] Set correct location for road markings
                (Transformation|SetRelativeLocation (Variables|Default|GetRoadMarks_Front) (Math|Vector|MakeVector (.x (Variables|/Script/Engine.SceneComponent|GetRelativeLocation (Variables|Default|GetAnchor_Front))) 0.0 0.0) false true)
                (Transformation|SetRelativeLocation (Variables|Default|GetRoadMarks_Back) (Math|Vector|MakeVector (.x (Variables|/Script/Engine.SceneComponent|GetRelativeLocation (Variables|Default|GetAnchor_Back))) 0.0 0.0) false true)))
            (:NewEnumerator3
              (Variables|Default|SetRoadIndex 3)
              (if (Variables|Setup|GetShowMarkings)
                ;[1 1 1] Set correct static mesh for the markings
                (Components|StaticMesh|SetStaticMesh (Variables|Default|GetRoadMarks_Front) "/Game/ProceduralCity/Meshes/Roads/ModularRoads/SM_CrossRoads_Side.SM_CrossRoads_Side")
                (Components|StaticMesh|SetStaticMesh (Variables|Default|GetRoadMarks_Back) "/Game/ProceduralCity/Meshes/Roads/ModularRoads/SM_CrossRoads_Side.SM_CrossRoads_Side")
                ;[1 1 1] Set correct location for road markings
                (Transformation|SetRelativeLocation (Variables|Default|GetRoadMarks_Front) (Math|Vector|MakeVector (.x (Variables|/Script/Engine.SceneComponent|GetRelativeLocation (Variables|Default|GetAnchor_Front))) 0.0 0.0) false true)
                (Transformation|SetRelativeLocation (Variables|Default|GetRoadMarks_Back) (Math|Vector|MakeVector (.x (Variables|/Script/Engine.SceneComponent|GetRelativeLocation (Variables|Default|GetAnchor_Back))) 0.0 0.0) false true)))))
        (:then_1
          (|SETSCALES_2))
        (:then_2
          (Rendering|SetVisibility (Variables|Default|GetPlane) (Variables|Setup|GetShowMiddle) false))))
    (:then_1
      (switch Utilities|FlowControl|Switch|SwitchonEnum_CrossRoads_Lines (Variables|Setup|GetLines)
        (:NewEnumerator0
          ;[1 1 1] Hide the back line and center the front line
          (Rendering|SetVisibility (Variables|Default|GetRoadMarks_Back) false false)
          (Transformation|SetRelativeLocation (Variables|Default|GetRoadMarks_Front) "-20.000000, 0,1.000000" false true)
          (Utilities|FlowControl|Sequence
            (:then_0
              ;[1 1 1] Do we add Stop Signs?
              (if (Variables|Setup|GetAddStopSign)
                ;[1 1 1] Set the actor class and the scale
                (ChildActorComponent|SetChildActorClass (Variables|Default|GetStopSign_Front) "/Game/ProceduralCity/Blueprints/Props/Roads/BP_StopSign.BP_StopSign_C")
                (Transformation|SetWorldScale3D (Variables|Default|GetStopSign_Front) "1.000000,1.000000,1.000000")
                ;[1 1 1] Set location
                (Transformation|SetRelativeLocation _stopsign_front (Math|Vector|MakeVector 0.0 (.y _relativelocation_2) (.z _relativelocation_2)) false true)
                (else
                  (ChildActorComponent|SetChildActorClass (Variables|Default|GetStopSign_Front) 0))))
            (:then_1
              ;[1 1 1] Do we add traffic lights?
              (if (Variables|Setup|GetAddTrafficLight)
                ;[1 1 1] Set location and scale
                (Transformation|SetWorldScale3D (Variables|Default|GetTrafficLight_Front) "1.000000,1.000000,1.000000")
                (Transformation|SetRelativeLocation _trafficlight_front (Math|Vector|MakeVector 0.0 (.y _relativelocation) (.z _relativelocation)) false true)
                (switch Utilities|FlowControl|Switch|SwitchonEnum_TrafficLightType (Variables|Setup|GetLightType)
                  (:NewEnumerator0
                    (ChildActorComponent|SetChildActorClass (Variables|Default|GetTrafficLight_Front) "/Game/ProceduralCity/Blueprints/Props/Roads/BP_StopLightSmall.BP_StopLightSmall_C"))
                  (:NewEnumerator1
                    (ChildActorComponent|SetChildActorClass (Variables|Default|GetTrafficLight_Front) "/Game/ProceduralCity/Blueprints/Props/Roads/BP_StopLightBig.BP_StopLightBig_C")))
                (else
                  (ChildActorComponent|SetChildActorClass (Variables|Default|GetTrafficLight_Front) 0)
                  (ChildActorComponent|SetChildActorClass (Variables|Default|GetTrafficLight_Front) 0))))))
        (:NewEnumerator1
          (Utilities|FlowControl|Sequence
            (:then_0
              ;[1 1 1] Do we add Stop Signs?
              (if (Variables|Setup|GetAddStopSign)
                ;[1 1 1] Set the actor class and the scale
                (ChildActorComponent|SetChildActorClass (Variables|Default|GetStopSign_Front) "/Game/ProceduralCity/Blueprints/Props/Roads/BP_StopSign.BP_StopSign_C")
                (Transformation|SetWorldScale3D (Variables|Default|GetStopSign_Front) "1.000000,1.000000,1.000000")
                ;[1 1 1] Set the correct location
                (Transformation|SetRelativeLocation _stopsign_front_2 (Math|Vector|MakeVector (.x (Variables|/Script/Engine.SceneComponent|GetRelativeLocation (Variables|Default|GetAnchor_Front))) (.y _relativelocation_4) (.z _relativelocation_4)) false true)
                (Transformation|SetRelativeLocation _stopsign_back (Math|Vector|MakeVector (.x (Variables|/Script/Engine.SceneComponent|GetRelativeLocation (Variables|Default|GetAnchor_Back))) (.y _relativelocation_3) (.z _relativelocation_3)) false true)
                (else
                  (ChildActorComponent|SetChildActorClass (Variables|Default|GetStopSign_Front) 0))))
            (:then_1
              ;[1 1 1] Do we add traffic lights?
              (if (Variables|Setup|GetAddTrafficLight)
                (Transformation|SetWorldScale3D (Variables|Default|GetTrafficLight_Front) "1.000000,1.000000,1.000000")
                (switch Utilities|FlowControl|Switch|SwitchonEnum_TrafficLightType (Variables|Setup|GetLightType)
                  (:NewEnumerator0
                    (ChildActorComponent|SetChildActorClass (Variables|Default|GetTrafficLight_Front) "/Game/ProceduralCity/Blueprints/Props/Roads/BP_StopLightSmall.BP_StopLightSmall_C"))
                  (:NewEnumerator1
                    (ChildActorComponent|SetChildActorClass (Variables|Default|GetTrafficLight_Front) "/Game/ProceduralCity/Blueprints/Props/Roads/BP_StopLightBig.BP_StopLightBig_C")))
                (else
                  (ChildActorComponent|SetChildActorClass (Variables|Default|GetTrafficLight_Front) 0)
                  (ChildActorComponent|SetChildActorClass (Variables|Default|GetTrafficLight_Front) 0))))))))
    (:then_2
      (CallFunction|FnSetLineStyle))
    (:then_3
      (CallFunction|FnCheckforRoads))))

(fn FnSetDrawDistance
  ;[1 1 1] Set Max Draw Distance
  (Class|PrimitiveComponent|SetCullDistance (Variables|Default|GetPlane) (Variables|Setup|GetMaxDrawDistance)))

(fn FnCheckforRoads
  (bind _roadmarks_back (Variables|Default|GetRoadMarks_Back))
  (bind _roadmarks_front (Variables|Default|GetRoadMarks_Front))
  (bind _returnvalue (Transformation|GetWorldRotation _roadmarks_back))
  (bind _returnvalue_2 (Transformation|GetWorldLocation _roadmarks_front))
  (bind _returnvalue_3 (Transformation|GetWorldRotation _roadmarks_front))
  (bind _returnvalue_4 (Transformation|GetWorldLocation _roadmarks_back))
  (bind _returnvalue_5 (Math|Vector|GetForwardVector _returnvalue))
  (bind _returnvalue_6 (Math|Vector|GetForwardVector _returnvalue_3))
  (bind _returnvalue_7 (* _returnvalue_5 4e+02))
  (bind _returnvalue_8 (* _returnvalue_6 4e+02))
  (bind _returnvalue_9 (+ _returnvalue_4 _returnvalue_7))
  (bind _returnvalue_10 (+ _returnvalue_2 _returnvalue_8))
  (if (Variables|Setup|GetCheckForRoads)
    ;[1 1 1] Are we displaying 2 lines?
    (if (Utilities|Enum|Equal(Enum) (Variables|Setup|GetLines) "NewEnumerator1")
      (Utilities|FlowControl|Sequence
        (:then_0
          ;[1 1 1] Trace on the front road marks
          (bind (_outhit _returnvalue_11) (Collision|LineTraceByChannel (+ _returnvalue_10 (Math|Vector|MakeVector 0.0 0.0 1e+04)) (- _returnvalue_10 (Math|Vector|MakeVector 0.0 0.0 1e+04)) "TraceTypeQuery1" false 0 "None"))
          (if _returnvalue_11
            (Utilities|FlowControl|Sequence
              (:then_0
                ;[1 1 1] Is the hit actor another road?
                (Utilities|Casting|CastToBP_GenericRoad_Base (.HitActor (Collision|BreakHitResult _outhit))
                  (:CastFailed
                    (LocalVariables|SetHideFront true))))
              (:then_1
                ;[1 1 1] Is the hit actor another crossroad?
                (bind _asbp_cross_roads (Utilities|Casting|CastToBP_CrossRoads (.HitActor (Collision|BreakHitResult _outhit))))
                (CallFunction|SetDefaults _asbp_cross_roads)
                (LocalVariables|SetHideFront true))
              (:then_2
                (if (LocalVariables|GetHideFront)
                  ;[1 1 1] Hide markings and props on the front
                  (Components|StaticMesh|SetStaticMesh (Variables|Default|GetRoadMarks_Front) 0)
                  (ChildActorComponent|SetChildActorClass (Variables|Default|GetStopSign_Front) 0)
                  (ChildActorComponent|SetChildActorClass (Variables|Default|GetTrafficLight_Front) 0))))))
        (:then_1
          ;[1 1 1] Trace on the back road marks
          (bind (_outhit_2 _returnvalue_12) (Collision|LineTraceByChannel (+ _returnvalue_9 (Math|Vector|MakeVector 0.0 0.0 1e+04)) (- _returnvalue_9 (Math|Vector|MakeVector 0.0 0.0 1e+04)) "TraceTypeQuery1" false 0 "None"))
          (if _returnvalue_12
            (Utilities|FlowControl|Sequence
              (:then_0
                ;[1 1 1] Is the hit actor another road?
                (Utilities|Casting|CastToBP_GenericRoad_Base (.HitActor (Collision|BreakHitResult _outhit_2))
                  (:CastFailed
                    (LocalVariables|SetHideBack true))))
              (:then_1
                ;[1 1 1] Is the hit actor another crossroad?
                (bind _asbp_cross_roads_2 (Utilities|Casting|CastToBP_CrossRoads (.HitActor (Collision|BreakHitResult _outhit_2))))
                (CallFunction|SetDefaults _asbp_cross_roads_2)
                (LocalVariables|SetHideBack true))
              (:then_2
                (if (LocalVariables|GetHideBack)
                  ;[1 1 1] Hide markings and props on the back
                  (Components|StaticMesh|SetStaticMesh (Variables|Default|GetRoadMarks_Back) 0)
                  (ChildActorComponent|SetChildActorClass (Variables|Default|GetStopSign_Back) 0)
                  (ChildActorComponent|SetChildActorClass (Variables|Default|GetTrafficLight_Back) 0))))))))))

(fn FnSetLineStyle
  ;[1 1 1] Switch on LineStyle
  (switch Utilities|FlowControl|Switch|SwitchonEnum_CrossRoads_LineStyle (Variables|Setup|GetLineStyle)
    (:NewEnumerator0
      (Rendering|Material|SetMaterial (Variables|Default|GetRoadMarks_Front) 0 "/Game/ProceduralCity/Materials/Roads/MI_Road_Standard.MI_Road_Standard"))
    (:NewEnumerator1
      (Rendering|Material|SetMaterial (Variables|Default|GetRoadMarks_Front) 0 "/Game/ProceduralCity/Materials/Roads/MI_Road_Style2.MI_Road_Style2"))))