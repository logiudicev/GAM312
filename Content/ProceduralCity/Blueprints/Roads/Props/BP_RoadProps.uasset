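; Spline-based road prop actor for the procedural city that lines a spline with repeated meshes of a selected prop type.
; FnSpawnProps looks up the type in PropDetails, then places spline mesh components at intervals of mesh length plus spacing, with a cull distance.
; The last segment either stretches to the final spline point or is destroyed, per StretchMeshes.
; It runs from construction, which then applies CloseLoop, or the SpawnProps event.
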(event Custom|Spawn%20Props
  (CallFunction|FnSpawnProps))

(fn ConstructionScript
  (CallFunction|FnSpawnProps)
  (Spline|SetClosedLoop (Variables|Default|GetSpline) (Variables|Setup|GetCloseLoop) true))

(fn FnSpawnProps
  (bind _spline (Variables|Default|GetSpline))
  (bind _spline_2 (Variables|Default|GetSpline))
  (bind _spline_3 (Variables|Default|GetSpline))
  (bind _spline_4 (Variables|Default|GetSpline))
  (bind _returnvalue (Spline|GetNumberOfSplinePoints _spline_3))
  (bind _returnvalue_2 (- _returnvalue 1))
  ;[1 1 1] Loop through prop list
  (bind _array_element (Utilities|Array|ForEachLoopwithBreak (Variables|Setup|GetPropDetails) :!label _label)
    (:LoopBody
      (LocalVariables|SetProp _array_element)
      ;[1 1 1] Is the the correct prop?
      (if (Utilities|Enum|Equal(Enum) (Variables|Setup|GetPropType) (Utilities|Struct|BreakStruct_RoadProps_Props (LocalVariables|GetProp)))
        (goto _label Break)))
    (:Completed
      ;[1 1 1] Get Mesh length
      (LocalVariables|SetMeshLength (.X (Math|Vector|BreakVector (Utilities|Struct|BreakStruct_RoadProps_Props (LocalVariables|GetProp)))))
      ;[1 1 1] Calculate Total Props to spawn based on the road width
      (LocalVariables|SetTotalProps (.ReturnValue (Math|Float|Division(WholeandRemainder) (Spline|GetSplineLength (Variables|Default|GetSpline)) (+ (LocalVariables|GetMeshLength) (Utilities|Struct|BreakStruct_RoadProps_Props (LocalVariables|GetProp))))))
      ;[1 1 1] Loop through all props
      (for _index (range 0 (- (LocalVariables|GetTotalProps) 1))
        (LocalVariables|SetIndex _index)
        ;[1 1 1] Create new mesh
        (bind _returnvalue_3 (AddComponent|AddSplineMeshComponent false))
        (LocalVariables|SetSplineMeshComponent _returnvalue_3)
        (Components|StaticMesh|SetStaticMesh (LocalVariables|GetSplineMeshComponent) (Utilities|Struct|BreakStruct_RoadProps_Props (LocalVariables|GetProp)))
        (Class|PrimitiveComponent|SetCullDistance (LocalVariables|GetSplineMeshComponent) (Variables|Setup|GetMaxDrawDistance))
        (Transformation|AttachComponentToComponent (LocalVariables|GetSplineMeshComponent) (Variables|Default|GetDefaultSceneRoot) "None" "KeepRelative" "KeepRelative" "KeepRelative" true)
        (if (!= (LocalVariables|GetIndex) (- (LocalVariables|GetTotalProps) 1))
          ;[1 1 1] Set Start and End of mesh
          (SplineMesh|SetStartandEnd (LocalVariables|GetSplineMeshComponent) (Spline|GetLocationatDistanceAlongSpline _spline (* (LocalVariables|GetIndex) (+ (LocalVariables|GetMeshLength) (.Spacing (Utilities|Struct|BreakStruct_RoadProps_Props (LocalVariables|GetProp))))) "Local") (* (Spline|GetDirectionatDistanceAlongSpline _spline (* (LocalVariables|GetIndex) (+ (LocalVariables|GetMeshLength) (.Spacing (Utilities|Struct|BreakStruct_RoadProps_Props (LocalVariables|GetProp))))) "Local") (.TangentLength (Utilities|Struct|BreakStruct_RoadProps_Props (LocalVariables|GetProp)))) (Spline|GetLocationatDistanceAlongSpline _spline_2 (+ (* (LocalVariables|GetIndex) (+ (LocalVariables|GetMeshLength) (.Spacing (Utilities|Struct|BreakStruct_RoadProps_Props (LocalVariables|GetProp))))) (LocalVariables|GetMeshLength)) "Local") (* (Spline|GetDirectionatDistanceAlongSpline _spline_2 (+ (* (LocalVariables|GetIndex) (+ (LocalVariables|GetMeshLength) (.Spacing (Utilities|Struct|BreakStruct_RoadProps_Props (LocalVariables|GetProp))))) (LocalVariables|GetMeshLength)) "Local") (.TangentLength (Utilities|Struct|BreakStruct_RoadProps_Props (LocalVariables|GetProp)))) true :!class /Script/Engine.SplineMeshComponent)
          (elif (Variables|Setup|GetStretchMeshes)
            (SplineMesh|SetStartandEnd (LocalVariables|GetSplineMeshComponent) (Spline|GetLocationatDistanceAlongSpline _spline (* (LocalVariables|GetIndex) (+ (LocalVariables|GetMeshLength) (.Spacing (Utilities|Struct|BreakStruct_RoadProps_Props (LocalVariables|GetProp))))) "Local") (* (Spline|GetDirectionatDistanceAlongSpline _spline (* (LocalVariables|GetIndex) (+ (LocalVariables|GetMeshLength) (.Spacing (Utilities|Struct|BreakStruct_RoadProps_Props (LocalVariables|GetProp))))) "Local") (.TangentLength (Utilities|Struct|BreakStruct_RoadProps_Props (LocalVariables|GetProp)))) (Spline|GetLocationatSplinePoint _spline_4 _returnvalue_2 "Local") (* (Class|SplineComponent|GetDirectionatSplinePoint _spline_4 _returnvalue_2 "Local") (.TangentLength (Utilities|Struct|BreakStruct_RoadProps_Props (LocalVariables|GetProp)))) true :!class /Script/Engine.SplineMeshComponent)
            (else
              (Components|DestroyComponent (LocalVariables|GetSplineMeshComponent)))))))))