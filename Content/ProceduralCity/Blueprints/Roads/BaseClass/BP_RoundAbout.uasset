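; BP_RoundAbout is a procedural city road roundabout whose centerpiece prop is selectable.
; The construction script sets cull distance on the roundabout and cover meshes and applies the chosen material.
; On BeginPlay, after a short random delay, the SPAWN PROP graph sets the child actor class from the Prop enum: fountain, statue, flags or sign.
; Signs also receive the town name and text size.
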(event EventBeginPlay
  (Utilities|FlowControl|Delay (Math|Random|RandomFloatinRange 0.0 0.5))
  (|SPAWNPROP))

(fn ConstructionScript
  ;[1 1 1] Set max draw distance
  (Class|PrimitiveComponent|SetCullDistance (Variables|Default|GetPCG_RoundAbout) (Variables|Setup|GetCullDistance))
  (Rendering|Material|SetMaterial (Variables|Default|GetPCG_RoundAbout) 0 (Variables|Setup|GetMaterial)))