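; City limits actor for a procedural city, defining its bounds and preparing the area inside.
; Construction script scales box, cylinder and triangle bounds, marker and optional floor, then fits two crossing splines to the box corners.
; FlattenTerrain line-traces vertically to find the Landscape and applies both splines with EditorApplySpline, an editor-only technique.
; SetCullDistanceVolume finds the CullDistanceVolume tagged with the city name and scales it to the box bounds.
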(event Custom|Flatten%20Terrain
  (CallFunction|FnFlattenTerrain))

(event Custom|SetCullDistanceVolume
  (CallFunction|FnSetCullDistanceVolume))

(fn ConstructionScript
  (bind _corner3 (Variables|Default|GetCorner3))
  (bind _corner4 (Variables|Default|GetCorner4))
  (bind _corner1 (Variables|Default|GetCorner1))
  (bind _corner2 (Variables|Default|GetCorner2))
  (bind _boundsscalebox (Variables|Setup|GetBoundsScaleBox))
  (bind _returnvalue (* _boundsscalebox 0.625))
  (bind _returnvalue_2 (Transformation|GetWorldLocation _corner3))
  (bind _returnvalue_3 (Transformation|GetWorldLocation _corner4))
  (bind _returnvalue_4 (Transformation|GetWorldLocation _corner1))
  (bind _returnvalue_5 (Transformation|GetWorldLocation _corner2))
  (bind _returnvalue_6 (- _returnvalue_2 _returnvalue_3))
  (bind _returnvalue_7 (- _returnvalue_4 _returnvalue_5))
  (bind _returnvalue_8 (Math|Vector|VectorLength _returnvalue_6))
  (bind _returnvalue_9 (Math|Vector|VectorLength _returnvalue_7))
  (bind _returnvalue_10 (* _returnvalue_8 0.5))
  (bind _returnvalue_11 (* _returnvalue_9 0.5))
  ;[1 1 1] Set material to bounds
  (Rendering|Material|SetMaterial (Variables|Default|GetMarker) 0 "/Game/ProceduralCity/Materials/Zones/Mi_CityLimits.MI_CityLimits")
  (Utilities|FlowControl|Sequence
    (:then_0
      ;[1 1 1] Set Bound Scale
      (Transformation|SetWorldScale3D (Variables|Default|GetBounds) (Variables|Setup|GetBoundsScaleBox))
      (Transformation|SetWorldScale3D (Variables|Default|GetBoundsTriangle) (Variables|Setup|GetBoundScaleTriangle))
      (Transformation|SetWorldScale3D (Variables|Default|GetBoundsCylinder) (Variables|Setup|GetBoundScaleCylinder))
      ;[1 1 1] Scale visual marker
      (Transformation|SetWorldScale3D (Variables|Default|GetMarker) (* (Variables|Setup|GetBoundsScaleBox) 0.625))
      ;[1 1 1] Scale floor
      (Transformation|SetWorldScale3D (Variables|Default|GetFloor) (Math|Vector|MakeVector (.x _returnvalue) (.y _returnvalue) 0.25))
      ;[1 1 1] Set Marker visibility
      (Rendering|SetVisibility (Variables|Default|GetMarker) (Variables|Setup|GetMarkerVisible) false)
      (Development|SetHiddeninGame (Variables|Default|GetMarker) (Variables|Setup|GetMarkerHidden) false)
      ;[1 1 1] Set Floor material
      (Rendering|Material|SetMaterial (Variables|Default|GetFloor) 0 (Variables|Setup|GetFloorMaterial))
      ;[1 1 1] Show or hide floor
      (if (Variables|Setup|GetShowFloor)
        (Rendering|SetVisibility (Variables|Default|GetFloor) true false)
        (Collision|SetCollisionEnabled (Variables|Default|GetFloor) "QueryAndPhysics")
        (else
          (Rendering|SetVisibility (Variables|Default|GetFloor) false false)
          (Collision|SetCollisionEnabled (Variables|Default|GetFloor) "NoCollision"))))
    (:then_1
      (Utilities|FlowControl|Sequence
        (:then_0
          ;[1 1 1] Adjust the spline1 based on the size of the box
          (Spline|SetLocationatSplinePoint (Variables|Default|GetSpline1) 0 (/ (+ (Transformation|GetWorldLocation (Variables|Default|GetCorner3)) (Transformation|GetWorldLocation (Variables|Default|GetCorner4))) 2) "World" true)
          (Spline|SetLocationatSplinePoint (Variables|Default|GetSpline1) 1 (/ (+ (Transformation|GetWorldLocation (Variables|Default|GetCorner1)) (Transformation|GetWorldLocation (Variables|Default|GetCorner2))) 2) "World" true)
          ;[1 1 1] SetStart and End Widths
          (Variables|Default|SetStartWidth1 _returnvalue_11)
          (Variables|Default|SetEndWidth1 _returnvalue_11))
        (:then_1
          ;[1 1 1] Adjust the spline2 based on the size of the box
          (Spline|SetLocationatSplinePoint (Variables|Default|GetSpline2) 0 (/ (+ (Transformation|GetWorldLocation (Variables|Default|GetCorner4)) (Transformation|GetWorldLocation (Variables|Default|GetCorner1))) 2) "World" true)
          (Spline|SetLocationatSplinePoint (Variables|Default|GetSpline2) 1 (/ (+ (Transformation|GetWorldLocation (Variables|Default|GetCorner2)) (Transformation|GetWorldLocation (Variables|Default|GetCorner3))) 2) "World" true)
          ;[1 1 1] SetStart and End Widths
          (Variables|Default|SetStartWidth2 _returnvalue_10)
          (Variables|Default|SetEndWidth2 _returnvalue_10))))))

(fn FnFlattenTerrain
  (bind (_found _landscape) (CallFunction|FnGetLandscape))
  (if _found
    (LocalVariables|SetTerrain _landscape)
    (Utilities|FlowControl|Sequence
      (:then_0
        ;[1 1 1] Apply Spline1
        (Landscape|Editor|EditorApplySpline (LocalVariables|GetTerrain) (Variables|Default|GetSpline1) (Variables|Default|GetStartWidth1) (Variables|Default|GetEndWidth1) 0.0 2e+02 0.0 0.0 (- (Spline|GetNumberOfSplinePoints (Variables|Default|GetSpline2)) 1) true true 0))
      (:then_1
        ;[1 1 1] Apply Spline1
        (Landscape|Editor|EditorApplySpline (LocalVariables|GetTerrain) (Variables|Default|GetSpline2) (Variables|Default|GetStartWidth2) (Variables|Default|GetEndWidth2) 0.0 2e+02 0.0 0.0 (- (Spline|GetNumberOfSplinePoints (Variables|Default|GetSpline2)) 1) true true 0)))))

(fn FnGetLandscape
  (bind _returnvalue (Transformation|GetActorLocation))
  (bind _returnvalue_2 (+ _returnvalue "0, 0,10000.000000"))
  (Utilities|FlowControl|Sequence
    (:then_0
      (bind (_outhits _returnvalue_3) (Class|KismetSystemLibrary|LineTraceMultiforObjects _returnvalue_2 (+ _returnvalue_2 (* (Transformation|GetActorUpVector) -2e+04)) (Utilities|Array|MakeArray "ObjectTypeQuery1") false 0 "ForDuration" true))
      (if _returnvalue_3
        (bind _array_element (Utilities|Array|ForEachLoopwithBreak _outhits :!label _label)
          (:LoopBody
            (LocalVariables|SetHitActor (.HitActor (Collision|BreakHitResult _array_element)))
            ;[1 1 1] Check to see if the Hit Actor is a landscape
            (if (== (Utilities|GetClass (.HitActor (Collision|BreakHitResult _array_element))) "/Script/Landscape.Landscape")
              ;[1 1 1] Cast to Landscape
              (bind _aslandscape (Utilities|Casting|CastToLandscape (LocalVariables|GetHitActor)))
              (LocalVariables|SetTerrain _aslandscape)
              (LocalVariables|SetFoundTerrain true)
              (goto _label Break))))))
    (:then_1
      (return (LocalVariables|GetFoundTerrain) (LocalVariables|GetTerrain)))))

(fn FnSetCullDistanceVolume
  ;[1 1 1] Loop through all cull distance volumes
  (bind _outactors (Actor|GetAllActorsOfClass "/Script/Engine.CullDistanceVolume"))
  (bind _array_element (Utilities|Array|ForEachLoopwithBreak _outactors :!label _label)
    (:LoopBody
      (LocalVariables|SetCullVolume _array_element)
      ;[1 1 1] Check to see it has the City Name as a tag
      (if (Actor|ActorHasTag (LocalVariables|GetCullVolume) (Variables|Setup|GetCityName))
        (LocalVariables|SetFoundIt true)
        (goto _label Break)))
    (:Completed
      ;[1 1 1] Check if we found the cull volume
      (if (LocalVariables|GetFoundIt)
        ;[1 1 1] Set Bounds Scale
        (Transformation|SetActorScale3D (LocalVariables|GetCullVolume) (* (Variables|Setup|GetBoundsScaleBox) 0.32))))))