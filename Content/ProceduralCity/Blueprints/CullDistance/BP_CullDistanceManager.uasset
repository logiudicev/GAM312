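; BP_CullDistanceManager tracks cull distance objects for the procedural city and which one is currently active.
; FnRegisterCullDistance adds each object passed to it to CullDistanceList.
; FnCheckCullDistance makes the passed object active if none is valid or a different one is active, returning Activate as true only when it switches.
; Event graph and construction script are empty, so all logic runs through calls to these two functions.
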(event EventBeginPlay)

(event Collision|EventActorBeginOverlap
  (params (OtherActor :type Actor%20Object%20Reference)))

(event EventTick
  (params (DeltaSeconds :type Float%20%28single-precision%29)))

(fn ConstructionScript)

(fn FnRegisterCullDistance
  (params (Cull%20Distance :type BP%20Change%20Cull%20Distances%20Object%20Reference))
  (Utilities|Array|Add (Variables|Setup|GetCullDistanceList) Cull%20Distance))

(fn FnCheckCullDistance
  (params (Cull%20Distance :type BP%20Change%20Cull%20Distances%20Object%20Reference))
  (LocalVariables|SetNewDistance Cull%20Distance)
  (Utilities|FlowControl|Sequence
    (:then_0
      (Utilities|IsValid (Variables|Setup|GetActiveCullDistance)
        (:Is%20Valid
          (if (!= (Variables|Setup|GetActiveCullDistance) (LocalVariables|GetNewDistance))
            (Variables|Setup|SetActiveCullDistance (LocalVariables|GetNewDistance) :!label _label)
            (LocalVariables|SetActivate true)
            (else
              (LocalVariables|SetActivate false))))
        (:Is%20Not%20Valid
          (goto _label))))
    (:then_1
      (return (LocalVariables|GetActivate)))))