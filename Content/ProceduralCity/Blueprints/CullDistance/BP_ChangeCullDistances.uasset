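; Trigger volume actor that changes the procedural city's cull distances when an actor tagged Player enters it.
; On overlap it passes its cull distance options to the referenced city, first asking the manager for approval if one is set.
; A DoOnce blocks repeat firing until the player leaves.
; The construction script applies the trigger's scale and visibility settings.
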(event OnComponentBeginOverlap(Trigger)
  (params (OverlappedComponent :type Primitive%20Component%20Object%20Reference) (OtherActor :type Actor%20Object%20Reference) (OtherComp :type Primitive%20Component%20Object%20Reference) (OtherBodyIndex :type Integer) (bFromSweep :type Boolean) (SweepResult :type Hit%20Result%20Structure%20%28by%20ref%29))
  (if (Actor|ActorHasTag OtherActor "Player")
    (Utilities|FlowControl|DoOnce false
      (:Completed
        (Utilities|IsValid (Variables|Setup|GetCityReference)
          (:Is%20Valid
            (Utilities|IsValid (Variables|Setup|GetManagerReference)
              (:Is%20Valid
                (bind _can_activate (Default|FnCheckCullDistance (Variables|Setup|GetManagerReference) self))
                (if _can_activate
                  (Default|EventSetCullDistances (Variables|Setup|GetCityReference) (Variables|Setup|GetOptions) false (Utilities|String|Append (Utilities|GetDisplayName self) " loading...") :!label _label)))
              (:Is%20Not%20Valid
                (goto _label)))))))))

(event OnComponentEndOverlap(Trigger)
  (params (OverlappedComponent :type Primitive%20Component%20Object%20Reference) (OtherActor :type Actor%20Object%20Reference) (OtherComp :type Primitive%20Component%20Object%20Reference) (OtherBodyIndex :type Integer))
  (if (Actor|ActorHasTag OtherActor "Player")
    (Utilities|FlowControl|DoOnce false) ; enters at Reset
  ))

(event EventBeginPlay)

(event Collision|EventActorBeginOverlap
  (params (OtherActor :type Actor%20Object%20Reference)))

(event EventTick
  (params (DeltaSeconds :type Float%20%28single-precision%29)))

(fn ConstructionScript
  (Transformation|SetWorldScale3D (Variables|Default|GetTrigger) (Variables|Setup|GetTriggerScale))
  (Rendering|SetVisibility (Variables|Default|GetTrigger) (Variables|Setup|GetTriggerVisible) false)
  (Development|SetHiddeninGame (Variables|Default|GetTrigger) (Variables|Setup|GetTriggerHidden) false))