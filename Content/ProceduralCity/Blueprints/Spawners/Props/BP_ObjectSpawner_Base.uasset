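; Base spawner for procedural city props that spawns an actor when the player enters a trigger, optionally hiding or destroying it on exit.
; Without an impostor it uses the activation trigger; with one, the impostor trigger swaps a static-mesh stand-in for the actor, sparing player-controlled pawns on exit.
; Random per-slot materials chosen for the impostor pass to the actor.
; Spawns receive city and PCG tags; child classes can override show/hide events.
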(event OnComponentBeginOverlap(ActivationTrigger)
  (params (OverlappedComponent :type Primitive%20Component%20Object%20Reference) (OtherActor :type Actor%20Object%20Reference) (OtherComp :type Primitive%20Component%20Object%20Reference) (OtherBodyIndex :type Integer) (bFromSweep :type Boolean) (SweepResult :type Hit%20Result%20Structure%20%28by%20ref%29))
  ;[1 1 1] ACTIVATION TRIGGER
  (if (and (Actor|ActorHasTag OtherActor "Player") (not (Variables|Setup|GetUseImpostor)))
    (Utilities|FlowControl|Sequence
      (:then_0
        (Variables|Default|SetCanDespawn false)
        (if (not (Utilities|IsValid (Variables|Default|GetSpawnedActor)))
          (CallFunction|FnSpawnActor false)
          (else
            (switch Utilities|FlowControl|Switch|SwitchonEnum_InteriorDespawnMethod (Variables|Setup|GetDespawnMethod)
              (:NewEnumerator0
                (CallFunction|FnShowActor)
                (CallFunction|EventShowActor))
              (:NewEnumerator1
                (CallFunction|FnSpawnActor false))))))
      (:then_1
        (Utilities|FlowControl|Delay 0.5)
        (Variables|Default|SetCanDespawn true)))))

(event OnComponentEndOverlap(ActivationTrigger)
  (params (OverlappedComponent :type Primitive%20Component%20Object%20Reference) (OtherActor :type Actor%20Object%20Reference) (OtherComp :type Primitive%20Component%20Object%20Reference) (OtherBodyIndex :type Integer))
  ;[1 1 1] ACTIVATION TRIGGER
  (if (and (Actor|ActorHasTag OtherActor "Player") (not (Variables|Setup|GetUseImpostor)))
    (Utilities|FlowControl|Delay 1.0)
    (if (and (Variables|Setup|GetDespawnActor?) (Variables|Default|GetCanDespawn))
      (switch Utilities|FlowControl|Switch|SwitchonEnum_InteriorDespawnMethod (Variables|Setup|GetDespawnMethod)
        (:NewEnumerator0
          (CallFunction|FnHideActor)
          (CallFunction|EventHideActor))
        (:NewEnumerator1
          (CallFunction|FnDestroyActor))))))

(event OnComponentBeginOverlap(ImpostorTrigger)
  (params (OverlappedComponent :type Primitive%20Component%20Object%20Reference) (OtherActor :type Actor%20Object%20Reference) (OtherComp :type Primitive%20Component%20Object%20Reference) (OtherBodyIndex :type Integer) (bFromSweep :type Boolean) (SweepResult :type Hit%20Result%20Structure%20%28by%20ref%29))
  ;[1 1 1] IMPOSTOR TRIGGER
  (if (and (Actor|ActorHasTag OtherActor "Player") (Variables|Setup|GetUseImpostor))
    (if (not (Variables|Default|GetActorHasSpawned))
      (Utilities|IsValid (Variables|Default|GetSpawnedImpostor)
        (:Is%20Valid
          (CallFunction|FnSpawnActor false))))))

(event OnComponentEndOverlap(ImpostorTrigger)
  (params (OverlappedComponent :type Primitive%20Component%20Object%20Reference) (OtherActor :type Actor%20Object%20Reference) (OtherComp :type Primitive%20Component%20Object%20Reference) (OtherBodyIndex :type Integer))
  ;[1 1 1] IMPOSTOR TRIGGER
  (if (and (Actor|ActorHasTag OtherActor "Player") (Variables|Setup|GetUseImpostor))
    (if (Variables|Setup|GetDespawnActor?)
      (Utilities|IsValid (Variables|Default|GetSpawnedActor)
        (:Is%20Valid
          (Utilities|FlowControl|Delay 0.2)
          (bind _aspawn (Utilities|Casting|CastToPawn (Variables|Default|GetSpawnedActor))
            (:then
              (if (not (Pawn|IsPlayerControlled _aspawn))
                (CallFunction|FnSpawnActor true :!label _label)))
            (:CastFailed
              (goto _label))))))))

(event EventBeginPlay
  ;[1 1 1] If we use an impostor, then scale the Activation Trigger to 0
  (if (Variables|Setup|GetUseImpostor)
    (Transformation|SetWorldScale3D (Variables|Default|GetActivationTrigger) "0.010000,0.010000,0.010000")
    ;[1 1 1] Check if we have not spawned the impostor
    (if (not (Utilities|IsValid (Variables|Default|GetSpawnedImpostor)))
      (CallFunction|EventSpawnImpostor))))

(fn ConstructionScript
  ;[1 1 1] Set trigger scales
  (Transformation|SetWorldScale3D (Variables|Default|GetActivationTrigger) (Variables|Setup|GetActivationTriggerScale))
  (Transformation|SetWorldScale3D (Variables|Default|GetImpostorTrigger) (Variables|Setup|GetImpostorTriggerScale))
  ;[1 1 1] If we use an impostor, then scale the Activation Trigger to 0
  (if (Variables|Setup|GetUseImpostor)
    (Transformation|SetWorldScale3D (Variables|Default|GetActivationTrigger) "0, 0, 0")))

(fn FnSpawnActor
  (params (Spawn%20Impostor :type Boolean))
  (if Spawn%20Impostor
    (Utilities|FlowControl|Sequence
      (:then_0
        ;[1 1 1] Switch on Despawn Method
        (switch Utilities|FlowControl|Switch|SwitchonEnum_InteriorDespawnMethod (Variables|Setup|GetDespawnMethod)
          (:NewEnumerator0
            ;[1 1 1] Hide Actor
            (CallFunction|FnHideActor)
            (CallFunction|EventHideActor))
          (:NewEnumerator1
            ;[1 1 1] Destroy Actor
            (CallFunction|FnDestroyActor)
            (Variables|Default|SetActorHasSpawned false))))
      (:then_1
        ;[1 1 1] Show Impostor
        (Rendering|SetActorHiddenInGame (Variables|Default|GetSpawnedImpostor) false)
        (Collision|SetActorEnableCollision (Variables|Default|GetSpawnedImpostor) true)))
    (else
      (Utilities|FlowControl|Sequence
        (:then_0
          ;[1 1 1] Hide Impostor
          (if (Variables|Setup|GetUseImpostor)
            (Rendering|SetActorHiddenInGame (Variables|Default|GetSpawnedImpostor) true)
            (Collision|SetActorEnableCollision (Variables|Default|GetSpawnedImpostor) false)))
        (:then_1
          ;[1 1 1] Spawn Actor
          (bind _returnvalue (Game|SpawnActorfromClass (Variables|Setup|GetSpawnActor) (Math|Transform|MakeTransform (Transformation|GetActorLocation) (Transformation|GetActorRotation)) "AlwaysSpawn" 0 0))
          (Variables|Default|SetSpawnedActor _returnvalue)
          ;[1 1 1] Add appropriate tags
          (CallFunction|FnAddTags (Variables|Default|GetSpawnedActor))
          (Variables|Default|SetActorHasSpawned true)
          ;[1 1 1] Do we randomize the material?
          (if (Variables|Setup|GetRandomizeMaterial)
            ;[1 1 1] Send material list to spawned actor
            (Class|BPBPIPCGPropInterface|FnGetMaterials(Message) (Variables|Default|GetSpawnedActor) (Variables|Default|GetFinalMaterialList))))))))

(fn FnShowActor
  ;[1 1 1] If the actor is valid, show it
  (Utilities|IsValid (Variables|Default|GetSpawnedActor)
    (:Is%20Valid
      (Rendering|SetActorHiddenInGame (Variables|Default|GetSpawnedActor) false))))

(fn FnHideActor
  ;[1 1 1] If the actor is valid, hide it
  (Utilities|IsValid (Variables|Default|GetSpawnedActor)
    (:Is%20Valid
      (Rendering|SetActorHiddenInGame (Variables|Default|GetSpawnedActor) true))))

(fn FnDestroyActor
  ;[1 1 1] If the actor is valid, destroy it
  (Utilities|IsValid (Variables|Default|GetSpawnedActor)
    (:Is%20Valid
      (Actor|DestroyActor (Variables|Default|GetSpawnedActor)))))

(fn FnSpawnImpostor
  ;[1 1 1] Spawn SM Actor
  (bind _returnvalue (Game|SpawnActorfromClass "/Script/Engine.StaticMeshActor" (Math|Transform|MakeTransform (Transformation|GetActorLocation) (Transformation|GetActorRotation)) "AlwaysSpawn" 0 0))
  (Variables|Default|SetSpawnedImpostor _returnvalue)
  ;[1 1 1] Set Mobility to Movable
  (Transformation|SetMobility (Variables|Default|GetSpawnedImpostor) "Movable")
  ;[1 1 1] Set the impostor Static Mesh
  (Components|StaticMesh|SetStaticMesh (Variables|/Script/Engine.StaticMeshActor|GetStaticMeshComponent (Variables|Default|GetSpawnedImpostor)) (Variables|Setup|GetImpostorMesh))
  ;[1 1 1] Attach Impostor to the BP
  (Transformation|AttachActorToActor (Variables|Default|GetSpawnedImpostor) self "None" "KeepWorld" "KeepWorld" "KeepWorld" false)
  ;[1 1 1] Add appropriate tags
  (CallFunction|FnAddTags (Variables|Default|GetSpawnedImpostor)))

(fn FnAddTags
  (params (Actor :type Actor%20Object%20Reference))
  (LocalVariables|SetNewActor Actor)
  (Utilities|FlowControl|Sequence
    (:then_0
      ;[1 1 1] Add the City Name as a tag
      (Utilities|Array|Add (Variables|/Script/Engine.Actor|GetTags (LocalVariables|GetNewActor)) (Variables|Setup|GetCityName)))
    (:then_1
      ;[1 1 1] Add Foliage tag
      (if (Variables|Setup|GetMarkAsFoliage)
        (Utilities|Array|Add (Variables|/Script/Engine.Actor|GetTags (LocalVariables|GetNewActor)) "pcgFoliage")))
    (:then_2
      ;[1 1 1] Add fixed prop tag
      (if (Variables|Setup|GetMarkAsFixedProp)
        (Utilities|Array|Add (Variables|/Script/Engine.Actor|GetTags (LocalVariables|GetNewActor)) "pcgFixedProps")
        ;[1 1 1] Add prop tag
        (Utilities|Array|AddUnique (Variables|/Script/Engine.Actor|GetTags (LocalVariables|GetNewActor)) "pcgProp" :!label _label)))
    (:then_3
      ;[1 1 1] Add random prop tag
      (if (Variables|Setup|GetMarkAsRandomProp)
        (Utilities|Array|Add (Variables|/Script/Engine.Actor|GetTags (LocalVariables|GetNewActor)) "pcgRandomProps")
        (goto _label)))
    (:then_4
      ;[1 1 1] Add all additional tags to the actor
      (for _array_element (Variables|Setup|GetAdditionalTags)
        (Utilities|Array|Add (Variables|/Script/Engine.Actor|GetTags (LocalVariables|GetNewActor)) _array_element)))))

(fn FnRandomizeMaterials
  ;[1 1 1] Loop through all the random materials
  (for _array_element (Variables|Setup|GetRandomMaterialList)
    (LocalVariables|SetMaterial _array_element)
    ;[1 1 1] Set a random material per Material Index
    (Utilities|Map|Add (Variables|Default|GetFinalMaterialList) (.MaterialID (Utilities|Struct|BreakStruct_RandomMaterials (LocalVariables|GetMaterial))) (Utilities|Array|Get(acopy) (.MaterialList (Utilities|Struct|BreakStruct_RandomMaterials (LocalVariables|GetMaterial))) (Math|Random|RandomIntegerinRange 0 (Utilities|Array|LastIndex (.MaterialList (Utilities|Struct|BreakStruct_RandomMaterials (LocalVariables|GetMaterial))))))))
  ;[1 1 1] Loop through the final material list
  (bind _keys (Utilities|Map|Keys (Variables|Default|GetFinalMaterialList)))
  (for _array_element_2 _keys
    (LocalVariables|SetMatIndex _array_element_2)
    ;[1 1 1] Set Material
    (Rendering|Material|SetMaterial (Variables|/Script/Engine.StaticMeshActor|GetStaticMeshComponent (Variables|Default|GetSpawnedImpostor)) (LocalVariables|GetMatIndex) (.Value (Utilities|Map|Find (Variables|Default|GetFinalMaterialList) (LocalVariables|GetMatIndex))))))

(event Custom|EventShowActor
  ;[1 1 1] Overridable Events
)

(event Custom|EventHideActor
  ;[1 1 1] Overridable Events
)

(event EventFnSetCityName
  (params (City%20Name :type Name :default "None"))
  (Variables|Setup|SetCityName City%20Name))

(event Custom|EventSpawnImpostor
  (if (Variables|Setup|GetUseImpostor)
    (CallFunction|FnSpawnImpostor)
    ;[1 1 1] Do we select a random material?
    (if (Variables|Setup|GetRandomizeMaterial)
      ;[1 1 1] Set Random materials
      (CallFunction|FnRandomizeMaterials))))

(event EventFnPropPlaced
  (if (Variables|Setup|GetUseImpostor)
    (CallFunction|FnSpawnImpostor)
    ;[1 1 1] Do we select a random material?
    (if (Variables|Setup|GetRandomizeMaterial)
      ;[1 1 1] Set Random materials
      (CallFunction|FnRandomizeMaterials))))