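; Procedural city spawner that scatters random foliage along a spline, offset to the left, right or both sides.
; Box traces reject steep slopes and hits on tagged city content, then give the position and normal for placement.
; Each pick spawns its actor class or a static mesh actor, tagged for the spawner.
; Separate events remove foliage by tag or bake tagged mesh actors into one HISM actor per mesh.
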(event Custom|1_SpawnFoliage
  (CallFunction|FnSpawnFoliage))

(event Custom|2_RemoveFoliage
  (CallFunction|FnRemoveFoliage))

(event Custom|3_ConvertToHISM
  (CallFunction|FnConvertFoliagetoHISM))

(event EventEventSpawnFoliage
  (CallFunction|FnSpawnFoliage))

(event EventEventRemoveFoliage
  (CallFunction|FnRemoveFoliage))

(event EventEventConverttoHISM
  (CallFunction|FnConvertFoliagetoHISM))

(fn ConstructionScript
  (|CallParentFunction))

(fn FnSpawnFoliage
  (bind _spline (Variables|Default|GetSpline))
  (bind _spawnnormal (Variables|Default|GetSpawnNormal))
  ;[1 1 1] Loop through FoliageToSpawn
  (for _index (range 0 (- (Variables|Setup|GetFoliageToSpawn) 1))
    ;[1 1 1] Get random location and offset
    (LocalVariables|SetSplineDistance (Math|Random|RandomFloatinRange 0.0 (Spline|GetSplineLength (Variables|Default|GetSpline))))
    (LocalVariables|SetSplineOffset (Math|Random|RandomFloatinRange (Variables|Setup|GetMinWidth) (Variables|Setup|GetMaxWidth)))
    (if (and (Variables|Setup|GetSpawnRight) (Variables|Setup|GetSpawnLeft))
      ;[1 1 1] Randomize right or left offset from spline
      (if (Math|Random|RandomBool)
        _
        (else
          (LocalVariables|SetSplineOffset (* (LocalVariables|GetSplineOffset) -1.0))))
      ;[1 1 1] Get Random Location and random foliage from the list
      (LocalVariables|SetRandomLocation (+ (Spline|GetLocationatDistanceAlongSpline _spline (LocalVariables|GetSplineDistance) "World") (* (Math|Vector|GetRightVector (Spline|GetRotationatDistanceAlongSpline _spline (LocalVariables|GetSplineDistance) "World")) (LocalVariables|GetSplineOffset))) :!label _label)
      (LocalVariables|SetRandomIndex (Math|Random|RandomIntegerinRange 0 (- (Utilities|Array|Length (Variables|Setup|GetFoliageList)) 1)))
      ;[1 1 1] Set Foliage Reference
      (LocalVariables|SetFoliageActor (.ActorClassPriority (Utilities|Struct|BreakStruct_FoliageDetails_Spawner (Utilities|Array|Get(acopy) (Variables|Setup|GetFoliageList) (LocalVariables|GetRandomIndex)))))
      (LocalVariables|SetFoliageRef (.StaticMesh (Utilities|Struct|BreakStruct_FoliageDetails_Spawner (Utilities|Array|Get(acopy) (Variables|Setup|GetFoliageList) (LocalVariables|GetRandomIndex)))))
      ;[1 1 1] Check the spawn location
      (bind _can_spawn (CallFunction|FnCheckFoliageSpawnLocation (LocalVariables|GetRandomLocation) (Utilities|Array|Get(acopy) (Variables|Setup|GetFoliageList) (LocalVariables|GetRandomIndex))))
      (if _can_spawn
        ;[1 1 1] Set Foliage Rotation
        (if (and (.RandomYaw? (Utilities|Struct|BreakStruct_FoliageDetails_Spawner (Utilities|Array|Get(acopy) (Variables|Setup|GetFoliageList) (LocalVariables|GetRandomIndex)))) (.Aligntosurface? (Utilities|Struct|BreakStruct_FoliageDetails_Spawner (Utilities|Array|Get(acopy) (Variables|Setup|GetFoliageList) (LocalVariables|GetRandomIndex)))))
          (LocalVariables|SetTargetRotation (Math|Rotator|CombineRotators (Math|Rotator|MakeRotfromZ _spawnnormal) (Math|Vector|RotatorfromAxisandAngle _spawnnormal (Math|Random|RandomFloatinRange 0.0 359.0))))
          (elif (.RandomYaw? (Utilities|Struct|BreakStruct_FoliageDetails_Spawner (Utilities|Array|Get(acopy) (Variables|Setup|GetFoliageList) (LocalVariables|GetRandomIndex))))
            (LocalVariables|SetTargetRotation (Math|Vector|RotatorfromAxisandAngle (Variables|Default|GetSpawnNormal) (Math|Random|RandomFloatinRange 0.0 359.0)))
            (elif (.Aligntosurface? (Utilities|Struct|BreakStruct_FoliageDetails_Spawner (Utilities|Array|Get(acopy) (Variables|Setup|GetFoliageList) (LocalVariables|GetRandomIndex))))
              (LocalVariables|SetTargetRotation (Math|Rotator|MakeRotfromZX (Variables|Default|GetSpawnNormal) (Transformation|GetActorForwardVector))))))
        (if (Utilities|IsValidClass (LocalVariables|GetFoliageActor))
          ;[1 1 1] Spawn Foliage Actor
          (bind _returnvalue (Game|SpawnActorfromClass (LocalVariables|GetFoliageActor) (Math|Transform|MakeTransform (Variables|Default|GetSpawnLocation) (LocalVariables|GetTargetRotation) (Math|Vector|MakeVector (Math|Random|RandomFloatinRange (.MinScale (Utilities|Struct|BreakStruct_FoliageDetails_Spawner (Utilities|Array|Get(acopy) (Variables|Setup|GetFoliageList) (LocalVariables|GetRandomIndex)))) (.MaxScale (Utilities|Struct|BreakStruct_FoliageDetails_Spawner (Utilities|Array|Get(acopy) (Variables|Setup|GetFoliageList) (LocalVariables|GetRandomIndex))))) (Math|Random|RandomFloatinRange (.MinScale (Utilities|Struct|BreakStruct_FoliageDetails_Spawner (Utilities|Array|Get(acopy) (Variables|Setup|GetFoliageList) (LocalVariables|GetRandomIndex)))) (.MaxScale (Utilities|Struct|BreakStruct_FoliageDetails_Spawner (Utilities|Array|Get(acopy) (Variables|Setup|GetFoliageList) (LocalVariables|GetRandomIndex))))) (Math|Random|RandomFloatinRange (.MinScale (Utilities|Struct|BreakStruct_FoliageDetails_Spawner (Utilities|Array|Get(acopy) (Variables|Setup|GetFoliageList) (LocalVariables|GetRandomIndex)))) (.MaxScale (Utilities|Struct|BreakStruct_FoliageDetails_Spawner (Utilities|Array|Get(acopy) (Variables|Setup|GetFoliageList) (LocalVariables|GetRandomIndex))))))) "Undefined" 0 0))
          (LocalVariables|SetSpawnedActor _returnvalue)
          ;[1 1 1] Assign tags
          (Utilities|Array|AddUnique (Variables|/Script/Engine.Actor|GetTags (LocalVariables|GetSpawnedFoliage)) (Variables|Default|GetFoliageTag))
          (Utilities|Array|AddUnique (Variables|/Script/Engine.Actor|GetTags (LocalVariables|GetSpawnedFoliage)) (Variables|Default|GetCityName))
          (Utilities|Array|AddUnique (Variables|/Script/Engine.Actor|GetTags (LocalVariables|GetSpawnedFoliage)) (Utilities|String|StringToName (Utilities|GetDisplayName self)))
          (else
            ;[1 1 1] Spawn Foliage
            (bind _returnvalue_2 (Game|SpawnActorfromClass "/Script/Engine.StaticMeshActor" (Math|Transform|MakeTransform (Variables|Default|GetSpawnLocation) (LocalVariables|GetTargetRotation) (Math|Vector|MakeVector (Math|Random|RandomFloatinRange (.MinScale (Utilities|Struct|BreakStruct_FoliageDetails_Spawner (Utilities|Array|Get(acopy) (Variables|Setup|GetFoliageList) (LocalVariables|GetRandomIndex)))) (.MaxScale (Utilities|Struct|BreakStruct_FoliageDetails_Spawner (Utilities|Array|Get(acopy) (Variables|Setup|GetFoliageList) (LocalVariables|GetRandomIndex))))) (Math|Random|RandomFloatinRange (.MinScale (Utilities|Struct|BreakStruct_FoliageDetails_Spawner (Utilities|Array|Get(acopy) (Variables|Setup|GetFoliageList) (LocalVariables|GetRandomIndex)))) (.MaxScale (Utilities|Struct|BreakStruct_FoliageDetails_Spawner (Utilities|Array|Get(acopy) (Variables|Setup|GetFoliageList) (LocalVariables|GetRandomIndex))))) (Math|Random|RandomFloatinRange (.MinScale (Utilities|Struct|BreakStruct_FoliageDetails_Spawner (Utilities|Array|Get(acopy) (Variables|Setup|GetFoliageList) (LocalVariables|GetRandomIndex)))) (.MaxScale (Utilities|Struct|BreakStruct_FoliageDetails_Spawner (Utilities|Array|Get(acopy) (Variables|Setup|GetFoliageList) (LocalVariables|GetRandomIndex))))))) "Undefined" 0 0))
            (LocalVariables|SetSpawnedFoliage _returnvalue_2)
            ;[1 1 1] Set static mesh
            (Components|StaticMesh|SetStaticMesh (Variables|/Script/Engine.StaticMeshActor|GetStaticMeshComponent (LocalVariables|GetSpawnedFoliage)) (Utilities|Struct|BreakStruct_FoliageDetails_Spawner (Utilities|Array|Get(acopy) (Variables|Setup|GetFoliageList) (LocalVariables|GetRandomIndex))))
            ;[1 1 1] Set Cull Distance
            (Class|PrimitiveComponent|SetCullDistance (Variables|/Script/Engine.StaticMeshActor|GetStaticMeshComponent (LocalVariables|GetSpawnedFoliage)) (Variables|Setup|GetCullDistance))
            (Utilities|FlowControl|Sequence
              (:then_0
                ;[1 1 1] Assign tags
                (Utilities|Array|AddUnique (Variables|/Script/Engine.Actor|GetTags (LocalVariables|GetSpawnedFoliage)) (Variables|Default|GetFoliageTag))
                (Utilities|Array|AddUnique (Variables|/Script/Engine.Actor|GetTags (LocalVariables|GetSpawnedFoliage)) (Variables|Default|GetCityName))
                (Utilities|Array|AddUnique (Variables|/Script/Engine.Actor|GetTags (LocalVariables|GetSpawnedFoliage)) (Utilities|String|StringToName (Utilities|GetObjectName (LocalVariables|GetFoliageRef))))
                (Utilities|Array|AddUnique (Variables|/Script/Engine.Actor|GetTags (LocalVariables|GetSpawnedFoliage)) (Utilities|String|StringToName (Utilities|GetDisplayName self)))
                ;[1 1 1] Check if we have this Foliage tag in our FoliageTags array
                (if (not (Utilities|Array|ContainsItem (Variables|Default|GetFoliageTags) (Utilities|String|StringToName (Utilities|GetDisplayName (LocalVariables|GetFoliageRef)))))
                  ;[1 1 1] Add the tag to FoliageTags array
                  (Utilities|Array|AddUnique (Variables|Default|GetFoliageTags) (Utilities|String|StringToName (Utilities|GetDisplayName (LocalVariables|GetFoliageRef))))))
              (:then_1
                ;[1 1 1] Set Mobility and attach to the spawner
                (Transformation|SetMobility (LocalVariables|GetSpawnedFoliage) "Movable")
                (Transformation|AttachActorToActor (LocalVariables|GetSpawnedFoliage) self "None" "KeepWorld" "KeepWorld" "KeepWorld" true))))))
      (elif (Variables|Setup|GetSpawnLeft)
        (LocalVariables|SetSplineOffset (* (LocalVariables|GetSplineOffset) -1.0))
        (goto _label)
        (elif (Variables|Setup|GetSpawnRight)
          (goto _label)
          (else
            ;[1 1 1] Print Error
            (Development|PrintString "Foliage Spawner (Spline): NO SIDE SELECTED" true true "(R=1.000000,G=0.000000,B=0.000000,A=1.000000)" 5.0)))))))

(fn FnRemoveFoliage
  ;[1 1 1] Get all the foliage that belongs to this Spawner and remove it
  (bind _outactors (Actor|GetAllActorswithTag (Utilities|String|StringToName (Utilities|GetDisplayName self))))
  (for _array_element _outactors
    (Actor|DestroyActor _array_element)))

(fn FnCheckFoliageSpawnLocation
  (params (Location :type Vector) (Foliage :type Struct%20Foliage%20Details%20Spawner%20Structure))
  (LocalVariables|SetSpawnPoint Location)
  (LocalVariables|SetFoliageDetails Foliage)
  (Utilities|FlowControl|Sequence
    (:then_0
      (if (Variables|Setup|GetDebugFoliageTrace?)
        (LocalVariables|SetDebugType "ForDuration")
        (else
          (LocalVariables|SetDebugType "None")))
      (bind (_outhit _returnvalue) (Collision|BoxTraceByChannel (+ (LocalVariables|GetSpawnPoint) (Math|Vector|MakeVector 0.0 0.0 (Variables|Setup|GetTraceZOffset))) (- (LocalVariables|GetSpawnPoint) (Math|Vector|MakeVector 0.0 0.0 (Variables|Setup|GetTraceZOffset))) (+ (Utilities|Struct|BreakStruct_FoliageDetails_Spawner (LocalVariables|GetFoliageDetails)) (Variables|Setup|GetTracePadding)) (LocalVariables|GetSpawnRotation) "TraceTypeQuery1" false 0 (LocalVariables|GetDebugType) true "(R=1.000000,G=0.000000,B=0.000000,A=1.000000)" "(R=0.000000,G=1.000000,B=0.000000,A=1.000000)" (Variables|Setup|GetDebugTraceDuration)))
      (if _returnvalue
        (if (Math|Boolean|ANDBoolean (not (Math|Boolean|ORBoolean (Actor|ActorHasTag (.HitActor (Collision|BreakHitResult _outhit)) "pcgRoad") (Actor|ActorHasTag (.HitActor (Collision|BreakHitResult _outhit)) "pcgProp") (Actor|ActorHasTag (.HitActor (Collision|BreakHitResult _outhit)) "pcgBuilding") (Actor|ActorHasTag (.HitActor (Collision|BreakHitResult _outhit)) "pcgFoliage") (Actor|ActorHasTag "pcgConn"))) (<= (Math|Float|Absolute(Float) (.X (Math|Vector|BreakVector (.Normal (Collision|BreakHitResult _outhit))))) (.Maxslopetospawn (Utilities|Struct|BreakStruct_FoliageDetails_Spawner (LocalVariables|GetFoliageDetails)))) (<= (Math|Float|Absolute(Float) (.Y (Math|Vector|BreakVector (.Normal (Collision|BreakHitResult _outhit))))) (.Maxslopetospawn (Utilities|Struct|BreakStruct_FoliageDetails_Spawner (LocalVariables|GetFoliageDetails)))))
          (LocalVariables|SetSpawn true)
          (Variables|Default|SetSpawnLocation (.ImpactPoint (Collision|BreakHitResult _outhit)))
          (Variables|Default|SetSpawnNormal (.Normal (Collision|BreakHitResult _outhit)))
          (else
            (LocalVariables|SetSpawn false)))))
    (:then_1
      (return (LocalVariables|GetSpawn)))))

(fn FnConvertFoliagetoHISM
  ;[1 1 1] Check that we have at least 1 tag
  (if (> (Utilities|Array|Length (Variables|Default|GetFoliageTags)) 0)
    ;[1 1 1] Go through all the tags
    (for _array_element (Variables|Default|GetFoliageTags)
      (LocalVariables|SetTag _array_element)
      ;[1 1 1] Get all actors of each tag
      (bind _outactors (Actor|GetAllActorswithTag (LocalVariables|GetTag)))
      (LocalVariables|SetList _outactors)
      (Utilities|FlowControl|Sequence
        (:then_0
          ;[1 1 1] Spawn HISM actor in the scene
          (bind _returnvalue (Game|SpawnActorfromClass "/Game/ProceduralCity/Blueprints/Buildings/BP_PCG_HISM_Foliage.BP_PCG_HISM_Foliage_C" (Math|Transform|MakeTransform "0, 0, 0") "AlwaysSpawn" 0 0))
          (LocalVariables|SetHISMActor _returnvalue)
          ;[1 1 1] Add foliage tag
          (Utilities|Array|AddUnique (Variables|/Script/Engine.Actor|GetTags (LocalVariables|GetHISMActor)) (Variables|Default|GetFoliageTag))
          ;[1 1 1] Add city tag
          (Utilities|Array|AddUnique (Variables|/Script/Engine.Actor|GetTags (LocalVariables|GetHISMActor)) (Utilities|String|StringToName (Utilities|GetDisplayName self)))
          ;[1 1 1] Set the HISM actor's static mesh by using the first static mesh from the Foliage List
          (Components|StaticMesh|SetStaticMesh (Variables|/Game/ProceduralCity/Blueprints/Buildings/BP_PCG_HISM_Foliage.BP_PCG_HISM_Foliage_C|GetHISM (LocalVariables|GetHISMActor)) (Variables|/Script/Engine.StaticMeshComponent|GetStaticMesh (Actor|GetComponentbyClass (Utilities|Array|Get(acopy) (LocalVariables|GetList)) "/Script/Engine.StaticMeshComponent")))
          ;[1 1 1] Attach to this spawner
          (Transformation|AttachActorToActor (LocalVariables|GetHISMActor) self "None" "KeepWorld" "KeepWorld" "KeepWorld" true))
        (:then_1
          ;[1 1 1] Go through all actors with this unique ID
          (for _array_element_2 (LocalVariables|GetList)
            (LocalVariables|SetFoliageRef _array_element_2)
            ;[1 1 1] Check that this foliage is part of the current spawner
            (if (Utilities|Array|ContainsItem (Variables|/Script/Engine.Actor|GetTags (LocalVariables|GetFoliageRef)) (Utilities|String|StringToName (Utilities|GetDisplayName self)))
              ;[1 1 1] Add instance to HISM actor by using this building's transform
              (Class|InstancedStaticMeshComponent|AddInstanceWorldSpace (Variables|/Game/ProceduralCity/Blueprints/Buildings/BP_PCG_HISM_Foliage.BP_PCG_HISM_Foliage_C|GetHISM (LocalVariables|GetHISMActor)) (Transformation|GetActorTransform (LocalVariables|GetFoliageRef)))
              (Actor|DestroyActor (LocalVariables|GetFoliageRef)))))))))