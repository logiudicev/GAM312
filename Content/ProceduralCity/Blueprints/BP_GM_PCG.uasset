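; BP_GM_PCG is the procedural city Blueprint, apparently a game mode, with a function for spawning third-person characters at PlayerStarts.
; FnSpawnPlayers spawns a character at each PlayerStart, calls CreatePlayer, then has player controller 0 possess the pawn and applies control-rotation yaw.
; Every iteration reuses index 0, so that controller moves to each new pawn.
; The delayed spawn call is disconnected from BeginPlay, so it never runs.
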(event EventBeginPlay)

(fn ConstructionScript)

(fn FnSpawnPlayers
  (Utilities|FlowControl|Sequence
    (:then_0
      (bind _outactors (Actor|GetAllActorsOfClass "/Script/Engine.PlayerStart"))
      (Variables|Default|SetPlayerStartList _outactors))
    (:then_1
      (for _array_element (Variables|Default|GetPlayerStartList)
        (LocalVariables|SetStart _array_element)
        ;[1 1 1] Create Player
        (Class|GameplayStatics|CreatePlayer 0)
        ;[1 1 1] Spawn Player BP in the world
        (bind _returnvalue (Game|SpawnActorfromClass "/Game/ProceduralCity/Blueprints/Characters/BP_ThirdPersonCharacter.BP_ThirdPersonCharacter_C" (Transformation|GetActorTransform (LocalVariables|GetStart)) "AlwaysSpawn" 0 0))
        (bind _output_get (LocalVariables|SetSpawnedActor _returnvalue))
        ;[1 1 1] Convert to Pawn
        (bind _aspawn (Utilities|Casting|CastToPawn _output_get))
        (LocalVariables|SetSpawnedPawn _aspawn)
        ;[1 1 1] Have Player Controller possess the spawned player
        (Pawn|Possess (Game|GetPlayerController 0) (LocalVariables|GetSpawnedPawn))
        ;[1 1 1] Set Actor Rotation
        (Transformation|SetActorRotation (LocalVariables|GetSpawnedPawn) (Math|Rotator|MakeRotator 0.0 0.0 (.yaw (Pawn|GetControlRotation (Game|GetPlayerController 0) :!class /Script/Engine.Controller))))))))