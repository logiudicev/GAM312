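; Base zone actor for procedural city generation that holds building definitions and sorts them by footprint.
; Its construction script configures box, triangle and cylinder bounds markers plus a zone name label.
; CategorizeBuildings builds an area-sorted list, then splits buildings into deep, wide and square lists, each ordered by its dominant dimension.
; All ordering uses a hand-written insertion sort that swaps values and buildings in parallel.
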(event Custom|Categorize%20Buildings
  (CallFunction|FnCategorizebyArea)
  (CallFunction|FnCategorizebyShape))

(fn ConstructionScript
  ;[1 1 1] Set the material for the bounds
  (Rendering|Material|SetMaterial (Variables|Default|GetBoundsTriangle) 0 (Variables|Setup|GetMaterial))
  ;[1 1 1] Set Bounds Scale
  (Transformation|SetWorldScale3D (Variables|Default|GetBoundsBox) (Variables|Setup|GetBoundScaleBox))
  (Transformation|SetWorldScale3D (Variables|Default|GetBoundsTriangle) (Variables|Setup|GetBoundScaleTriangle))
  (Transformation|SetWorldScale3D (Variables|Default|GetBoundsCylinder) (Variables|Setup|GetBoundScaleCylinder))
  (Transformation|SetWorldLocation (Variables|Default|GetZoneName) (Transformation|GetWorldLocation (Variables|Default|GetTextAnchor)) false true)
  (Rendering|Components|TextRender|SetText (Variables|Default|GetZoneName) (Variables|Setup|GetZone%20Name))
  ;[1 1 1] Set Marker visibility
  (Rendering|SetVisibility (Variables|Default|GetBoundsBox) (Variables|Setup|GetMarkerVisible) false)
  (Development|SetHiddeninGame (Variables|Default|GetBoundsBox) (Variables|Setup|GetMarkerHidden) false))

(fn FnCategorizebyArea
  ;[1 1 1] Set SortedBuildings to BuildingDetails
  (Variables|Setup-Spawn|SetSortedBuildingsSize (Variables|Setup-Spawn|GetBuildingDetails))
  ;[1 1 1] Loop through all buildings
  (for _array_element (Variables|Setup-Spawn|GetBuildingDetails)
    (LocalVariables|SetBuilding _array_element)
    ;[1 1 1] Add the building area to the AreasList array
    (Utilities|Array|Add (LocalVariables|GetAreasList) (* (.X (Math|Vector2D|BreakVector2D (.Bounds (Utilities|Struct|BreakStruct_BuildingDetails (LocalVariables|GetBuilding))))) (.Y (Math|Vector2D|BreakVector2D (.Bounds (Utilities|Struct|BreakStruct_BuildingDetails (LocalVariables|GetBuilding))))))))
  ;[1 1 1] Sort Buildings by Size
  (bind _sorted_buildings (CallFunction|FnSortValues (LocalVariables|GetAreasList) (Variables|Setup-Spawn|GetBuildingDetails)))
  (Variables|Setup-Spawn|SetSortedBuildingsSize _sorted_buildings))

(fn FnCategorizebyShape
  ;[1 1 1] Clear shape arrays
  (Utilities|Array|Clear (Variables|Setup-Spawn|GetSortedBuildingsDepth))
  (Utilities|Array|Clear (Variables|Setup-Spawn|GetSortedBuildingsWide))
  (Utilities|Array|Clear (Variables|Setup-Spawn|GetSortedBuildingsSquare))
  ;[1 1 1] Loop thorugh all buildings
  (for _array_element (Variables|Setup-Spawn|GetBuildingDetails)
    (LocalVariables|SetBuilding _array_element)
    ;[1 1 1] Is this building more deep than wide?
    (if (> (.X (Math|Vector2D|BreakVector2D (.Bounds (Utilities|Struct|BreakStruct_BuildingDetails (LocalVariables|GetBuilding))))) (.Y (Math|Vector2D|BreakVector2D (.Bounds (Utilities|Struct|BreakStruct_BuildingDetails (LocalVariables|GetBuilding))))))
      ;[1 1 1] Add building to list (Deep)
      (Utilities|Array|Add (Variables|Setup-Spawn|GetSortedBuildingsDepth) (LocalVariables|GetBuilding))
      (else
        ;[1 1 1] Is this building more wide than deep?
        (if (< (.X (Math|Vector2D|BreakVector2D (.Bounds (Utilities|Struct|BreakStruct_BuildingDetails (LocalVariables|GetBuilding))))) (.Y (Math|Vector2D|BreakVector2D (.Bounds (Utilities|Struct|BreakStruct_BuildingDetails (LocalVariables|GetBuilding))))))
          ;[1 1 1] Add building to list (Wide)
          (Utilities|Array|Add (Variables|Setup-Spawn|GetSortedBuildingsWide) (LocalVariables|GetBuilding))
          (else
            ;[1 1 1] Add building to list (Square)
            (Utilities|Array|Add (Variables|Setup-Spawn|GetSortedBuildingsSquare) (LocalVariables|GetBuilding)))))))
  (Utilities|FlowControl|Sequence
    (:then_0
      ;[1 1 1] DEEP
      ;;[1 1 1] Loop through all Deep buildings
      (for _array_element_2 (Variables|Setup-Spawn|GetSortedBuildingsDepth)
        (LocalVariables|SetBuilding _array_element_2)
        ;;[1 1 1] Add the building value to the List array
        (Utilities|Array|Add (LocalVariables|GetList) (.X (Math|Vector2D|BreakVector2D (.Bounds (Utilities|Struct|BreakStruct_BuildingDetails (LocalVariables|GetBuilding)))))))
      ;;[1 1 1] Sort Buildings
      (bind _sorted_buildings (CallFunction|FnSortValues (LocalVariables|GetList) (Variables|Setup-Spawn|GetSortedBuildingsDepth)))
      (Variables|Setup-Spawn|SetSortedBuildingsDepth _sorted_buildings)
      ;;[1 1 1] Clear List
      (Utilities|Array|Clear (LocalVariables|GetList)))
    (:then_1
      ;[1 1 1] WIDE
      ;;[1 1 1] Loop through all Wide buildings
      (for _array_element_3 (Variables|Setup-Spawn|GetSortedBuildingsWide)
        (LocalVariables|SetBuilding _array_element_3)
        ;;[1 1 1] Add the building value to the List array
        (Utilities|Array|Add (LocalVariables|GetList) (.Y (Math|Vector2D|BreakVector2D (.Bounds (Utilities|Struct|BreakStruct_BuildingDetails (LocalVariables|GetBuilding)))))))
      ;;[1 1 1] Sort Buildings
      (bind _sorted_buildings_2 (CallFunction|FnSortValues (LocalVariables|GetList) (Variables|Setup-Spawn|GetSortedBuildingsWide)))
      (Variables|Setup-Spawn|SetSortedBuildingsWide _sorted_buildings_2)
      ;;[1 1 1] Clear List
      (Utilities|Array|Clear (LocalVariables|GetList)))
    (:then_2
      ;[1 1 1] SQUARE
      ;;[1 1 1] Loop through all Square buildings
      (for _array_element_4 (Variables|Setup-Spawn|GetSortedBuildingsSquare)
        (LocalVariables|SetBuilding _array_element_4)
        ;;[1 1 1] Add the building value to the List array
        (Utilities|Array|Add (LocalVariables|GetList) (.Y (Math|Vector2D|BreakVector2D (.Bounds (Utilities|Struct|BreakStruct_BuildingDetails (LocalVariables|GetBuilding)))))))
      ;;[1 1 1] Sort Buildings
      (bind _sorted_buildings_3 (CallFunction|FnSortValues (LocalVariables|GetList) (Variables|Setup-Spawn|GetSortedBuildingsSquare)))
      (Variables|Setup-Spawn|SetSortedBuildingsSquare _sorted_buildings_3)
      ;;[1 1 1] Clear List
      (Utilities|Array|Clear (LocalVariables|GetList)))))

(fn FnSortValues
  (params (Value%20List :type Array%20of%20Floats%20%28single-precision%29) (Building%20List :type Array%20of%20Struct%20Building%20Details%20Structures))
  (LocalVariables|SetValueList Value%20List)
  (LocalVariables|SetBuildingList Building%20List)
  ;[1 1 1] INSERTION SORT CODE
  ;;[1 1 1] Loop while i is less than the length of the array
  (while (< (LocalVariables|Geti) (Utilities|Array|Length (LocalVariables|GetValueList)))
    ;;[1 1 1] Set j to the value of i
    (LocalVariables|Setj (LocalVariables|Geti))
    ;;[1 1 1] Loop while the J is bigger than 0 and the value of array in pos j-1 is bigger than position j
    (while (and (> (LocalVariables|Getj) 0) (> (Utilities|Array|Get(acopy) (LocalVariables|GetValueList) (- (LocalVariables|Getj) 1)) (Utilities|Array|Get(acopy) (LocalVariables|GetValueList) (LocalVariables|Getj))))
      (Utilities|FlowControl|Sequence
        (:then_0
          ;;[1 1 1] Swap values
          (Utilities|Array|Swap (LocalVariables|GetValueList) (LocalVariables|Getj) (- (LocalVariables|Getj) 1))
          ;;[1 1 1] Swap buildings
          (Utilities|Array|Swap (LocalVariables|GetBuildingList) (LocalVariables|Getj) (- (LocalVariables|Getj) 1)))
        (:then_1
          ;;[1 1 1] Decrease j by 1
          (Math|Integer|DecrementInt (LocalVariables|Getj)))))
    ;;[1 1 1] Increase i by 1
    (Math|Integer|IncrementInt (LocalVariables|Geti)))
  (return (LocalVariables|GetBuildingList)))