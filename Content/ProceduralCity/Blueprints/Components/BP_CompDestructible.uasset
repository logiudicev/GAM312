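; Actor component that makes its owner destructible, swapping it for a spawned destructible class when health runs out.
; Damage events only store the amount; actor hits subtract it from health after a short delay.
; At zero health it hides the owner, spawns the replacement and tells PCG building interiors to simulate physics.
; Debris impulse, sound, cleanup and owner destruction are present but disconnected, so they never run.
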(event Custom|EventReceivedDamage
  (params (DamagedActor :type Actor%20Object%20Reference) (Damage :type Float%20%28single-precision%29) (DamageType :type Damage%20Type%20Object%20Reference) (InstigatedBy :type Controller%20Object%20Reference) (DamageCauser :type Actor%20Object%20Reference))
  ;[1 1 1] Bind on Damage event
  (Variables|Default|SetDamageAmount Damage))

(event Custom|EventHit
  (params (SelfActor :type Actor%20Object%20Reference) (OtherActor :type Actor%20Object%20Reference) (NormalImpulse :type Vector) (Hit :type Hit%20Result%20Structure%20%28by%20ref%29))
  (bind (_bblockinghit _binitialoverlap _time _distance _location _impactpoint _normal _impactnormal) (Collision|BreakHitResult Hit))
  ;[1 1 1] Bind OnActorHit event
  (Variables|Default|SetHitLocation _impactpoint)
  (Variables|Default|SetImpactNormal _impactnormal)
  (CallFunction|EventApplyDamage))

(event EventBeginPlay
  (if (and (Variables|Setup|GetActive) (Utilities|IsValidClass (Variables|Setup|GetDMClass)))
    ;[1 1 1] Bind OnActorHit event
    (Collision|BindEventtoOnActorHit (Components|GetOwner) (delegate Custom|EventHit))
    ;[1 1 1] Bind on Damage event
    (EventDispatchers|BindEventtoOnTakeAnyDamage (Components|GetOwner) (delegate Custom|EventReceivedDamage))))

(event Custom|EventApplyDamage
  (params (DMRef :type Actor%20Object%20Reference))
  (Variables|Default|SetDMRef DMRef)
  (Utilities|FlowControl|Delay 0.1)
  ;[1 1 1] Set new Total Health
  (Variables|Setup|SetTotalHealth (- (Variables|Setup|GetTotalHealth) (Variables|Default|GetDamageAmount)))
  ;[1 1 1] Check if the HP is 0 or less
  (if (<= (Variables|Setup|GetTotalHealth) 0.0)
    ;[1 1 1] Save the Owner's Transform
    (Variables|Default|SetNewDMTransform (Transformation|GetActorTransform (Components|GetOwner)))
    ;[1 1 1] Hide the Owner
    (Rendering|SetActorHiddenInGame (Components|GetOwner) true)
    ;[1 1 1] Disable Owner collision
    (Collision|SetActorEnableCollision (Components|GetOwner) false)
    ;[1 1 1] Spawn destructible class
    (bind _returnvalue (Game|SpawnActorfromClass (Variables|Setup|GetDMClass) (Variables|Default|GetNewDMTransform) "AlwaysSpawn" 0 0))
    (Variables|Default|SetDMRef _returnvalue)
    ;[1 1 1] Set all spawned objects to simulate physics
    (bind _asbp_pcgbuilding_base (Utilities|Casting|CastToBP_PCGBuilding_Base (Components|GetOwner))
      (:then
        (Class|BPBPIPCGBuildingInterior|FnSimulatePhysicsAllActors(Message) (Variables|/Game/ProceduralCity/Blueprints/Buildings/BP_PCGBuilding_Base.BP_PCGBuilding_Base_C|GetInteriorActor _asbp_pcgbuilding_base)))
      (:CastFailed
        _))
    ;[1 1 1] Simulate physics and apply damage to destructible mesh
    (Utilities|IsValid (Variables|Default|GetDMRef))))