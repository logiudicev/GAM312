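; Base Blueprint for a simple procedural city building, made from one scaled mesh sized by depth, width and floor count.
; Construction script either applies set dimensions or, with RandomOnMove, randomizes size and optionally picks a listed material, then handles bounds and cull distance.
; Interface events re-randomize floors and material, assign a zone type and set cull distance.
; Destroy is empty with disconnected damage nodes, and FnGetBounds returns zeros.
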(fn ConstructionScript
  (if (Variables|Setup-Random|GetRandomOnMove?)
    (CallFunction|RandomSize)
    (if (Variables|Setup-Random|GetRandomMaterial)
      (CallFunction|RandomizeMaterial)
      (Variables|Setup|SetCurrentBounds (* (.BoxExtent (Collision|GetComponentBounds (Variables|Default|GetMesh))) 2.0) :!label _label)
      (Class|PrimitiveComponent|SetCullDistance (Variables|Default|GetMesh) (Variables|Setup|GetCullDistance)))
    (else
      (CallFunction|SetSize)
      (goto _label))))

(event Custom|RandomSize
  (bind _floorrange (Variables|Setup-Random|GetFloorRange))
  (bind _depthrange (Variables|Setup-Random|GetDepthRange))
  (bind _widthrange (Variables|Setup-Random|GetWidthRange))
  (Variables|Setup|SetDepth (Math|Float|Truncate (Math|Random|RandomFloatinRange (.x _depthrange) (.y _depthrange))))
  (Variables|Setup|SetWidth (Math|Float|Truncate (Math|Random|RandomFloatinRange (.x _widthrange) (.y _widthrange))))
  (Variables|Setup|SetNumberOfFloors (Math|Float|Truncate (Math|Random|RandomFloatinRange (.x _floorrange) (.y _floorrange))))
  (CallFunction|SetSize))

(event Custom|RandomFloors
  (bind _floorrange (Variables|Setup-Random|GetFloorRange))
  (Variables|Setup|SetNumberOfFloors (Math|Float|Truncate (Math|Random|RandomFloatinRange (.x _floorrange) (.y _floorrange))))
  (CallFunction|SetSize))

(event Custom|RandomizeMaterial
  (Variables|Setup|SetMaterial (Utilities|Array|Get(acopy) (Variables|Setup-Random|GetMaterialList) (Math|Random|RandomIntegerinRange 0 (- (Utilities|Array|Length (Variables|Setup-Random|GetMaterialList)) 1))))
  (CallFunction|SetMaterial))

(event Custom|Destroy
  (params (DamageCauser :type Actor%20Object%20Reference)))

(event EventFnSetParameters
  ;[1 1 1] Interface calls
  (CallFunction|RandomFloors)
  (CallFunction|RandomizeMaterial)
  (Class|PrimitiveComponent|SetCullDistance (Variables|Default|GetMesh) (Variables|Setup|GetCullDistance)))

(event EventFnSetBuildingZone
  (params (Zone :type Enum_ZoneType%20Enum :default "NewEnumerator0"))
  ;[1 1 1] Interface calls
  (Variables|Setup|SetZoneType Zone))

(event EventFnSetCullDistance
  (params (Cull%20Distance :type Float%20%28single-precision%29))
  ;[1 1 1] Interface calls
  (Class|PrimitiveComponent|SetCullDistance (Variables|Default|GetMesh) Cull%20Distance))

(event Custom|SetSize
  (Transformation|SetWorldScale3D (Variables|Default|GetMesh) (Math|Vector|MakeVector (* (Variables|Setup|GetDepth) (Variables|Default|GetUnitConversion)) (* (Variables|Setup|GetWidth) (Variables|Default|GetUnitConversion)) (* (Variables|Setup|GetNumberOfFloors) (Variables|Default|GetUnitConversion)))))

(event Custom|SetMaterial
  (Rendering|Material|SetMaterial (Variables|Default|GetMesh) 0 (Variables|Setup|GetMaterial)))

(fn FnGetBounds
  (return "0, 0, 0" "0, 0, 0"))

(fn FnGetBuildingZone
  (return (Variables|Setup|GetZoneType)))