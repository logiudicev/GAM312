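; Base actor for a procedural building's interior floor that spawns its furnishings when a player enters its trigger, on load events, or at start.
; BeginPlay matches parent building rotation and rolls per-actor spawn chances from a seeded stream for static, interactive and random lists.
; Spawned actors register with the parent interior; on exit, despawnable ones are hidden (optionally destroyed later) or destroyed.
; PopulateInteractiveList captures tagged props as parent-relative spawn entries.
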(event OnComponentBeginOverlap(Trigger)
  (params (OverlappedComponent :type Primitive%20Component%20Object%20Reference) (OtherActor :type Actor%20Object%20Reference) (OtherComp :type Primitive%20Component%20Object%20Reference) (OtherBodyIndex :type Integer) (bFromSweep :type Boolean) (SweepResult :type Hit%20Result%20Structure%20%28by%20ref%29))
  ;[1 1 1] Did we overlap a Player?
  (if (Actor|ActorHasTag OtherActor "Player")
    (if (Variables|Default|GetCanOverlap)
      (Variables|Default|SetOverlapped true)
      (Utilities|FlowControl|DoOnce false
        (:Completed
          (Utilities|FlowControl|Sequence
            (:then_0
              (Variables|Default|SetCanDespawn false)
              (if (Variables|Default|GetFirstSpawn?)
                (CallFunction|FnSpawnObjects)
                (Variables|Default|SetFirstSpawn? false)
                (else
                  (switch Utilities|FlowControl|Switch|SwitchonEnum_InteriorDespawnMethod (Variables|Setup|GetDespawnMethod)
                    (:NewEnumerator0
                      ;[1 1 1] Check that we have at least 1 spawned object to show
                      (if (> (Utilities|Map|Length (Variables|Default|GetSpawnedActors)) 0)
                        (CallFunction|FnShowObjects)
                        (else
                          (CallFunction|FnSpawnObjects))))
                    (:NewEnumerator1
                      (CallFunction|FnSpawnObjects))))))
            (:then_1
              (Utilities|FlowControl|Delay 0.5)
              (Variables|Default|SetCanDespawn true))))))))

(event OnComponentEndOverlap(Trigger)
  (params (OverlappedComponent :type Primitive%20Component%20Object%20Reference) (OtherActor :type Actor%20Object%20Reference) (OtherComp :type Primitive%20Component%20Object%20Reference) (OtherBodyIndex :type Integer))
  ;[1 1 1] Did we overlap the Player?
  (if (Actor|ActorHasTag OtherActor "Player")
    (if (Variables|Default|GetCanOverlap)
      (Utilities|FlowControl|Sequence
        (:then_0
          (Utilities|FlowControl|DoOnce false) ; enters at Reset
        )
        (:then_1
          (Variables|Default|SetOverlapped false)
          (Utilities|FlowControl|Delay 1.0)
          (if (Variables|Default|GetCanDespawn)
            (switch Utilities|FlowControl|Switch|SwitchonEnum_InteriorDespawnMethod (Variables|Setup|GetDespawnMethod)
              (:NewEnumerator0
                (CallFunction|FnHideObjects)
                ;[1 1 1] Do we want Delayed Destruction of spawned objects?
                (if (Variables|Setup|GetDelayedDestruction)
                  ;[1 1 1] Wait Delay Destruction Time
                  (Utilities|FlowControl|RetriggerableDelay (Variables|Setup|GetDelayDestructionTime))
                  (if (not (Variables|Default|GetOverlapped))
                    ;[1 1 1] Destroy spawned objects
                    (CallFunction|FnDestroyObjects))))
              (:NewEnumerator1
                (CallFunction|FnDestroyObjects)))))))))

(event Custom|Populate%20Interactive%20List
  (CallFunction|FnGetInteractiveProps))

(event Custom|EventLoadInteriors
  (Variables|Default|SetOverlapped true)
  (Utilities|FlowControl|DoOnce false
    (:Completed
      (Utilities|FlowControl|Sequence
        (:then_0
          (Variables|Default|SetCanDespawn false)
          (if (Variables|Default|GetFirstSpawn?)
            (CallFunction|FnSpawnObjects)
            (Variables|Default|SetFirstSpawn? false)
            (else
              (switch Utilities|FlowControl|Switch|SwitchonEnum_InteriorDespawnMethod (Variables|Setup|GetDespawnMethod)
                (:NewEnumerator0
                  ;[1 1 1] Check that we have at least 1 spawned object to show
                  (if (> (Utilities|Map|Length (Variables|Default|GetSpawnedActors)) 0)
                    (CallFunction|FnShowObjects)
                    (else
                      (CallFunction|FnSpawnObjects))))
                (:NewEnumerator1
                  (CallFunction|FnSpawnObjects))))))
        (:then_1
          (Utilities|FlowControl|Delay 0.5)
          (Variables|Default|SetCanDespawn true))))))

(event Custom|EventUnloadInteriors
  (Utilities|FlowControl|Sequence
    (:then_0
      (Utilities|FlowControl|DoOnce false) ; enters at Reset
    )
    (:then_1
      (Variables|Default|SetOverlapped false)
      (Utilities|FlowControl|Delay 1.0)
      (if (Variables|Default|GetCanDespawn)
        (switch Utilities|FlowControl|Switch|SwitchonEnum_InteriorDespawnMethod (Variables|Setup|GetDespawnMethod)
          (:NewEnumerator0
            (CallFunction|FnHideObjects)
            ;[1 1 1] Do we want Delayed Destruction of spawned objects?
            (if (Variables|Setup|GetDelayedDestruction)
              ;[1 1 1] Wait Delay Destruction Time
              (Utilities|FlowControl|RetriggerableDelay (Variables|Setup|GetDelayDestructionTime))
              (if (not (Variables|Default|GetOverlapped))
                ;[1 1 1] Destroy spawned objects
                (CallFunction|FnDestroyObjects))))
          (:NewEnumerator1
            (CallFunction|FnDestroyObjects)))))))

(event EventBeginPlay
  ;[1 1 1] Set initial parameters
  (CallFunction|FnGetRandomStaticActor)
  (CallFunction|FnSetRelativeRotation)
  (Utilities|FlowControl|Delay 0.05)
  (CallFunction|FnCalculateSpawnChance)
  (if (Variables|Default|GetStartLoaded)
    (Variables|Default|SetOverlapped true)
    (Utilities|FlowControl|DoOnce false
      (:Completed
        (Utilities|FlowControl|Sequence
          (:then_0
            (Variables|Default|SetCanDespawn false)
            (if (Variables|Default|GetFirstSpawn?)
              (CallFunction|FnSpawnObjects)
              (Variables|Default|SetFirstSpawn? false)
              (else
                (switch Utilities|FlowControl|Switch|SwitchonEnum_InteriorDespawnMethod (Variables|Setup|GetDespawnMethod)
                  (:NewEnumerator0
                    ;[1 1 1] Check that we have at least 1 spawned object to show
                    (if (> (Utilities|Map|Length (Variables|Default|GetSpawnedActors)) 0)
                      (CallFunction|FnShowObjects)
                      (else
                        (CallFunction|FnSpawnObjects))))
                  (:NewEnumerator1
                    (CallFunction|FnSpawnObjects))))))
          (:then_1
            (Utilities|FlowControl|Delay 0.5)
            (Variables|Default|SetCanDespawn true)))))))

(fn ConstructionScript
  (Rendering|SetVisibility (Variables|Default|GetTrigger) (Variables|Setup|GetTriggerVisible) false)
  (Development|SetHiddeninGame (Variables|Default|GetTrigger) (Variables|Setup|GetTriggerHidden) false)
  (Transformation|SetWorldScale3D (Variables|Default|GetTrigger) (Variables|Setup|GetTriggerScale))
  (|DISPLAYHELPERLOCATION))

(fn FnSpawnObjects
  ;[1 1 1] Clear the Spawned Objects array
  (Utilities|Map|Clear (Variables|Default|GetSpawnedActors))
  (Utilities|FlowControl|Sequence
    (:then_0
      ;[1 1 1] Spawn Random Static Actor?
      (if (Variables|Setup|GetSpawnRandomStaticActor?)
        (LocalVariables|SetActor (Variables|Default|GetRandomStaticActor))
        ;[1 1 1] Do we spawn this actor?
        (if (and (.Value (Utilities|Map|Find (Variables|Default|GetSpawnListStatic) (LocalVariables|GetIndex))) (.ReturnValue (Utilities|Map|Find (Variables|Default|GetSpawnListStatic) (LocalVariables|GetIndex)))) :!label _label
          ;[1 1 1] Set Location Helper location
          (Transformation|SetRelativeTransform (Variables|Default|GetLocationHelper) (Utilities|Struct|BreakStruct_InteriorActors (LocalVariables|GetActor)) false true)
          ;[1 1 1] Is this the first spawn or is this actor  allowed to despawn?
          (if (or (Variables|Default|GetFirstSpawn?) (Utilities|Struct|BreakStruct_InteriorActors (LocalVariables|GetActor)))
            ;[1 1 1] Spawn actor
            (bind _returnvalue (Game|SpawnActorfromClass (Utilities|Struct|BreakStruct_InteriorActors (LocalVariables|GetActor)) (Transformation|GetWorldTransform (Variables|Default|GetLocationHelper)) "AlwaysSpawn" 0 0))
            (LocalVariables|SetSpawnedActor _returnvalue)
            ;[1 1 1] Add reference to SpawnedObjects array
            (Utilities|Map|Add (Variables|Default|GetSpawnedActors) (LocalVariables|GetSpawnedActor) (Utilities|Struct|BreakStruct_InteriorActors (LocalVariables|GetActor)))))
        (else
          ;[1 1 1] Go through all Static Actors
          (for (_array_element _array_index) (Variables|Setup|GetStaticActorList)
            (LocalVariables|SetActor _array_element)
            (LocalVariables|SetIndex _array_index)
            (goto _label)))))
    (:then_1
      ;[1 1 1] Go through all Interactive Actors
      (for (_array_element_2 _array_index_2) (Variables|Setup|GetInteractiveActorList)
        (LocalVariables|SetActor _array_element_2)
        (LocalVariables|SetIndex _array_index_2)
        ;[1 1 1] Do we spawn this actor?
        (if (and (.Value (Utilities|Map|Find (Variables|Default|GetSpawnListInteractive) (LocalVariables|GetIndex))) (.ReturnValue (Utilities|Map|Find (Variables|Default|GetSpawnListInteractive) (LocalVariables|GetIndex))))
          ;[1 1 1] Set Location Helper location
          (Transformation|SetRelativeTransform (Variables|Default|GetLocationHelper) (Utilities|Struct|BreakStruct_InteriorActors (LocalVariables|GetActor)) false true)
          ;[1 1 1] Is this the first spawn or is this actor  allowed to despawn?
          (if (or (Variables|Default|GetFirstSpawn?) (Utilities|Struct|BreakStruct_InteriorActors (LocalVariables|GetActor)))
            ;[1 1 1] Spawn actor
            (bind _returnvalue_2 (Game|SpawnActorfromClass (Utilities|Struct|BreakStruct_InteriorActors (LocalVariables|GetActor)) (Transformation|GetWorldTransform (Variables|Default|GetLocationHelper)) "AlwaysSpawn" 0 0))
            (LocalVariables|SetSpawnedActor _returnvalue_2)
            ;[1 1 1] Add reference to SpawnedObjects array
            (Utilities|Map|Add (Variables|Default|GetSpawnedActors) (LocalVariables|GetSpawnedActor) (Utilities|Struct|BreakStruct_InteriorActors (LocalVariables|GetActor)))))))
    (:then_2
      ;[1 1 1] Go through all Interactive Actors
      (for (_array_element_3 _array_index_3) (Variables|Setup|GetRandomActorList)
        (LocalVariables|SetActor _array_element_3)
        (LocalVariables|SetIndex _array_index_3)
        ;[1 1 1] Do we spawn this actor?
        (if (and (.Value (Utilities|Map|Find (Variables|Default|GetSpawnListRandom) (LocalVariables|GetIndex))) (.ReturnValue (Utilities|Map|Find (Variables|Default|GetSpawnListRandom) (LocalVariables|GetIndex))))
          ;[1 1 1] Set Location Helper location
          (Transformation|SetRelativeTransform (Variables|Default|GetLocationHelper) (Utilities|Struct|BreakStruct_InteriorActors (LocalVariables|GetActor)) false true)
          ;[1 1 1] Is this the first spawn or is this actor  allowed to despawn?
          (if (or (Variables|Default|GetFirstSpawn?) (Utilities|Struct|BreakStruct_InteriorActors (LocalVariables|GetActor)))
            ;[1 1 1] Spawn actor
            (bind _returnvalue_3 (Game|SpawnActorfromClass (Utilities|Struct|BreakStruct_InteriorActors (LocalVariables|GetActor)) (Transformation|GetWorldTransform (Variables|Default|GetLocationHelper)) "AlwaysSpawn" 0 0))
            (LocalVariables|SetSpawnedActor _returnvalue_3)
            ;[1 1 1] Add reference to SpawnedObjects array
            (Utilities|Map|Add (Variables|Default|GetSpawnedActors) (LocalVariables|GetSpawnedActor) (Utilities|Struct|BreakStruct_InteriorActors (LocalVariables|GetActor)))))))
    (:then_3
      (CallFunction|FnSetSpawnedActorstoParent))))

(fn FnDestroyObjects
  ;[1 1 1] Loop through the Spawned Actors
  (bind _keys (Utilities|Map|Keys (Variables|Default|GetSpawnedActors)))
  (for _array_element _keys
    (bind _output_get (LocalVariables|SetActor _array_element))
    (Utilities|IsValid _output_get
      (:Is%20Valid
        ;[1 1 1] Can we Despawn the actor?
        (if (.Value (Utilities|Map|Find (Variables|Default|GetSpawnedActors) (LocalVariables|GetActor)))
          ;[1 1 1] Destroy Actor
          (Actor|DestroyActor (LocalVariables|GetActor)))))))

(fn FnHideObjects
  ;[1 1 1] Loop through all Spawned Actors
  (bind _keys (Utilities|Map|Keys (Variables|Default|GetSpawnedActors)))
  (for _array_element _keys
    (bind _output_get (LocalVariables|SetActor _array_element))
    (Utilities|IsValid _output_get
      (:Is%20Valid
        ;[1 1 1] Can we Despawn the actor?
        (if (and (.Value (Utilities|Map|Find (Variables|Default|GetSpawnedActors) (LocalVariables|GetActor))) (.ReturnValue (Utilities|Map|Find (Variables|Default|GetSpawnedActors) (LocalVariables|GetActor))))
          ;[1 1 1] Hide Actor
          (Rendering|SetActorHiddenInGame (LocalVariables|GetActor) true))))))

(fn FnShowObjects
  ;[1 1 1] Loop through the Spawned Actors
  (bind _keys (Utilities|Map|Keys (Variables|Default|GetSpawnedActors)))
  (for _array_element _keys
    (bind _output_get (LocalVariables|SetActor _array_element))
    (Utilities|IsValid _output_get
      (:Is%20Valid
        ;[1 1 1] Can we Despawn the actor?
        (if (and (.Value (Utilities|Map|Find (Variables|Default|GetSpawnedActors) (LocalVariables|GetActor))) (.ReturnValue (Utilities|Map|Find (Variables|Default|GetSpawnedActors) (LocalVariables|GetActor))))
          ;[1 1 1] Show Actor
          (Rendering|SetActorHiddenInGame (LocalVariables|GetActor) false))))))

(fn FnGetRandomStaticActor
  (bind _staticactorlist (Variables|Setup|GetStaticActorList))
  ;[1 1 1] Select a random static actor
  (Variables|Default|SetRandomStaticActor (Utilities|Array|Get(acopy) _staticactorlist (Math|Random|RandomIntegerinRange 0 (Utilities|Array|LastIndex _staticactorlist)))))

(fn FnSetRelativeRotation
  (Utilities|IsValid (Variables|Setup|GetParentBuilding)
    (:Is%20Valid
      ;[1 1 1] Match the parent building's rotation
      (Transformation|SetActorRotation (Transformation|GetWorldRotation (Variables|/Game/ProceduralCity/Blueprints/Buildings/BP_PCGBuilding_Base.BP_PCGBuilding_Base_C|GetBuildingMesh (Variables|Setup|GetParentBuilding))) true))))

(fn FnGetInteractiveProps
  ;[1 1 1] Clear list
  (Utilities|Array|Clear (Variables|Setup|GetInteractiveActorList))
  (bind _outactors (Actor|GetAllActorswithTag (Variables|Setup|GetInteractivePropTag)))
  (for _array_element _outactors
    (LocalVariables|SetProp _array_element)
    ;[1 1 1] Save the prop information
    (Utilities|Array|Add (Variables|Setup|GetInteractiveActorList) (Utilities|Struct|MakeStruct_InteriorActors (Utilities|GetClass (LocalVariables|GetProp)) (Math|Transform|MakeTransform (- (Transformation|GetActorLocation (LocalVariables|GetProp)) (Transformation|GetActorLocation (Actor|GetAttachParentActor (LocalVariables|GetProp)))) (Math|Rotator|MakeRotator 0.0 0.0 (- (.yaw (Transformation|GetActorRotation (LocalVariables|GetProp))) (.yaw (Transformation|GetActorRotation (Actor|GetAttachParentActor (LocalVariables|GetProp))))))) 1.0 true))))

(fn FnCalculateSpawnChance
  (Utilities|FlowControl|Sequence
    (:then_0
      ;[1 1 1] Go through all static actors
      (for (_array_element _array_index) (Variables|Setup|GetStaticActorList)
        (LocalVariables|SetActor _array_element)
        (LocalVariables|SetIndex _array_index)
        ;[1 1 1] Do we spawn this actor?
        (if (>= (Math|Float|Clamp(Float) (Utilities|Struct|BreakStruct_InteriorActors (LocalVariables|GetActor))) (Math|Random|RandomFloatinRangefromStream 0.0 1.0 (Variables|Setup|GetRandomSeed)))
          ;[1 1 1] This actor can spawn
          (Utilities|Map|Add (Variables|Default|GetSpawnListStatic) (LocalVariables|GetIndex) true)
          (else
            ;[1 1 1] This actor cannot spawn
            (Utilities|Map|Add (Variables|Default|GetSpawnListStatic) (LocalVariables|GetIndex) false)))))
    (:then_1
      ;[1 1 1] Go through all interactive actors
      (for (_array_element_2 _array_index_2) (Variables|Setup|GetInteractiveActorList)
        (LocalVariables|SetActor _array_element_2)
        (LocalVariables|SetIndex _array_index_2)
        ;[1 1 1] Do we spawn this actor?
        (if (>= (Math|Float|Clamp(Float) (Utilities|Struct|BreakStruct_InteriorActors (LocalVariables|GetActor))) (Math|Random|RandomFloatinRangefromStream 0.0 1.0 (Variables|Setup|GetRandomSeed)))
          ;[1 1 1] This actor can spawn
          (Utilities|Map|Add (Variables|Default|GetSpawnListInteractive) (LocalVariables|GetIndex) true)
          (else
            ;[1 1 1] This actor cannot spawn
            (Utilities|Map|Add (Variables|Default|GetSpawnListInteractive) (LocalVariables|GetIndex) false)))))
    (:then_2
      ;[1 1 1] Go through all random actors
      (for (_array_element_3 _array_index_3) (Variables|Setup|GetRandomActorList)
        (LocalVariables|SetActor _array_element_3)
        (LocalVariables|SetIndex _array_index_3)
        ;[1 1 1] Do we spawn this actor?
        (if (>= (Math|Float|Clamp(Float) (Utilities|Struct|BreakStruct_InteriorActors (LocalVariables|GetActor))) (Math|Random|RandomFloatinRangefromStream 0.0 1.0 (Variables|Setup|GetRandomSeed)))
          ;[1 1 1] This actor can spawn
          (Utilities|Map|Add (Variables|Default|GetSpawnListRandom) (LocalVariables|GetIndex) true)
          (else
            ;[1 1 1] This actor cannot spawn
            (Utilities|Map|Add (Variables|Default|GetSpawnListRandom) (LocalVariables|GetIndex) false)))))))

(fn FnSetSpawnedActorstoParent
  ;[1 1 1] Get Parent Interior BP reference
  (bind _asbp_interior_base (Utilities|Casting|CastToBP_Interior_Base (Variables|Default|GetParentInteriorBP)))
  (LocalVariables|SetParent _asbp_interior_base)
  ;[1 1 1] Add all spawned actors to the Spawned Static Actors array in the Parent
  (bind _keys (Utilities|Map|Keys (Variables|Default|GetSpawnedActors)))
  (for _array_element _keys
    (Utilities|Array|Add (Variables|/Game/ProceduralCity/Blueprints/Buildings/Interiors/BaseClasses/BP_Interior_Base.BP_Interior_Base_C|GetSpawnedObjectsList (LocalVariables|GetParent)) _array_element)))