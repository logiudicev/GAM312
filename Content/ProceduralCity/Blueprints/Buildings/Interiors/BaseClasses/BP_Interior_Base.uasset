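; Base Blueprint for procedural city building interiors, spawning contents when the player enters a trigger fitted to the parent building.
; Floor actors spawn per all, ranged or listed floors, receiving per-floor seeds.
; Global props spawn from relative transforms after a stream-based chance roll.
; On exit, props are hidden or destroyed, optionally after a delay, and parent-building collision can be toggled with player presence.
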(event OnComponentBeginOverlap(Trigger)
  (params (OverlappedComponent :type Primitive%20Component%20Object%20Reference) (OtherActor :type Actor%20Object%20Reference) (OtherComp :type Primitive%20Component%20Object%20Reference) (OtherBodyIndex :type Integer) (bFromSweep :type Boolean) (SweepResult :type Hit%20Result%20Structure%20%28by%20ref%29))
  ;[1 1 1] Did we overlap the Player?
  (if (Actor|ActorHasTag OtherActor "Player")
    (Utilities|FlowControl|DoOnce false
      (:Completed
        ;[1 1 1] Enable Collision
        (if (and (Variables|Setup|GetDisableCollision) (Utilities|IsValid (Variables|Setup|GetParentBuilding)))
          (Collision|SetActorEnableCollision (Variables|Setup|GetParentBuilding) true))
        ;[1 1 1] Load Interiors
        (CallFunction|EventLoadInteriors)
        (Utilities|FlowControl|Sequence
          (:then_0
            (Variables|Default|SetCanDespawn false)
            (Variables|Default|SetOverlapped true)
            (if (Variables|Default|GetFirstSpawn?)
              (CallFunction|FnSpawnObjects)
              (Variables|Default|SetFirstSpawn? false)
              (else
                (switch Utilities|FlowControl|Switch|SwitchonEnum_InteriorDespawnMethod (Variables|GlobalSpawns|GetDespawnMethod)
                  (:NewEnumerator0
                    ;[1 1 1] Check that we have at least 1 spawned object to show
                    (if (> (Utilities|Map|Length (Variables|Default|GetSpawnedActors)) 0)
                      (CallFunction|FnShowObjects)
                      (else
                        (CallFunction|FnSpawnObjects))))
                  (:NewEnumerator1
                    (CallFunction|FnSpawnObjects))))))
          (:then_1
            (Utilities|FlowControl|Delay 0.5)
            (Variables|Default|SetCanDespawn true)))))))

(event OnComponentEndOverlap(Trigger)
  (params (OverlappedComponent :type Primitive%20Component%20Object%20Reference) (OtherActor :type Actor%20Object%20Reference) (OtherComp :type Primitive%20Component%20Object%20Reference) (OtherBodyIndex :type Integer))
  ;[1 1 1] Did we overlap the Player?
  (if (Actor|ActorHasTag OtherActor "Player")
    (Utilities|FlowControl|Sequence
      (:then_0
        (Utilities|FlowControl|DoOnce false) ; enters at Reset
      )
      (:then_1
        ;[1 1 1] Disable Collision
        (if (and (Variables|Setup|GetDisableCollision) (Utilities|IsValid (Variables|Setup|GetParentBuilding)))
          (Collision|SetActorEnableCollision (Variables|Setup|GetParentBuilding) false))
        (CallFunction|EventUnloadInteriors)
        (Variables|Default|SetOverlapped false)
        (Utilities|FlowControl|Delay 1.0)
        (if (Variables|Default|GetCanDespawn)
          (switch Utilities|FlowControl|Switch|SwitchonEnum_InteriorDespawnMethod (Variables|GlobalSpawns|GetDespawnMethod)
            (:NewEnumerator0
              (CallFunction|FnHideObjects)
              ;[1 1 1] Do we want Delayed Destruction of spawned objects?
              (if (Variables|GlobalSpawns|GetDelayedDestruction)
                ;[1 1 1] Wait Delay Destruction Time
                (Utilities|FlowControl|RetriggerableDelay (Variables|GlobalSpawns|GetDelayDestructionTime))
                (if (not (Variables|Default|GetOverlapped))
                  ;[1 1 1] Destroy spawned objects
                  (CallFunction|FnDestroyObjects))))
            (:NewEnumerator1
              (CallFunction|FnDestroyObjects))))))))

(event Custom|RandomizeSeeds
  (CallFunction|FnRandomizeSeed))

(event EventBeginPlay
  (bind _parentbuilding (Variables|Setup|GetParentBuilding))
  ;[1 1 1] Wait a random delay
  (Utilities|FlowControl|Delay (Math|Random|RandomFloatinRange 0.0 0.2))
  ;[1 1 1] Set initial parameters
  (CallFunction|FnSetTriggerSize)
  (CallFunction|FnCalculateFloors)
  (CallFunction|FnSetRelativeRotation)
  (CallFunction|FnCalculateSpawnChance)
  ;[1 1 1] Do we start with interiors loaded?
  (if (Variables|Setup|GetStartLoaded)
    ;[1 1 1] Load interiors
    (CallFunction|EventLoadInteriors)
    (CallFunction|FnSpawnObjects)
    (Variables|Default|SetFirstSpawn? false)
    (else
      ;[1 1 1] Wait random time
      (Utilities|FlowControl|Delay (Math|Random|RandomFloatinRange 0.0 0.3))
      ;[1 1 1] Disable Collision
      (if (Variables|Setup|GetDisableCollision)
        (Utilities|IsValid _parentbuilding
          (:Is%20Valid
            (Collision|SetActorEnableCollision _parentbuilding false)))))))

(fn ConstructionScript
  (CallFunction|FnSetTriggerSize)
  (CallFunction|FnCalculateFloors)
  (Rendering|SetVisibility (Variables|Default|GetTrigger) (Variables|Setup|GetShowTrigger) false)
  (Development|SetHiddeninGame (Variables|Default|GetTrigger) (Variables|Setup|GetTriggerHidden) false))

(fn FnSetTriggerSize
  (bind _parentbuilding (Variables|Setup|GetParentBuilding))
  (bind _triggerscale (Variables|Setup|GetTriggerScale))
  (bind _buildingmesh (Variables|/Game/ProceduralCity/Blueprints/Buildings/BP_PCGBuilding_Base.BP_PCGBuilding_Base_C|GetBuildingMesh _parentbuilding))
  (bind _staticmesh (Variables|/Script/Engine.StaticMeshComponent|GetStaticMesh _buildingmesh))
  (bind _returnvalue (StaticMesh|GetBounds _staticmesh))
  (bind (_origin _boxextent) (Math|BoxSphereBounds|BreakBoxSphereBounds _returnvalue))
  (Utilities|IsValid (Variables|Setup|GetParentBuilding)
    (:Is%20Valid
      ;[1 1 1] Set Interior to the parent building's location
      (Transformation|SetActorLocation (Transformation|GetActorLocation (Variables|Setup|GetParentBuilding)) false true)
      ;[1 1 1] Align and resize the trigger with the parent building's box extent
      (Transformation|SetRelativeLocation (Variables|Default|GetTrigger) _origin false true)
      (Transformation|SetWorldScale3D (Variables|Default|GetTrigger) (Math|Vector|MakeVector (.x _triggerscale) (.y _triggerscale) (/ (.z (* (* _boxextent (Transformation|GetActorScale3D _parentbuilding)) (Variables|Setup|GetTriggerHeightMultiplier))) 32.0))))
    (:Is%20Not%20Valid
      (Transformation|SetWorldScale3D (Variables|Default|GetTrigger) (Variables|Setup|GetTriggerScale)))))

(fn FnSpawnFloorActors
  ;[1 1 1] Loop through all Floor Actors
  (for _array_element (Variables|Setup|GetFloorActors)
    (LocalVariables|SetFloor _array_element)
    ;[1 1 1] Switch on the Floor Setup of this Floor Actor
    (switch Utilities|FlowControl|Switch|SwitchonEnum_Interior_FloorSetup (Utilities|Struct|BreakStruct_Interior_Floor (LocalVariables|GetFloor))
      (:NewEnumerator0
        ;[1 1 1] Loop through all the floors
        (for _index (range 0 (- (Utilities|Struct|BreakStruct_Interior_FloorSetup (Variables|Setup|GetFloorDetails)) 1))
          (LocalVariables|SetIndex _index)
          ;[1 1 1] Spawn a random Floor Actor on the current floor
          (bind _returnvalue (Game|SpawnActorfromClass (Utilities|Array|Get(acopy) (Utilities|Struct|BreakStruct_Interior_Floor (LocalVariables|GetFloor)) (Math|Random|RandomIntegerinRange 0 (Utilities|Array|LastIndex (Utilities|Struct|BreakStruct_Interior_Floor (LocalVariables|GetFloor))))) (Math|Transform|MakeTransform (Utilities|Array|Get(acopy) (Variables|Setup|GetFloorLocations) (LocalVariables|GetIndex)) (Transformation|GetActorRotation)) "AlwaysSpawn" 0 0))
          (LocalVariables|SetSpawnedActor _returnvalue)
          ;[1 1 1] Set self as the Parent Interior BP of the floor
          (bind _asbp_interior_floor_base (Utilities|Casting|CastToBP_InteriorFloor_Base (LocalVariables|GetSpawnedActor)))
          (LocalVariables|SetSpawnedFloor _asbp_interior_floor_base)
          (Variables|/Game/ProceduralCity/Blueprints/Buildings/Interiors/BaseClasses/BP_InteriorFloor_Base.BP_InteriorFloor_Base_C|SetParentInteriorBP (LocalVariables|GetSpawnedFloor) self)
          ;[1 1 1] Get current seed
          (Variables|Default|SetCurrentSeed (Utilities|Array|Get(acopy) (Variables|Setup|GetRandomSeedList) (LocalVariables|GetIndex)))
          ;[1 1 1] Set spawn seed
          (Variables|/Game/ProceduralCity/Blueprints/Buildings/Interiors/BaseClasses/BP_InteriorFloor_Base.BP_InteriorFloor_Base_C|SetRandomSeed (LocalVariables|GetSpawnedFloor) (Variables|Default|GetCurrentSeed))
          ;[1 1 1] Add reference to SpawnedObjects array
          (Utilities|Array|Add (Variables|Default|GetSpawnedFloors) (LocalVariables|GetSpawnedActor))
          ;[1 1 1] If we StarLoaded is True, also load the floor interiors
          (if (Variables|Setup|GetStartLoaded)
            (Variables|/Game/ProceduralCity/Blueprints/Buildings/Interiors/BaseClasses/BP_InteriorFloor_Base.BP_InteriorFloor_Base_C|SetStartLoaded (LocalVariables|GetSpawnedFloor) true))))
      (:NewEnumerator1
        ;[1 1 1] Loop through all the floors
        (for _index_2 (range 0 (- (Utilities|Struct|BreakStruct_Interior_FloorSetup (Variables|Setup|GetFloorDetails)) 1))
          (LocalVariables|SetIndex _index_2)
          ;[1 1 1] Is hte current floor within the Floor Range?
          (if (and (>= (+ (LocalVariables|GetIndex) 1) (.FloorRange-Min (Utilities|Struct|BreakStruct_Interior_Floor (LocalVariables|GetFloor)))) (<= (+ (LocalVariables|GetIndex) 1) (.FloorRange-Max (Utilities|Struct|BreakStruct_Interior_Floor (LocalVariables|GetFloor)))))
            ;[1 1 1] Spawn a random Floor Actor on the current floor
            (bind _returnvalue_2 (Game|SpawnActorfromClass (Utilities|Array|Get(acopy) (Utilities|Struct|BreakStruct_Interior_Floor (LocalVariables|GetFloor)) (Math|Random|RandomIntegerinRange 0 (Utilities|Array|LastIndex (Utilities|Struct|BreakStruct_Interior_Floor (LocalVariables|GetFloor))))) (Math|Transform|MakeTransform (Utilities|Array|Get(acopy) (Variables|Setup|GetFloorLocations) (LocalVariables|GetIndex)) (Transformation|GetActorRotation)) "AlwaysSpawn" 0 0))
            (LocalVariables|SetSpawnedActor _returnvalue_2)
            ;[1 1 1] Set self as the Parent Interior BP of the floor
            (bind _asbp_interior_floor_base_2 (Utilities|Casting|CastToBP_InteriorFloor_Base (LocalVariables|GetSpawnedActor)))
            (LocalVariables|SetSpawnedFloor _asbp_interior_floor_base_2)
            (Variables|/Game/ProceduralCity/Blueprints/Buildings/Interiors/BaseClasses/BP_InteriorFloor_Base.BP_InteriorFloor_Base_C|SetParentInteriorBP (LocalVariables|GetSpawnedFloor) self)
            ;[1 1 1] Get current seed
            (Variables|Default|SetCurrentSeed (Utilities|Array|Get(acopy) (Variables|Setup|GetRandomSeedList) (LocalVariables|GetIndex)))
            ;[1 1 1] Set spawn seed
            (Variables|/Game/ProceduralCity/Blueprints/Buildings/Interiors/BaseClasses/BP_InteriorFloor_Base.BP_InteriorFloor_Base_C|SetRandomSeed (LocalVariables|GetSpawnedFloor) (Variables|Default|GetCurrentSeed))
            ;[1 1 1] Add reference to SpawnedObjects array
            (Utilities|Array|Add (Variables|Default|GetSpawnedFloors) (LocalVariables|GetSpawnedActor))
            ;[1 1 1] If we StarLoaded is True, also load the floor interiors
            (if (Variables|Setup|GetStartLoaded)
              (Variables|/Game/ProceduralCity/Blueprints/Buildings/Interiors/BaseClasses/BP_InteriorFloor_Base.BP_InteriorFloor_Base_C|SetStartLoaded (LocalVariables|GetSpawnedFloor) true)))))
      (:NewEnumerator2
        ;[1 1 1] Loop through all the floors
        (for _index_3 (range 0 (- (Utilities|Struct|BreakStruct_Interior_FloorSetup (Variables|Setup|GetFloorDetails)) 1))
          (LocalVariables|SetIndex _index_3)
          ;[1 1 1] Is the current floor included in the Specific Floor list?
          (if (Utilities|Array|ContainsItem (Utilities|String|ParseIntoArray (Utilities|Struct|BreakStruct_Interior_Floor (LocalVariables|GetFloor)) ",") (Utilities|String|ToString(Integer) (+ (LocalVariables|GetIndex) 1)))
            ;[1 1 1] Spawn a random Floor Actor on the current floor
            (bind _returnvalue_3 (Game|SpawnActorfromClass (Utilities|Array|Get(acopy) (Utilities|Struct|BreakStruct_Interior_Floor (LocalVariables|GetFloor)) (Math|Random|RandomIntegerinRange 0 (Utilities|Array|LastIndex (Utilities|Struct|BreakStruct_Interior_Floor (LocalVariables|GetFloor))))) (Math|Transform|MakeTransform (Utilities|Array|Get(acopy) (Variables|Setup|GetFloorLocations) (LocalVariables|GetIndex)) (Transformation|GetActorRotation)) "AlwaysSpawn" 0 0))
            (LocalVariables|SetSpawnedActor _returnvalue_3)
            ;[1 1 1] Set self as the Parent Interior BP of the floor
            (bind _asbp_interior_floor_base_3 (Utilities|Casting|CastToBP_InteriorFloor_Base (LocalVariables|GetSpawnedActor)))
            (LocalVariables|SetSpawnedFloor _asbp_interior_floor_base_3)
            (Variables|/Game/ProceduralCity/Blueprints/Buildings/Interiors/BaseClasses/BP_InteriorFloor_Base.BP_InteriorFloor_Base_C|SetParentInteriorBP (LocalVariables|GetSpawnedFloor) self)
            ;[1 1 1] Get current seed
            (Variables|Default|SetCurrentSeed (Utilities|Array|Get(acopy) (Variables|Setup|GetRandomSeedList) (LocalVariables|GetIndex)))
            ;[1 1 1] Set spawn seed
            (Variables|/Game/ProceduralCity/Blueprints/Buildings/Interiors/BaseClasses/BP_InteriorFloor_Base.BP_InteriorFloor_Base_C|SetRandomSeed (LocalVariables|GetSpawnedFloor) (Variables|Default|GetCurrentSeed))
            ;[1 1 1] Add reference to SpawnedObjects array
            (Utilities|Array|Add (Variables|Default|GetSpawnedFloors) (LocalVariables|GetSpawnedActor))
            ;[1 1 1] If we StarLoaded is True, also load the floor interiors
            (if (Variables|Setup|GetStartLoaded)
              (Variables|/Game/ProceduralCity/Blueprints/Buildings/Interiors/BaseClasses/BP_InteriorFloor_Base.BP_InteriorFloor_Base_C|SetStartLoaded (LocalVariables|GetSpawnedFloor) true))))))))

(fn FnDestroyObjects
  ;[1 1 1] Loop through all the Spawned Actors
  (bind _keys (Utilities|Map|Keys (Variables|Default|GetSpawnedActors)))
  (for _array_element _keys
    (bind _output_get (LocalVariables|SetActor _array_element))
    (Utilities|IsValid _output_get
      (:Is%20Valid
        ;[1 1 1] Can we Despawn the actor?
        (if (.Value (Utilities|Map|Find (Variables|Default|GetSpawnedActors) (LocalVariables|GetActor)))
          ;[1 1 1] Destroy Actor
          (Actor|DestroyActor (LocalVariables|GetActor)))))))

(fn FnHideObjects
  ;[1 1 1] Loop through all Spawned Actors
  (bind _keys (Utilities|Map|Keys (Variables|Default|GetSpawnedActors)))
  (for _array_element _keys
    (bind _output_get (LocalVariables|SetActor _array_element))
    (Utilities|IsValid _output_get
      (:Is%20Valid
        ;[1 1 1] Can we Despawn the actor?
        (if (and (.Value (Utilities|Map|Find (Variables|Default|GetSpawnedActors) (LocalVariables|GetActor))) (.ReturnValue (Utilities|Map|Find (Variables|Default|GetSpawnedActors) (LocalVariables|GetActor))))
          ;[1 1 1] Hide Actor
          (Rendering|SetActorHiddenInGame (LocalVariables|GetActor) true))))))

(fn FnShowObjects
  ;[1 1 1] Loop through all the Spawned Actors
  (bind _keys (Utilities|Map|Keys (Variables|Default|GetSpawnedActors)))
  (for _array_element _keys
    (bind _output_get (LocalVariables|SetActor _array_element))
    (Utilities|IsValid _output_get
      (:Is%20Valid
        ;[1 1 1] Can we Despawn the actor?
        (if (and (.Value (Utilities|Map|Find (Variables|Default|GetSpawnedActors) (LocalVariables|GetActor))) (.ReturnValue (Utilities|Map|Find (Variables|Default|GetSpawnedActors) (LocalVariables|GetActor))))
          ;[1 1 1] Show Actor
          (Rendering|SetActorHiddenInGame (LocalVariables|GetActor) false))))))

(fn FnSetRelativeRotation
  (Utilities|IsValid (Variables|Setup|GetParentBuilding)
    (:Is%20Valid
      ;[1 1 1] Match the parent building's rotation
      (Transformation|SetActorRotation (Transformation|GetWorldRotation (Variables|/Game/ProceduralCity/Blueprints/Buildings/BP_PCGBuilding_Base.BP_PCGBuilding_Base_C|GetBuildingMesh (Variables|Setup|GetParentBuilding))) true))))

(fn FnCalculateFloors
  (bind _returnvalue (Transformation|GetActorLocation))
  (bind _floordetails (Variables|Setup|GetFloorDetails))
  (bind (_floorheight _usefloorheightlist _floorheightlist) (Utilities|Struct|BreakStruct_Interior_FloorSetup _floordetails))
  ;[1 1 1] Clear the array
  (Utilities|Array|Clear (Variables|Setup|GetFloorLocations))
  ;[1 1 1] Loop through all the floors
  (for _index (range 0 (- (Utilities|Struct|BreakStruct_Interior_FloorSetup (Variables|Setup|GetFloorDetails)) 1))
    (LocalVariables|SetIndex _index)
    ;[1 1 1] Add the current floor location to the array
    (Utilities|Array|Add (Variables|Setup|GetFloorLocations) (Math|Vector|MakeVector (.x _returnvalue) (.y _returnvalue) (select _usefloorheightlist (Utilities|Array|Get(acopy) _floorheightlist (LocalVariables|GetIndex)) (* (LocalVariables|GetIndex) _floorheight))))))

(fn FnRandomizeSeed
  ;[1 1 1] Clear list
  (Utilities|Array|Clear (Variables|Setup|GetRandomSeedList))
  ;[1 1 1] Loop through all the floors
  (for _index (range 0 (- (Utilities|Struct|BreakStruct_Interior_FloorSetup (Variables|Setup|GetFloorDetails)) 1))
    (LocalVariables|SetIndex _index)
    ;[1 1 1] Set random seed for current floor
    (Class|KismetMathLibrary|SeedRandomStream (Variables|Default|GetCurrentSeed))
    ;[1 1 1] Add a new seed entry
    (Utilities|Array|Add (Variables|Setup|GetRandomSeedList) (Variables|Default|GetCurrentSeed))))

(fn FnSpawnObjects
  ;[1 1 1] Clear the Spawned Objects array
  (Utilities|Map|Clear (Variables|Default|GetSpawnedActors))
  ;[1 1 1] Go through all Static Actors
  (for (_array_element _array_index) (Variables|GlobalSpawns|GetGlobalActorList)
    (LocalVariables|SetActor _array_element)
    (LocalVariables|SetIndex _array_index)
    ;[1 1 1] Do we spawn this actor?
    (if (and (.Value (Utilities|Map|Find (Variables|Default|GetSpawnList) (LocalVariables|GetIndex))) (.ReturnValue (Utilities|Map|Find (Variables|Default|GetSpawnList) (LocalVariables|GetIndex))))
      ;[1 1 1] Set Location Helper location
      (Transformation|SetRelativeTransform (Variables|Default|GetLocationHelper) (Utilities|Struct|BreakStruct_InteriorActors (LocalVariables|GetActor)) false true)
      ;[1 1 1] Is this the first spawn or is this actor  allowed to despawn?
      (if (or (Variables|Default|GetFirstSpawn?) (Utilities|Struct|BreakStruct_InteriorActors (LocalVariables|GetActor)))
        ;[1 1 1] Spawn actor
        (bind _returnvalue (Game|SpawnActorfromClass (Utilities|Struct|BreakStruct_InteriorActors (LocalVariables|GetActor)) (Transformation|GetWorldTransform (Variables|Default|GetLocationHelper)) "AlwaysSpawn" 0 0))
        (LocalVariables|SetSpawnedActor _returnvalue)
        ;[1 1 1] Add reference to SpawnedObjects array
        (Utilities|Map|Add (Variables|Default|GetSpawnedActors) (LocalVariables|GetSpawnedActor) (Utilities|Struct|BreakStruct_InteriorActors (LocalVariables|GetActor)))))))

(fn FnCalculateSpawnChance
  ;[1 1 1] Go through all static actors
  (for (_array_element _array_index) (Variables|GlobalSpawns|GetGlobalActorList)
    (LocalVariables|SetActor _array_element)
    (LocalVariables|SetIndex _array_index)
    ;[1 1 1] Do we spawn this actor?
    (if (>= (Math|Float|Clamp(Float) (Utilities|Struct|BreakStruct_InteriorActors (LocalVariables|GetActor))) (Math|Random|RandomFloatinRangefromStream 0.0 1.0 (Variables|Default|GetCurrentSeed)))
      ;[1 1 1] This actor can spawn
      (Utilities|Map|Add (Variables|Default|GetSpawnList) (LocalVariables|GetIndex) true)
      (else
        ;[1 1 1] This actor cannot spawn
        (Utilities|Map|Add (Variables|Default|GetSpawnList) (LocalVariables|GetIndex) false)))))

(event Custom|EventLoadInteriors
  (if (Variables|Default|GetFirstSpawn?)
    (CallFunction|FnSpawnFloorActors)
    (else
      (CallFunction|FnShowObjects))))

(event Custom|EventUnloadInteriors
  (CallFunction|FnHideObjects))

(event EventFnSimulatePhysicsAllActors
  ;[1 1 1] Loop through all spawned object actors
  (for _array_element (Variables|Default|GetSpawnedObjectsList)
    ;[1 1 1] Loop through all static mesh components and simulate physics
    (if (Utilities|Array|IsValidIndex (Actor|GetComponentsByClass _array_element "/Script/Engine.StaticMeshComponent"))
      (for _array_element_2 (Actor|GetComponentsByClass _array_element "/Script/Engine.StaticMeshComponent")
        (Physics|SetSimulatePhysics _array_element_2 true)))))