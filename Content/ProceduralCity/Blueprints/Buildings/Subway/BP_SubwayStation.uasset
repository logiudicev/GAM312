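; BP_SubwayStation is a procedural-city building that lets the player fast-travel between subway stations.
; It maps same-city stations on its own or connecting lines, and its trigger freezes the player and shows WBP_SubwayHUD.
; Travel teleports the player to the target's TeleportVolume, first requesting its streamed BP_CitySection, found by upward box trace, and retrying each second until loaded.
; Interface events handle naming, zone, city, cull distance and spline-based landscape alignment.
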(event OnComponentBeginOverlap(MenuTrigger)
  (params (OverlappedComponent :type Primitive%20Component%20Object%20Reference) (OtherActor :type Actor%20Object%20Reference) (OtherComp :type Primitive%20Component%20Object%20Reference) (OtherBodyIndex :type Integer) (bFromSweep :type Boolean) (SweepResult :type Hit%20Result%20Structure%20%28by%20ref%29))
  ;[1 1 1] Did we overlap the Player?
  (Variables|Default|SetOverlapActor OtherActor)
  (if (Actor|ActorHasTag OtherActor "Player")
    ;[1 1 1] Do we have at least 1 other station on the map?
    (if (> (Utilities|Map|Length (Variables|Default|GetStationMap)) 0)
      (Utilities|FlowControl|Sequence
        (:then_0
          ;[1 1 1] Stop the Player's movement
          (bind _ascharacter (Utilities|Casting|CastToCharacter (Variables|Default|GetOverlapActor)))
          (Pawn|Components|CharacterMovement|DisableMovement (Variables|/Script/Engine.Character|GetCharacterMovement _ascharacter)))
        (:then_1
          ;[1 1 1] Show the Station HUD
          (CallFunction|FnShowHUD))))))

(event Custom|EventDelayedStationCheck
  (Utilities|FlowControl|Delay 1.0)
  (CallFunction|FnGotoStation (Variables|Default|GetTargetStation)))

(event Custom|GetStationList
  ;[1 1 1] Get all the stations on the same line
  (CallFunction|FnGetStations)
  ;[1 1 1] Check if we are part of a city Section
  (CallFunction|FnCheckSection))

(event Custom|Set%20Cull%20Distance
  ;[1 1 1] Set max draw distance
  (Class|PrimitiveComponent|SetCullDistance (Variables|Default|GetMesh) (Variables|Setup|GetCullDistance)))

(fn ConstructionScript
  (Utilities|FlowControl|Sequence
    (:then_0
      ;[1 1 1] Set station material
      (Rendering|Material|SetMaterial (Variables|Default|GetMesh) 0 (Variables|Setup|GetSubwayMaterial))
      ;[1 1 1] Set Text parameters
      (Rendering|Components|TextRender|SetText (Variables|Default|GetTextRender) (Utilities|Text|ToText(Name) (Variables|Setup|GetStationName)))
      (Rendering|Components|TextRender|SetTextRenderColor (Variables|Default|GetTextRender) (Variables|Setup|GetTitleColor)))
    (:then_1
      ;[1 1 1] Show or Hide the Helper flag
      (Rendering|SetVisibility (Variables|Default|GetFlag) (Variables|Setup|GetShowHelperFlag) false))
    (:then_2
      ;[1 1 1] Set max draw distance
      (Class|PrimitiveComponent|SetCullDistance (Variables|Default|GetMesh) (Variables|Setup|GetCullDistance)))))

(fn FnGetStations
  ;[1 1 1] Clear Station Map
  (Utilities|Map|Clear (Variables|Default|GetStationMap))
  ;[1 1 1] Go through all the stations in the scene
  (bind _outactors (Actor|GetAllActorsOfClass "BP_SubwayStation_C"))
  (for _array_element _outactors
    (LocalVariables|SetStation _array_element)
    ;[1 1 1] Check that we are not selecting this station
    (if (!= (LocalVariables|GetStation) self)
      (Utilities|FlowControl|Sequence
        (:then_0
          ;[1 1 1] Check that this station is part of the city and part of the same line
          (if (and (Utilities|Name|Equal(Name) (Variables|BP_SubwayStation_C|GetCityName (LocalVariables|GetStation)) (Variables|Setup|GetCityName)) (Utilities|Name|Equal(Name) (Variables|BP_SubwayStation_C|GetSubwayLine (LocalVariables|GetStation)) (Variables|Setup|GetSubwayLine)))
            ;[1 1 1] Add Station to map
            (Utilities|Map|Add (Variables|Default|GetStationMap) (LocalVariables|GetStation) (Variables|Setup|GetSubwayLine))))
        (:then_1
          ;[1 1 1] Check that this station is part of the city and part of the connecting lines
          (if (and (Utilities|Name|Equal(Name) (Variables|BP_SubwayStation_C|GetCityName (LocalVariables|GetStation)) (Variables|Setup|GetCityName)) (Utilities|Array|ContainsItem (Variables|Setup|GetLineConnections) (Variables|BP_SubwayStation_C|GetSubwayLine (LocalVariables|GetStation))))
            ;[1 1 1] Add Station to map
            (Utilities|Map|Add (Variables|Default|GetStationMap) (LocalVariables|GetStation) (Variables|BP_SubwayStation_C|GetSubwayLine (LocalVariables|GetStation)))))))))

(fn FnGotoStation
  (params (Station :type BP%20Subway%20Station%20Object%20Reference))
  (Variables|Default|SetTargetStation Station)
  ;[1 1 1] Check if we dont have a City Section (no level streaming)
  (if (not (Utilities|IsValid (Variables|Setup|GetCitySection)))
    _
    (else
      (|CHECKCITYSECTION)))
  ;[1 1 1] Remove cursor and set focus to Game only
  (Variables|/Script/Engine.PlayerController|SetbShowMouseCursor (Game|GetPlayerController 0) false)
  (Input|SetInputModeGameOnly (Game|GetPlayerController 0))
  ;[1 1 1] Remove the HUD
  (Widget|RemovefromParent (Variables|Default|GetHUDRef))
  (Variables|Default|SetHUDRef 0)
  (Utilities|IsValid (Variables|Default|GetTargetStation)
    (:Is%20Valid
      ;[1 1 1] Teleport the Player to the new station
      (Transformation|SetActorLocationAndRotation (Variables|Default|GetOverlapActor) (Transformation|GetWorldLocation (Variables|BP_SubwayStation_C|GetTeleportVolume (Variables|Default|GetTargetStation))) (Transformation|GetWorldRotation (Variables|BP_SubwayStation_C|GetTeleportVolume (Variables|Default|GetTargetStation))))
      (Pawn|SetControlRotation (Game|GetPlayerController 0) (Transformation|GetWorldRotation (Variables|BP_SubwayStation_C|GetTeleportVolume (Variables|Default|GetTargetStation)))))
    (:Is%20Not%20Valid
      _))
  ;[1 1 1] Allow Player to walk again
  (bind _ascharacter (Utilities|Casting|CastToCharacter (Variables|Default|GetOverlapActor)))
  (Pawn|Components|CharacterMovement|SetMovementMode (Variables|/Script/Engine.Character|GetCharacterMovement _ascharacter) "MOVE_Walking" 0))

(fn FnShowHUD
  ;[1 1 1] Check that we dont have a HUD yet
  (if (not (Utilities|IsValid (Variables|Default|GetHUDRef)))
    ;[1 1 1] Create Subway Station menu
    (bind _returnvalue (UserInterface|CreateWidget "/Game/ProceduralCity/Blueprints/Widgets/WBP_SubwayHUD.WBP_SubwayHUD_C"))
    (bind _output_get (Variables|Default|SetHUDRef _returnvalue))
    (UserInterface|Viewport|AddtoPlayerScreen _output_get)
    ;[1 1 1] Set the owner to the Player
    (Default|FnSetOwner (Variables|Default|GetHUDRef) self)
    ;[1 1 1] Show the menu
    (Default|FnShowMenu (Variables|Default|GetHUDRef) (Variables|Default|GetStationMap) (Variables|Setup|GetAddLineToName))))

(fn FnAlignLandscape
  (bind _landscape_found (CallFunction|FnGetLandscape))
  (if _landscape_found
    (Utilities|IsValid (Variables|Setup-Landscape|GetLandscape)
      (:Is%20Valid
        ;[1 1 1] Apply Spline
        (Landscape|Editor|EditorApplySpline (Variables|Setup-Landscape|GetLandscape) (Variables|Default|GetSpline) (Variables|Setup-Landscape|GetStartWidth) (Variables|Setup-Landscape|GetEndWidth) (Variables|Setup-Landscape|GetStartSideFalloff) (Variables|Setup-Landscape|GetEndSideFalloff) 0.0 0.0 (Spline|GetNumberOfSplinePoints (Variables|Default|GetSpline)) (Variables|Setup-Landscape|GetRaiseHeight) (Variables|Setup-Landscape|GetLowerHeight) (Utilities|Array|Get(acopy) (Utilities|Array|MakeArray 0 0 0 0 0 0 0 0 0) (Variables|Setup-Landscape|GetLandscapeLayerIndex))))
      (:Is%20Not%20Valid
        ;[1 1 1] Landscape NOT FOUND!
        (Development|PrintString (Utilities|String|Append (Utilities|GetDisplayName self) ": Landscape actor NOT FOUND!") true true "(R=1.000000,G=0.000000,B=0.007289,A=1.000000)" 5.0)))))

(fn FnGetLandscape
  (bind _outactors (Actor|GetAllActorsOfClass "/Script/Landscape.Landscape"))
  (if (> (Utilities|Array|Length _outactors) 0)
    (bind _output_get (Variables|Setup-Landscape|SetLandscape (Utilities|Array|Get(acopy) _outactors)))
    (return (Utilities|IsValid _output_get))))

(fn FnSetDefaultName
  ;[1 1 1] Set the default Station Name
  (Variables|Setup|SetStationName (Utilities|String|StringToName (Utilities|GetDisplayName self))))

(fn FnCheckSection
  (bind _returnvalue (Transformation|GetActorLocation))
  ;[1 1 1] Do a box trace for city Sections
  (bind (_outhits _returnvalue_2) (Class|KismetSystemLibrary|BoxTraceMultiforObjects _returnvalue (+ _returnvalue "0, 0,200000.000000") "2.000000,2.000000,2.000000" (Transformation|GetActorRotation) (Utilities|Array|MakeArray "ObjectTypeQuery7") false 0 "None" true))
  (if _returnvalue_2
    (bind _array_element (Utilities|Array|ForEachLoopwithBreak _outhits)
      (:LoopBody
        (LocalVariables|SetHitActor (.HitActor (Collision|BreakHitResult _array_element)))
        ;[1 1 1] Did we find the local CitySection?
        (if (== (Utilities|GetClass (LocalVariables|GetHitActor)) "/Game/ProceduralCity/Blueprints/Main/BP_CitySection.BP_CitySection_C")
          ;[1 1 1] Save the City Section
          (bind _asbp_city_section (Utilities|Casting|CastToBP_CitySection (LocalVariables|GetHitActor)))
          (Variables|Setup|SetCitySection _asbp_city_section))))))

(event Custom|AlignLandscape
  (CallFunction|FnAlignLandscape))

(event EventFnSetParameters
  (CallFunction|FnSetDefaultName)
  ;[1 1 1] Set max draw distance
  (Class|PrimitiveComponent|SetCullDistance (Variables|Default|GetMesh) (Variables|Setup|GetCullDistance)))

(event EventFnSetCullDistance
  (params (Cull%20Distance :type Float%20%28single-precision%29))
  ;[1 1 1] Set max draw distance
  (Class|PrimitiveComponent|SetCullDistance (Variables|Default|GetMesh) Cull%20Distance))

(event EventFnGetTerrain
  (CallFunction|FnGetLandscape))

(event EventFnAlignTerrain
  (params (Landscape :type Landscape%20Object%20Reference))
  (CallFunction|FnAlignLandscape))

(event EventFnSetBuildingZone
  (params (Zone :type Enum_ZoneType%20Enum :default "NewEnumerator0"))
  (Variables|Setup|SetZoneType Zone))

(event EventFnSetCityName
  (params (City%20Name :type Name :default "None"))
  (Variables|Setup|SetCityName City%20Name))

(fn FnGetBounds
  (return "0, 0, 0" "0, 0, 0"))

(fn FnGetBuildingZone
  (return (Variables|Setup|GetZoneType)))