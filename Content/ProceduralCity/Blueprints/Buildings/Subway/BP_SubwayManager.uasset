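; BP_SubwayManager collects the subway stations that belong to a city in the procedural city.
; The GetCityStations event calls FnGetStations, which gathers every BP_SubwayStation actor in the scene.
; Stations whose actor tags contain CityName are appended to StationList, which is not cleared beforehand.
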(event Custom|Get%20City%20Stations
  (CallFunction|FnGetStations))

(fn ConstructionScript)

(fn FnGetStations
  ;[1 1 1] Get all subway stations in the scene
  (bind _outactors (Actor|GetAllActorsOfClass "/Game/ProceduralCity/Blueprints/Buildings/Subway/BP_SubwayStation.BP_SubwayStation_C"))
  (bind _output_get (LocalVariables|SetList _outactors))
  ;[1 1 1] Loop through all stations
  (for _array_element _output_get
    (LocalVariables|SetStation _array_element)
    ;[1 1 1] Check this station is part of the city
    (if (Utilities|Array|ContainsItem (Variables|/Script/Engine.Actor|GetTags (LocalVariables|GetStation)) (Variables|Setup|GetCityName))
      ;[1 1 1] Add station to the list
      (Utilities|Array|Add (Variables|Setup|GetStationList) (LocalVariables|GetStation)))))