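; Base building actor for the procedural city that sets its mesh, tag and cull distance on construction.
; A seeded random stream picks a material per slot on BeginPlay when enabled.
; It can spawn and attach an interior Blueprint, passing it the parent building and city name.
; Interface events set zone, city and culling, and flatten landscape beneath it through EditorApplySpline, using splines sized from mesh bounds.
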(event Custom|SetRandomMaterial
  (CallFunction|FnRandomizeMaterials))

(event Custom|RandomizeSeed
  (CallFunction|FnRandomizeSeed))

(event Custom|Spawn%20Interior%20BP
  (CallFunction|FnSpawnInteriorBP))

(event Custom|Attach%20Interior%20BP
  ;[1 1 1] Attach interior to building
  (Transformation|AttachActorToActor (Variables|Setup|GetInteriorActor) self "None" "KeepWorld" "KeepWorld" "KeepRelative" true))

(event EventBeginPlay
  ;[1 1 1] Randomize building materials
  (if (Variables|Setup|GetRandomMaterial)
    (CallFunction|FnRandomizeMaterials)))

(fn ConstructionScript
  ;[1 1 1] Set parameters
  (CallFunction|FnSetParams))

(fn FnAlignLandscape
  (bind _falloff (Variables|Setup-Landscape|GetFallOff))
  (bind _width (Variables|Setup-Landscape|GetWidth))
  (Utilities|IsValid (Variables|Setup-Landscape|GetLandscape)
    (:Is%20Valid
      (CallFunction|FnSetSplines)
      ;[1 1 1] Apply Spline - Width
      (Landscape|Editor|EditorApplySpline (Variables|Setup-Landscape|GetLandscape) (Variables|Default|GetSplineWidth) _width _width _falloff _falloff 0.0 0.0 (Spline|GetNumberOfSplinePoints (Variables|Default|GetSplineWidth)) (Variables|Setup-Landscape|GetRaiseHeight) (Variables|Setup-Landscape|GetLowerHeight) (Utilities|Array|Get(acopy) (Utilities|Array|MakeArray 0 0 0) (Variables|Setup-Landscape|GetLandscapeLayerIndex))))
    (:Is%20Not%20Valid
      ;[1 1 1] Landscape NOT FOUND!
      (Development|PrintString (Utilities|String|Append (Utilities|GetDisplayName self) ": Landscape actor NOT FOUND!") true true "(R=1.000000,G=0.000000,B=0.007289,A=1.000000)" 5.0))))

(fn FnSetParams
  ;[1 1 1] Set the static mesh
  (Components|StaticMesh|SetStaticMesh (Variables|Default|GetBuildingMesh) (Variables|Setup|GetMesh))
  ;[1 1 1] Add unique ID as a tag
  (Utilities|Array|AddUnique (Variables|Actor|GetTags) (Variables|Setup|GetUniqueID))
  ;[1 1 1] Randomize the seed
  (CallFunction|FnRandomizeSeed)
  ;[1 1 1] Set max draw distance to all static meshes
  (for _array_element (Actor|GetComponentsByClass "/Script/Engine.StaticMeshComponent")
    (Class|PrimitiveComponent|SetCullDistance _array_element (Variables|Setup|GetCullDistance))))

(fn FnRandomizeMaterials
  ;[1 1 1] Check that we have at least 1 entry
  (if (> (Utilities|Array|Length (Variables|Setup|GetRandomMaterialList)) 0)
    ;[1 1 1] Loop through the material list
    (for _array_element (Variables|Setup|GetRandomMaterialList)
      (LocalVariables|SetMaterial _array_element)
      ;[1 1 1] Set a random material per Material Index
      (Utilities|Map|Add (Variables|Default|GetFinalMaterialList) (.MaterialID (Utilities|Struct|BreakStruct_RandomMaterials (LocalVariables|GetMaterial))) (Utilities|Array|Get(acopy) (.MaterialList (Utilities|Struct|BreakStruct_RandomMaterials (LocalVariables|GetMaterial))) (Math|Random|RandomIntegerinRangefromStream 0 (Utilities|Array|LastIndex (.MaterialList (Utilities|Struct|BreakStruct_RandomMaterials (LocalVariables|GetMaterial)))) (Variables|Setup|GetRandomSeed)))))
    ;[1 1 1] Loop through the final material list
    (bind _keys (Utilities|Map|Keys (Variables|Default|GetFinalMaterialList)))
    (for _array_element_2 _keys
      (LocalVariables|SetMatIndex _array_element_2)
      ;[1 1 1] Set Material
      (Rendering|Material|SetMaterial (Variables|Default|GetBuildingMesh) (LocalVariables|GetMatIndex) (.Value (Utilities|Map|Find (Variables|Default|GetFinalMaterialList) (LocalVariables|GetMatIndex)))))))

(fn FnRandomizeSeed
  ;[1 1 1] Set a random seed
  (Class|KismetMathLibrary|SeedRandomStream (Variables|Setup|GetRandomSeed)))

(fn FnSetSplines
  (Utilities|FlowControl|Sequence
    (:then_0
      ;[1 1 1] Set to the Left
      (Spline|SetLocationatSplinePoint (Variables|Default|GetSplineLength) 0 (+ (Transformation|GetActorLocation) (* (Transformation|GetActorForwardVector) (.X (Math|Vector|BreakVector (.BoxExtent (Collision|GetComponentBounds (Variables|Default|GetBuildingMesh))))))) "World" true)
      ;[1 1 1] Set to Right
      (Spline|SetLocationatSplinePoint (Variables|Default|GetSplineLength) (- (Spline|GetNumberOfSplinePoints (Variables|Default|GetSplineWidth)) 1) (+ (Transformation|GetActorLocation) (* (* (Transformation|GetActorForwardVector) -1.0) (.X (Math|Vector|BreakVector (.BoxExtent (Collision|GetComponentBounds (Variables|Default|GetBuildingMesh))))))) "World" true))
    (:then_1
      ;[1 1 1] Set to the Left
      (Spline|SetLocationatSplinePoint (Variables|Default|GetSplineWidth) 0 (+ (Transformation|GetActorLocation) (* (Transformation|GetActorRightVector) (.Y (Math|Vector|BreakVector (.BoxExtent (Collision|GetComponentBounds (Variables|Default|GetBuildingMesh))))))) "World" true)
      ;[1 1 1] Set to Right
      (Spline|SetLocationatSplinePoint (Variables|Default|GetSplineWidth) (- (Spline|GetNumberOfSplinePoints (Variables|Default|GetSplineWidth)) 1) (+ (Transformation|GetActorLocation) (* (* (Transformation|GetActorRightVector) -1.0) (.Y (Math|Vector|BreakVector (.BoxExtent (Collision|GetComponentBounds (Variables|Default|GetBuildingMesh))))))) "World" true))
    (:then_2
      ;[1 1 1] Calculate Width
      (Variables|Setup-Landscape|SetWidth (* (Spline|GetSplineLength (Variables|Default|GetSplineLength)) (Variables|Setup-Landscape|GetWidthFactor))))))

(fn FnSpawnInteriorBP
  (bind _buildingmesh (Variables|Default|GetBuildingMesh))
  (bind _returnvalue (Transformation|GetWorldTransform _buildingmesh))
  ;[1 1 1] Do we have a avalid interior actor class?
  (if (Utilities|IsValidClass (Variables|Setup|GetInteriorActorClass))
    ;[1 1 1] Spawn interior BP
    (bind _returnvalue_2 (Game|SpawnActorfromClass (Variables|Setup|GetInteriorActorClass) (Math|Transform|MakeTransform (.location _returnvalue) (.rotation _returnvalue)) "Undefined" 0 0))
    (LocalVariables|SetSpawnedInterior _returnvalue_2)
    ;[1 1 1] Set spawned interior as the new Interior Actor reference
    (bind _asbp_interior_base (Utilities|Casting|CastToBP_Interior_Base (LocalVariables|GetSpawnedInterior)))
    (Variables|Setup|SetInteriorActor _asbp_interior_base)
    (Variables|/Game/ProceduralCity/Blueprints/Buildings/Interiors/BaseClasses/BP_Interior_Base.BP_Interior_Base_C|SetParentBuilding (Variables|Setup|GetInteriorActor) self)
    (Default|FnRandomizeSeed (Variables|Setup|GetInteriorActor))
    (Utilities|Array|Add (Variables|/Script/Engine.Actor|GetTags (Variables|Setup|GetInteriorActor)) (Variables|Setup|GetCityName))
    ;[1 1 1] Attach interior to building
    (Transformation|AttachActorToActor (LocalVariables|GetSpawnedInterior) self "None" "KeepWorld" "KeepWorld" "KeepRelative" true)
    (return (Variables|Setup|GetInteriorActor))))

(event EventFnSetParameters
  (CallFunction|FnSetParams)
  (Utilities|FlowControl|Delay 0.2)
  (CallFunction|AttachInteriorBP))

(event EventFnSetCullDistance
  (params (Cull%20Distance :type Float%20%28single-precision%29))
  (Variables|Setup|SetCullDistance Cull%20Distance)
  ;[1 1 1] Set max draw distance to all static meshes
  (for _array_element (Actor|GetComponentsByClass "/Script/Engine.StaticMeshComponent")
    (Class|PrimitiveComponent|SetCullDistance _array_element (Variables|Setup|GetCullDistance))))

(event EventFnGetTerrain
  (bind (_landscape_found _landscape) (CallFunction|FnBPLGetLandscape self (Variables|Setup-Landscape|GetTerrainTraceLength)))
  (if _landscape_found
    (Variables|Setup-Landscape|SetLandscape _landscape)))

(event EventFnAlignTerrain
  (params (Landscape :type Landscape%20Object%20Reference))
  (Variables|Setup-Landscape|SetLandscape Landscape)
  (CallFunction|FnSetSplines)
  (Utilities|FlowControl|Delay 0.2)
  (CallFunction|FnAlignLandscape))

(event EventFnSetBuildingZone
  (params (Zone :type Enum_ZoneType%20Enum :default "NewEnumerator0"))
  (Variables|Setup|SetZoneType Zone))

(event EventFnSetCityName
  (params (City%20Name :type Name :default "None"))
  (Variables|Setup|SetCityName City%20Name))

(event Custom|AlignLandscape
  (CallFunction|FnAlignLandscape))

(event Custom|Set%20Splines
  (CallFunction|FnSetSplines))

(event Custom|EventSetCullDistance
  (params (Cull%20Distance :type Float%20%28single-precision%29))
  (Variables|Setup|SetCullDistance Cull%20Distance)
  ;[1 1 1] Set max draw distance to all static meshes
  (for _array_element (Actor|GetComponentsByClass "/Script/Engine.StaticMeshComponent")
    (Class|PrimitiveComponent|SetCullDistance _array_element (Variables|Setup|GetCullDistance))))

(fn FnGetBounds
  (bind (_origin _boxextent) (Collision|GetActorBounds false))
  (return _origin _boxextent))

(fn FnGetBuildingZone
  (return (Variables|Setup|GetZoneType)))