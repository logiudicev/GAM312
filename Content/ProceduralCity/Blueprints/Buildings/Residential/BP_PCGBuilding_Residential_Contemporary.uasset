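; Contemporary residential building Blueprint for the procedural city, adding a driveway and a spawned car on top of its parent building class.
; The construction script runs the parent's, applies a max draw distance to the Driveway and CarLocation components, then calls FnSpawnCar through a DoOnce.
; FnSpawnCar spawns a sedan object spawner at CarLocation's world transform.
; The event graph holds only disabled default events, so all logic runs at construction.
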(event EventBeginPlay
  (|CallParentFunction) ; This node is disabled and will not be called.\nDrag off pins to build functionality.
)

(event Collision|EventActorBeginOverlap
  (params (OtherActor :type Actor%20Object%20Reference))
  (|CallParentFunction OtherActor) ; This node is disabled and will not be called.\nDrag off pins to build functionality.
)

(event EventTick
  (params (DeltaSeconds :type Float%20%28single-precision%29))
  (|CallParentFunction DeltaSeconds) ; This node is disabled and will not be called.\nDrag off pins to build functionality.
)

(fn ConstructionScript
  (|CallParentFunction)
  ;[1 1 1] Set Max Draw Distance for Driveway
  (Class|PrimitiveComponent|SetCullDistance (Variables|Default|GetDriveway) (Variables|Default|GetCullDistance))
  (Utilities|FlowControl|DoOnce false
    (:Completed
      (CallFunction|FnSpawnCar))))

(fn FnSpawnCar
  ;[1 1 1] Spawn vehicle at CarLocation
  (Game|SpawnActorfromClass "/Game/ProceduralCity/Blueprints/Spawners/Props/BP_ObjectSpawner_Sedan.BP_ObjectSpawner_Sedan_C" (Transformation|GetWorldTransform (Variables|Default|GetCarLocation)) "Undefined" 0 0))