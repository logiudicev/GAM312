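; BP_SimplePawn is a pawn in the ProceduralCity project that varies its look at spawn and ragdolls when damaged.
; On BeginPlay it applies a random material from MaterialList to mesh slot 0 and a uniform random mesh scale within ScaleRange.
; Any damage, regardless of amount, enables mesh collision and physics simulation and disables capsule collision, with no health check or recovery.
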(event EventBeginPlay
  (CallFunction|FnRandomizeMaterial)
  (CallFunction|FnSetActorScale))

(event Game|Damage|EventAnyDamage
  (params (Damage :type Float%20%28single-precision%29) (DamageType :type Damage%20Type%20Object%20Reference) (InstigatedBy :type Controller%20Object%20Reference) (DamageCauser :type Actor%20Object%20Reference))
  ;[1 1 1] Enable Mesh collision
  (Collision|SetCollisionEnabled (Variables|Character|GetMesh) "QueryAndPhysics")
  ;[1 1 1] Have the body ragdoll
  (Physics|SetSimulatePhysics (Variables|Character|GetMesh) true)
  ;[1 1 1] Disable Capsule collision
  (Collision|SetCollisionEnabled (Variables|Collision|GetCapsuleComponent) "NoCollision"))

(fn ConstructionScript)

(fn FnRandomizeMaterial
  (bind _materiallist (Variables|Setup|GetMaterialList))
  ;[1 1 1] Set random material
  (Rendering|Material|SetMaterial (Variables|Character|GetMesh) 0 (Utilities|Array|Get(acopy) _materiallist (Math|Random|RandomIntegerinRange 0 (Utilities|Array|LastIndex _materiallist)))))

(fn FnSetActorScale
  (bind _scalerange (Variables|Setup|GetScaleRange))
  ;[1 1 1] Set a random scale
  (bind _output_get (LocalVariables|SetRandomScale (Math|Random|RandomFloatinRange (.x _scalerange) (.y _scalerange))))
  (Transformation|SetWorldScale3D (Variables|Character|GetMesh) (Math|Vector|MakeVector _output_get _output_get _output_get)))