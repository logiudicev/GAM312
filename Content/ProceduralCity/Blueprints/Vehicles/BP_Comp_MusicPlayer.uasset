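; Music player component, filed with the vehicle Blueprints, that plays a song list through its owner's AudioComponent.
; Starting it creates an on-screen widget showing the song name from the MusicList map and optionally autoplays; stopping pauses playback and removes the widget.
; Next and previous wrap around the list or pick randomly when shuffling.
; A one-second looping timer advances when a song ends and is paused along with playback.
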(event Custom|EventStartMusic
  (bind _returnvalue (Components|GetOwner))
  (bind _returnvalue_2 (Actor|GetComponentbyClass _returnvalue "/Script/Engine.AudioComponent"))
  (Utilities|IsValid _returnvalue_2
    (:Is%20Valid
      (Variables|Default|SetAudioSource _returnvalue_2)
      (CallFunction|FnCreateHUD)
      (if (Variables|Setup|GetAutoPlay?)
        (CallFunction|FnPlaySong)))
    (:Is%20Not%20Valid
      (|ERROR))))

(event Custom|EventStopMusic
  (|PAUSEMUSIC)
  (Utilities|IsValid (Variables|Default|GetHUDRef)
    (:Is%20Valid
      (Widget|RemovefromParent (Variables|Default|GetHUDRef)))))

(event Custom|EventCheckMusicIsPlaying
  (bind _returnvalue (Utilities|Time|SetTimerbyEvent (delegate Custom|EventCheckMusicIsPlaying) 1.0 true))
  (Variables|Default|SetCheckHandler _returnvalue)
  ;[1 1 1] If song is no longer playing, play the next song
  (if (and (not (Audio|Components|Audio|IsPlaying (Variables|Default|GetAudioSource))) (not (Variables|Default|GetIsPaused)))
    (CallFunction|FnPlayNext)))

(fn FnPlaySong
  (if (Variables|Setup|GetShuffleSongs)
    ;[1 1 1] Pick a random song
    (Variables|Default|SetCurrentIndex (Math|Random|RandomIntegerinRange 0 (- (Utilities|Map|Length (Variables|Setup|GetMusicList)) 1))))
  ;[1 1 1] Get Current song
  (bind _keys (Utilities|Map|Keys (Variables|Setup|GetMusicList)))
  (Variables|Default|SetCurrentSong (Utilities|Array|Get(acopy) _keys (Variables|Default|GetCurrentIndex)))
  ;[1 1 1] Play Song
  (Audio|Components|Audio|SetSound (Variables|Default|GetAudioSource) (Variables|Default|GetCurrentSong))
  (Audio|Components|Audio|Play (Variables|Default|GetAudioSource) 0.0)
  ;[1 1 1] Set song name in HUD
  (Default|FnChangeName (Variables|Default|GetHUDRef) (Utilities|Text|ToText(Name) (.Value (Utilities|Map|Find (Variables|Setup|GetMusicList) (Variables|Default|GetCurrentSong)))))
  (CallFunction|EventCheckMusicIsPlaying))

(fn FnCreateHUD
  ;[1 1 1] Create Music Player Widget
  (bind _returnvalue (UserInterface|CreateWidget "/Game/ProceduralCity/Blueprints/Widgets/WBP_MusicPlayer.WBP_MusicPlayer_C"))
  (bind _output_get (Variables|Default|SetHUDRef _returnvalue))
  (UserInterface|Viewport|AddtoPlayerScreen _output_get))

(fn FnPlayNext
  (if (Variables|Setup|GetShuffleSongs)
    ;[1 1 1] Pick a random song
    (Variables|Default|SetCurrentIndex (Math|Random|RandomIntegerinRange 0 (- (Utilities|Map|Length (Variables|Setup|GetMusicList)) 1)))
    (else
      ;[1 1 1] Is the current Index less than the total number of songs?
      (if (< (Variables|Default|GetCurrentIndex) (- (Utilities|Map|Length (Variables|Setup|GetMusicList)) 1))
        ;[1 1 1] Add 1 to the index
        (Math|Integer|IncrementInt (Variables|Default|GetCurrentIndex)
          (:%20%20
            _))
        (else
          ;[1 1 1] Reset Index
          (Variables|Default|SetCurrentIndex 0)))))
  (CallFunction|FnPlaySong))

(fn FnPlayPrevious
  (if (Variables|Setup|GetShuffleSongs)
    ;[1 1 1] Pick a random song
    (Variables|Default|SetCurrentIndex (Math|Random|RandomIntegerinRange 0 (- (Utilities|Map|Length (Variables|Setup|GetMusicList)) 1)))
    (else
      ;[1 1 1] Is the current Index bigger than 0?
      (if (> (Variables|Default|GetCurrentIndex) 0)
        ;[1 1 1] Add 1 to the index
        (Math|Integer|DecrementInt (Variables|Default|GetCurrentIndex)
          (:%20%20
            _))
        (else
          ;[1 1 1] Set Index to last song
          (Variables|Default|SetCurrentIndex (- (Utilities|Map|Length (Variables|Setup|GetMusicList)) 1))))))
  (CallFunction|FnPlaySong))

(fn FnPauseSong
  (Utilities|IsValid (Variables|/Script/Engine.AudioComponent|GetSound (Variables|Default|GetAudioSource))
    (:Is%20Valid
      (if (Variables|Default|GetIsPaused)
        ;[1 1 1] Unpause the music
        (Class|AudioComponent|SetPaused (Variables|Default|GetAudioSource) false)
        (Variables|Default|SetIsPaused false)
        ;[1 1 1] Unpause music check
        (Utilities|Time|UnpauseTimerbyHandle (Variables|Default|GetCheckHandler))
        (else
          ;[1 1 1] Pause the music
          (Class|AudioComponent|SetPaused (Variables|Default|GetAudioSource) true)
          (Variables|Default|SetIsPaused true)
          ;[1 1 1] Pause music check
          (Utilities|Time|PauseTimerbyHandle (Variables|Default|GetCheckHandler)))))
    (:Is%20Not%20Valid
      (CallFunction|FnPlaySong))))