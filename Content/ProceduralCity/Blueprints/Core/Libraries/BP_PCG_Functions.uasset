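; Blueprint function library of downward terrain trace helpers for the procedural city tools.
; fnBPLGetLandscape multi-traces WorldStatic objects along an actor's negative up vector and returns the first exact Landscape hit.
; fnBPLGetHitLocation raises a point on world Z by the trace length, then Visibility-traces back along negative up, returning any surface's hit location without checking success.
; Its debug type input is unused, as drawing is fixed to ForDuration.
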(fn FnBPLGetLandscape
  (params (Reference%20Actor :type Actor%20Object%20Reference) (Trace%20Length :type Float%20%28single-precision%29))
  (LocalVariables|SetActor Reference%20Actor)
  (LocalVariables|SetTerrainTraceLength Trace%20Length)
  ;[1 1 1] Trace downward looking for a Landscape
  (bind _outhits (Class|KismetSystemLibrary|LineTraceMultiforObjects 0 (Transformation|GetActorLocation (LocalVariables|GetActor)) (+ (Transformation|GetActorLocation (LocalVariables|GetActor)) (* (* (Transformation|GetActorUpVector (LocalVariables|GetActor)) -1.0) (LocalVariables|GetTerrainTraceLength))) (Utilities|Array|MakeArray "ObjectTypeQuery1") false 0 "None" true))
  (bind _array_element (Utilities|Array|ForEachLoopwithBreak _outhits :!label _label)
    (:LoopBody
      (LocalVariables|SetHitActor (.HitActor (Collision|BreakHitResult _array_element)))
      ;[1 1 1] Did we hit a landscape?
      (if (== (Utilities|GetClass (LocalVariables|GetHitActor)) "/Script/Landscape.Landscape")
        (LocalVariables|SetFound true)
        (bind _aslandscape (Utilities|Casting|CastToLandscape (LocalVariables|GetHitActor)))
        (LocalVariables|SetLandscapeActor _aslandscape)
        (goto _label Break)
        (else
          (LocalVariables|SetFound false))))
    (:Completed
      (return (LocalVariables|GetFound) (LocalVariables|GetLandscapeActor)))))

(fn FnBPLGetHitLocation
  (params (Location :type Vector) (Up%20Vector :type Vector) (Trace%20Length :type Float%20%28single-precision%29) (Debug%20Type :type EDrawDebugTrace%20Enum :default "None"))
  (LocalVariables|SetLoc Location)
  (LocalVariables|SetUp Up%20Vector)
  (LocalVariables|SetTraceLength Trace%20Length)
  (LocalVariables|SetDebug Debug%20Type)
  ;[1 1 1] Trace downward looking for a Landscape
  (bind _outhit (Collision|LineTraceByChannel 0 (+ (LocalVariables|GetLoc) (Math|Vector|MakeVector 0.0 0.0 (LocalVariables|GetTraceLength))) (+ (+ (LocalVariables|GetLoc) (Math|Vector|MakeVector 0.0 0.0 (LocalVariables|GetTraceLength))) (* (* (LocalVariables|GetUp) -1.0) (LocalVariables|GetTraceLength))) "TraceTypeQuery1" false 0 "ForDuration" true "(R=1.000000,G=0.000000,B=0.000000,A=1.000000)" "(R=0.000000,G=1.000000,B=0.000000,A=1.000000)" 1e+01))
  (bind _output_get (LocalVariables|SetHitLocation (.Location (Collision|BreakHitResult _outhit))))
  (return _output_get))